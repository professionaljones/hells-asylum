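; Test variant of the Asylum HUD that manages menus, end screens and the in-game player HUD for campaign and mission modes.
; BeginPlay creates most widgets upfront and immediately shows a new test HUD, while events add screens to the viewport and switch input modes.
; Other events animate objectives, timed messages, combat fades and gamepad/keyboard prompts on PlayerHUDWidget, which this file never assigns, as setup fills TestHUDWidget instead.
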(event EventBeginPlay
  (CallFunction|SetupWidgets))

(event EventSetMOOne
  (params (NewObjective :type Text))
  (bind _playerhudwidget (Variables|Default|GetPlayerHUDWidget))
  (bind _wp_playerobjectivedata (Variables|/Game/Dynamic/UserInterface/WBPs/Gameplay/WBP_PlayerHUD.WBP_PlayerHUD_C|GetWP_PlayerObjectiveData _playerhudwidget))
  (Rendering|Components|TextRender|SetText (Variables|/Game/Dynamic/UserInterface/WBPs/Gameplay/Components/WP_PlayerObjectiveData.WP_PlayerObjectiveData_C|GetMO_One _wp_playerobjectivedata) NewObjective)
  (UserInterface|Animation|PlayAnimation _wp_playerobjectivedata (Variables|/Game/Dynamic/UserInterface/WBPs/Gameplay/Components/WP_PlayerObjectiveData.WP_PlayerObjectiveData_C|GetMO_One_Set _wp_playerobjectivedata) 0.0 1 "Forward" 1.0)
  (Variables|Default|SetbMO_OneSet true))

(event EventSetSOTwoComplete
  (bind _playerhudwidget (Variables|Default|GetPlayerHUDWidget))
  (bind _wp_playerobjectivedata (Variables|/Game/Dynamic/UserInterface/WBPs/Gameplay/WBP_PlayerHUD.WBP_PlayerHUD_C|GetWP_PlayerObjectiveData _playerhudwidget))
  (UserInterface|Animation|PlayAnimation _wp_playerobjectivedata (Variables|/Game/Dynamic/UserInterface/WBPs/Gameplay/Components/WP_PlayerObjectiveData.WP_PlayerObjectiveData_C|GetSO_Two_Complete _wp_playerobjectivedata) 0.0 1 "Forward" 1.0))

(event EventSetSOOneComplete
  (bind _playerhudwidget (Variables|Default|GetPlayerHUDWidget))
  (bind _wp_playerobjectivedata (Variables|/Game/Dynamic/UserInterface/WBPs/Gameplay/WBP_PlayerHUD.WBP_PlayerHUD_C|GetWP_PlayerObjectiveData _playerhudwidget))
  (UserInterface|Animation|PlayAnimation _wp_playerobjectivedata (Variables|/Game/Dynamic/UserInterface/WBPs/Gameplay/Components/WP_PlayerObjectiveData.WP_PlayerObjectiveData_C|GetSO_One_Complete _wp_playerobjectivedata) 0.0 1 "Forward" 1.0))

(event EventSetMessagewithTime
  (params (NewMessage :type Text) (Time :type Float%20%28single-precision%29))
  (bind _playerhudwidget (Variables|Default|GetPlayerHUDWidget))
  (bind _wp_tutorialmessage (Variables|/Game/Dynamic/UserInterface/WBPs/Gameplay/WBP_PlayerHUD.WBP_PlayerHUD_C|GetWP_TutorialMessage _playerhudwidget))
  (bind _constructanimation (Variables|/Game/Dynamic/UserInterface/WBPs/Gameplay/Components/WP_TutorialMessage.WP_TutorialMessage_C|GetConstructAnimation _wp_tutorialmessage))
  (Widget|SetVisibility _wp_tutorialmessage "SelfHitTestInvisible")
  (Widget|SetVisibility (Variables|/Game/Dynamic/UserInterface/WBPs/Gameplay/Components/WP_TutorialMessage.WP_TutorialMessage_C|GetM2Text _wp_tutorialmessage) "Hidden")
  (Rendering|Components|TextRender|SetText (Variables|/Game/Dynamic/UserInterface/WBPs/Gameplay/Components/WP_TutorialMessage.WP_TutorialMessage_C|GetMessageText _wp_tutorialmessage) NewMessage)
  (UserInterface|Animation|PlayAnimation _wp_tutorialmessage _constructanimation 0.0 1 "Forward" 1.0)
  (Utilities|FlowControl|Delay Time)
  (UserInterface|Animation|PlayAnimation _wp_tutorialmessage _constructanimation 0.0 1 "Reverse" 1.0)
  (Utilities|FlowControl|Delay 1.2)
  (Widget|SetVisibility _wp_tutorialmessage "Hidden")
  (Class|UserWidget|StopAnimation _wp_tutorialmessage _constructanimation))

(event EventShowEndScreenMission
  (bind _missionendscreenwidget (Variables|Default|GetMissionEndScreenWidget))
  (UserInterface|Viewport|AddtoViewport _missionendscreenwidget 0)
  (Input|SetInputModeUIOnly (Game|GetPlayerController 0) _missionendscreenwidget "DoNotLock")
  (Widget|SetVisibility (Variables|Default|GetPlayerHUDWidget) "Hidden"))

(event EventShowConsoleMenu
  (bind _consolewidget (Variables|Default|GetConsoleWidget))
  (UserInterface|Viewport|AddtoViewport _consolewidget 0)
  (Input|SetInputModeGameandUI (Game|GetPlayerController 0) _consolewidget "DoNotLock" false)
  (Class|AsylumHUDInterface|ShowPlayerHUD false))

(event EventShowPlayerHUD
  (params (bShowHUD :type Boolean))
  (if bShowHUD
    (Widget|SetVisibility (Variables|Default|GetPlayerHUDWidget) "Visible")
    (else
      (Widget|SetVisibility (Variables|Default|GetPlayerHUDWidget) "Hidden"))))

(event EventOnKeyboardInput
  (params (bIsKeyboard? :type Boolean))
  (bind _playerhudwidget (Variables|Default|GetPlayerHUDWidget))
  (bind _wp_powerbar (Variables|/Game/Dynamic/UserInterface/WBPs/Gameplay/WBP_PlayerHUD.WBP_PlayerHUD_C|GetWP_PowerBar _playerhudwidget))
  (if bIsKeyboard?
    (if (not (Variables|Default|GetbPlayKBAnim?))
      (Variables|Default|SetbPlayKBAnim? true)
      (Class|UserWidget|PlayAnimationForward _wp_powerbar (Variables|/Game/Dynamic/UserInterface/WBPs/Gameplay/Components/WP_PowerBar.WP_PowerBar_C|GetGamepadSwitchAnim _wp_powerbar) 1.5)
      (Variables|Default|SetbPlayGPAnim? false)
      (Class|WidgetSwitcher|SetActiveWidgetIndex (Variables|/Game/Dynamic/UserInterface/WBPs/Gameplay/Components/WP_Interact.WP_Interact_C|GetWidgetSwitcher_0 (Variables|/Game/Dynamic/UserInterface/WBPs/Gameplay/WBP_PlayerHUD.WBP_PlayerHUD_C|GetWP_Interact (Variables|Default|GetPlayerHUDWidget)))))))

(event EventSetMessageTwowithTime
  (params (Message :type Text) (Time :type Float%20%28single-precision%29))
  (bind _playerhudwidget (Variables|Default|GetPlayerHUDWidget))
  (bind _wp_tutorialmessage (Variables|/Game/Dynamic/UserInterface/WBPs/Gameplay/WBP_PlayerHUD.WBP_PlayerHUD_C|GetWP_TutorialMessage _playerhudwidget))
  (bind _m2text (Variables|/Game/Dynamic/UserInterface/WBPs/Gameplay/Components/WP_TutorialMessage.WP_TutorialMessage_C|GetM2Text _wp_tutorialmessage))
  (bind _constructanimation_m2 (Variables|/Game/Dynamic/UserInterface/WBPs/Gameplay/Components/WP_TutorialMessage.WP_TutorialMessage_C|GetConstructAnimation_M2 _wp_tutorialmessage))
  (Widget|SetVisibility _wp_tutorialmessage "SelfHitTestInvisible")
  (Widget|SetVisibility (Variables|/Game/Dynamic/UserInterface/WBPs/Gameplay/Components/WP_TutorialMessage.WP_TutorialMessage_C|GetMessageText _wp_tutorialmessage) "Hidden")
  (Rendering|Components|TextRender|SetText _m2text Message)
  (Utilities|FlowControl|Sequence
    (:then_0
      (if (not (Widget|IsVisible _m2text))
        (Widget|SetVisibility _m2text "SelfHitTestInvisible")))
    (:then_1
      (UserInterface|Animation|PlayAnimation _wp_tutorialmessage _constructanimation_m2 0.0 1 "Forward" 1.0)
      (Utilities|FlowControl|Delay Time)
      (UserInterface|Animation|PlayAnimation _wp_tutorialmessage _constructanimation_m2 0.0 1 "Reverse" 1.0)
      (Utilities|FlowControl|Delay 1.2)
      (Widget|SetVisibility _wp_tutorialmessage "Hidden")
      (Class|UserWidget|StopAnimation _wp_tutorialmessage _constructanimation_m2))))

(event EventOnGamepadInput
  (params (bIsGamepad? :type Boolean))
  (bind _playerhudwidget (Variables|Default|GetPlayerHUDWidget))
  (bind _wp_powerbar (Variables|/Game/Dynamic/UserInterface/WBPs/Gameplay/WBP_PlayerHUD.WBP_PlayerHUD_C|GetWP_PowerBar _playerhudwidget))
  (if bIsGamepad?
    (if (not (Variables|Default|GetbPlayGPAnim?))
      (Variables|Default|SetbPlayGPAnim? true)
      (Class|UserWidget|PlayAnimationReverse _wp_powerbar (Variables|/Game/Dynamic/UserInterface/WBPs/Gameplay/Components/WP_PowerBar.WP_PowerBar_C|GetGamepadSwitchAnim _wp_powerbar) 1.5)
      (Variables|Default|SetbPlayKBAnim? false)
      (Class|WidgetSwitcher|SetActiveWidgetIndex (Variables|/Game/Dynamic/UserInterface/WBPs/Gameplay/Components/WP_Interact.WP_Interact_C|GetWidgetSwitcher_0 (Variables|/Game/Dynamic/UserInterface/WBPs/Gameplay/WBP_PlayerHUD.WBP_PlayerHUD_C|GetWP_Interact _playerhudwidget)) 1))))

(event EventShowEndScreenCampaign
  (Utilities|FlowControl|Delay 6.0)
  (UserInterface|Viewport|AddtoViewport (Variables|Default|GetGameOverWidget) 0)
  (Variables|/Script/Engine.PlayerController|SetbShowMouseCursor (Game|GetPlayerController 0) true)
  (Audio|PlaySound2D "/Game/Static/SF_Drama_Music_Pack/Cues/Desolate_Beauty/No_Synth/DB-NS_Loop_1_Cue.DB-NS_Loop_1_Cue" 1.0 1.0 0.0 0 0))

(event EventSetMOTwo
  (params (NewObjective :type Text))
  (bind _playerhudwidget (Variables|Default|GetPlayerHUDWidget))
  (bind _wp_playerobjectivedata (Variables|/Game/Dynamic/UserInterface/WBPs/Gameplay/WBP_PlayerHUD.WBP_PlayerHUD_C|GetWP_PlayerObjectiveData _playerhudwidget))
  (Rendering|Components|TextRender|SetText (Variables|/Game/Dynamic/UserInterface/WBPs/Gameplay/Components/WP_PlayerObjectiveData.WP_PlayerObjectiveData_C|GetMO_Two _wp_playerobjectivedata) NewObjective)
  (UserInterface|Animation|PlayAnimation _wp_playerobjectivedata (Variables|/Game/Dynamic/UserInterface/WBPs/Gameplay/Components/WP_PlayerObjectiveData.WP_PlayerObjectiveData_C|GetMO_Two_Set _wp_playerobjectivedata) 0.0 1 "Forward" 1.0))

(event EventShowCountdown
  (bind _returnvalue (UserInterface|CreateWidget "/Game/Dynamic/UserInterface/WBPs/Gameplay/WBP_Countdown.WBP_Countdown_C" (Game|GetPlayerController 0)))
  (UserInterface|Viewport|AddtoViewport _returnvalue 0))

(event EventOnMainMenuStart
  (bind _returnvalue (Game|GetPlayerController 0))
  (bind _mainmenuwidget (Variables|Default|GetMainMenuWidget))
  (UserInterface|Viewport|AddtoViewport _mainmenuwidget 0)
  (Input|SetInputModeUIOnly _returnvalue (Variables|/Game/Dynamic/UserInterface/WBPs/MainMenu/WBP_MainMenu.WBP_MainMenu_C|GetCampaignButton _mainmenuwidget) "DoNotLock")
  (Variables|/Script/Engine.PlayerController|SetbShowMouseCursor _returnvalue true))

(event EventOnCampaignStart
  (Utilities|FlowControl|Delay 0.2)
  (UserInterface|Viewport|AddtoViewport (Variables|Default|GetPlayerHUDWidget) 0)
  (Input|SetInputModeGameOnly (Game|Player|GetOwningPlayerController)))

(event EventOnMissionStart
  (Class|AsylumHUDInterface|OnCampaignStart)
  (Variables|/Game/Dynamic/UserInterface/WBPs/Gameplay/WBP_PlayerHUD.WBP_PlayerHUD_C|SetbIsMissionMode (Variables|Default|GetPlayerHUDWidget) true))

(event EventSetSOOne
  (params (NewObjective :type Text))
  (bind _playerhudwidget (Variables|Default|GetPlayerHUDWidget))
  (bind _wp_playerobjectivedata (Variables|/Game/Dynamic/UserInterface/WBPs/Gameplay/WBP_PlayerHUD.WBP_PlayerHUD_C|GetWP_PlayerObjectiveData _playerhudwidget))
  (Rendering|Components|TextRender|SetText (Variables|/Game/Dynamic/UserInterface/WBPs/Gameplay/Components/WP_PlayerObjectiveData.WP_PlayerObjectiveData_C|GetSO_One _wp_playerobjectivedata) NewObjective)
  (UserInterface|Animation|PlayAnimation _wp_playerobjectivedata (Variables|/Game/Dynamic/UserInterface/WBPs/Gameplay/Components/WP_PlayerObjectiveData.WP_PlayerObjectiveData_C|GetSO_One_Set _wp_playerobjectivedata) 0.0 1 "Forward" 1.0))

(event EventSetSOTwo
  (params (NewObjective :type Text))
  (bind _playerhudwidget (Variables|Default|GetPlayerHUDWidget))
  (bind _wp_playerobjectivedata (Variables|/Game/Dynamic/UserInterface/WBPs/Gameplay/WBP_PlayerHUD.WBP_PlayerHUD_C|GetWP_PlayerObjectiveData _playerhudwidget))
  (Rendering|Components|TextRender|SetText (Variables|/Game/Dynamic/UserInterface/WBPs/Gameplay/Components/WP_PlayerObjectiveData.WP_PlayerObjectiveData_C|GetSO_Two _wp_playerobjectivedata) NewObjective)
  (UserInterface|Animation|PlayAnimation _wp_playerobjectivedata (Variables|/Game/Dynamic/UserInterface/WBPs/Gameplay/Components/WP_PlayerObjectiveData.WP_PlayerObjectiveData_C|GetSO_Two_Set _wp_playerobjectivedata) 0.0 1 "Forward" 1.0))

(event EventSetMOOneComplete
  (bind _playerhudwidget (Variables|Default|GetPlayerHUDWidget))
  (bind _wp_playerobjectivedata (Variables|/Game/Dynamic/UserInterface/WBPs/Gameplay/WBP_PlayerHUD.WBP_PlayerHUD_C|GetWP_PlayerObjectiveData _playerhudwidget))
  (UserInterface|Animation|PlayAnimation _wp_playerobjectivedata (Variables|/Game/Dynamic/UserInterface/WBPs/Gameplay/Components/WP_PlayerObjectiveData.WP_PlayerObjectiveData_C|GetMO_One_Complete _wp_playerobjectivedata) 0.0 1 "Forward" 1.0)
  (Variables|Default|SetbMO_OneDone true))

(event EventSetMOTwoComplete
  (bind _playerhudwidget (Variables|Default|GetPlayerHUDWidget))
  (bind _wp_playerobjectivedata (Variables|/Game/Dynamic/UserInterface/WBPs/Gameplay/WBP_PlayerHUD.WBP_PlayerHUD_C|GetWP_PlayerObjectiveData _playerhudwidget))
  (UserInterface|Animation|PlayAnimation _wp_playerobjectivedata (Variables|/Game/Dynamic/UserInterface/WBPs/Gameplay/Components/WP_PlayerObjectiveData.WP_PlayerObjectiveData_C|GetMO_Two_Complete _wp_playerobjectivedata) 0.0 1 "Forward" 1.0))

(fn ConstructionScript)

(fn SetupWidgets
  (bind _returnvalue (Game|GetPlayerController 0))
  (bind _returnvalue_2 (UserInterface|CreateWidget "/Game/Static/UI_Kit/Widgets/WBP_PlayerHUD_N.WBP_PlayerHUD_N_C" _returnvalue))
  (bind _output_get (Variables|Default|SetTestHUDWidget _returnvalue_2))
  (UserInterface|Viewport|AddtoViewport _output_get 0)
  (bind _returnvalue_3 (UserInterface|CreateWidget "/Game/Dynamic/UserInterface/WBPs/Gameplay/WBP_PlayerJournal.WBP_PlayerJournal_C" _returnvalue))
  (Variables|Default|SetJournalWidget _returnvalue_3)
  (bind _returnvalue_4 (UserInterface|CreateWidget "/Game/Dynamic/UserInterface/WBPs/Gameplay/WBP_PlayerPauseMenu.WBP_PlayerPauseMenu_C" _returnvalue))
  (Variables|Default|SetPauseWidget _returnvalue_4)
  (bind _returnvalue_5 (UserInterface|CreateWidget "/Game/Dynamic/UserInterface/WBPs/MainMenu/WBP_GameOptions.WBP_GameOptions_C" _returnvalue))
  (Variables|Default|SetOptionsWidget _returnvalue_5)
  (bind _returnvalue_6 (UserInterface|CreateWidget "/Game/Dynamic/UserInterface/WBPs/MainMenu/Mission/WBP_MissionMenu.WBP_MissionMenu_C" _returnvalue))
  (Variables|Default|SetMissionMenuWidget _returnvalue_6)
  (bind _returnvalue_7 (UserInterface|CreateWidget "/Game/Dynamic/UserInterface/WBPs/MainMenu/WBP_MainMenu.WBP_MainMenu_C" _returnvalue))
  (Variables|Default|SetMainMenuWidget _returnvalue_7)
  (bind _returnvalue_8 (UserInterface|CreateWidget "/Game/Dynamic/UserInterface/WBPs/Gameplay/WBP_GameOverCampaign.WBP_GameOverCampaign_C" _returnvalue))
  (Variables|Default|SetGameOverWidget _returnvalue_8)
  (bind _returnvalue_9 (UserInterface|CreateWidget "/Game/Dynamic/UserInterface/WBPs/Gameplay/Mission/WP_MissionScoreResults.WP_MissionScoreResults_C" _returnvalue))
  (Variables|Default|SetMissionEndScreenWidget _returnvalue_9)
  (bind _returnvalue_10 (UserInterface|CreateWidget "/Game/Dynamic/UserInterface/WBPs/MainMenu/WBP_CampaignMenu.WBP_CampaignMenu_C"))
  (Variables|Default|SetCampaignMenuWidget _returnvalue_10)
  (bind _returnvalue_11 (UserInterface|CreateWidget "/Game/Dynamic/UserInterface/WBPs/MainMenu/WBP_SaveScreen.WBP_SaveScreen_C" _returnvalue))
  (Variables|Default|SetSaveScreenWidget _returnvalue_11)
  (bind _returnvalue_12 (UserInterface|CreateWidget "/Game/Dynamic/UserInterface/WBPs/MainMenu/WBP_LoadScreen.WBP_LoadScreen_C" _returnvalue))
  (Variables|Default|SetLoadScreenWidget _returnvalue_12)
  (bind _returnvalue_13 (UserInterface|CreateWidget "/Game/Dynamic/UserInterface/WBPs/WBP_ConsoleMenu.WBP_ConsoleMenu_C" _returnvalue))
  (Variables|Default|SetConsoleWidget _returnvalue_13)
  (bind _returnvalue_14 (UserInterface|CreateWidget "/Game/Dynamic/UserInterface/WBPs/WBP_DebugMenu.WBP_DebugMenu_C" _returnvalue))
  (Variables|Default|SetDebugWidget _returnvalue_14))

(fn UpdateOpacityinCombat
  (params (Condition :type Boolean))
  (bind _returnvalue (CallFunction|GetPC))
  (bind _playerhudwidget (Variables|Default|GetPlayerHUDWidget))
  (bind _wp_playerdata (Variables|/Game/Dynamic/UserInterface/WBPs/Gameplay/WBP_PlayerHUD.WBP_PlayerHUD_C|GetWP_PlayerData _playerhudwidget))
  (bind _fadeoutanimation (Variables|/Game/Dynamic/UserInterface/WBPs/Gameplay/Components/WP_PlayerData.WP_PlayerData_C|GetFadeOutAnimation _wp_playerdata))
  (if Condition
    (Class|UserWidget|PlayAnimationReverse _wp_playerdata _fadeoutanimation 2.0)
    (if (Variables|/Script/HellsAsylum.AsylumCharacter|GetbIsInCombat _returnvalue)
      (Class|AsylumHUDInterface|ShowPlayerPowerBar _playerhudwidget (Variables|/Script/HellsAsylum.AsylumSuitComponent|GetbEnableMainAbility (Variables|/Script/HellsAsylum.AsylumPlayerCharacter|GetGoetheSuitComponent _returnvalue))))
    (else
      (Class|UserWidget|PlayAnimationForward _wp_playerdata _fadeoutanimation 2.0))))
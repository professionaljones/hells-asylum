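; Base HUD for the Asylum game that owns the player's UI widgets and switches between main menu, campaign and mission presentation.
; BeginPlay pre-creates every screen widget, from player HUD, journal and pause to menus, game-over and score screens.
; Start events, after a short delay, show the main menu with UI-only input or the player HUD with game-only input, flagging mission mode for missions.
; A helper dims the player data panel outside combat.
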(event EventBeginPlay
  (CallFunction|SetupWidgets))

(event EventOnMainMenuStart
  (bind _returnvalue (Game|Player|GetOwningPlayerController))
  (bind _mainmenuwidget (Variables|Default|GetMainMenuWidget))
  (Utilities|FlowControl|Delay 0.2)
  (UserInterface|Viewport|AddtoViewport _mainmenuwidget 0)
  (Input|SetInputModeUIOnly _returnvalue (Variables|/Game/Dynamic/UserInterface/WBPs/MainMenu/WBP_MainMenu.WBP_MainMenu_C|GetCampaignButton _mainmenuwidget) "DoNotLock")
  (Variables|/Script/Engine.PlayerController|SetbShowMouseCursor _returnvalue true))

(event EventOnCampaignStart
  (Utilities|FlowControl|Delay 0.2)
  (UserInterface|Viewport|AddtoViewport (Variables|Default|GetPlayerHUDWidget) 0)
  (Input|SetInputModeGameOnly (Game|Player|GetOwningPlayerController)))

(event EventOnMissionStart
  (Class|AsylumHUDInterface|OnCampaignStart)
  (Variables|/Game/Dynamic/UserInterface/WBPs/Gameplay/WBP_PlayerHUD.WBP_PlayerHUD_C|SetbIsMissionMode (Variables|Default|GetPlayerHUDWidget) true))

(fn ConstructionScript)

(fn SetupWidgets
  (bind _returnvalue (Game|GetPlayerController 0))
  (bind _returnvalue_2 (UserInterface|CreateWidget "/Game/Dynamic/UserInterface/WBPs/Gameplay/WBP_PlayerHUD.WBP_PlayerHUD_C" _returnvalue))
  (Variables|Default|SetPlayerHUDWidget _returnvalue_2)
  (bind _returnvalue_3 (UserInterface|CreateWidget "/Game/Dynamic/UserInterface/WBPs/Gameplay/WBP_PlayerJournal.WBP_PlayerJournal_C" _returnvalue))
  (Variables|Default|SetJournalWidget _returnvalue_3)
  (bind _returnvalue_4 (UserInterface|CreateWidget "/Game/Dynamic/UserInterface/WBPs/Gameplay/WBP_PlayerPauseMenu.WBP_PlayerPauseMenu_C" _returnvalue))
  (Variables|Default|SetPauseWidget _returnvalue_4)
  (bind _returnvalue_5 (UserInterface|CreateWidget "/Game/Dynamic/UserInterface/WBPs/MainMenu/WBP_GameOptions.WBP_GameOptions_C" _returnvalue))
  (Variables|Default|SetOptionsWidget _returnvalue_5)
  (bind _returnvalue_6 (UserInterface|CreateWidget "/Game/Dynamic/UserInterface/WBPs/MainMenu/Mission/WBP_MissionMenu.WBP_MissionMenu_C" _returnvalue))
  (Variables|Default|SetMissionMenuWidget _returnvalue_6)
  (bind _returnvalue_7 (UserInterface|CreateWidget "/Game/Dynamic/UserInterface/WBPs/MainMenu/WBP_MainMenu.WBP_MainMenu_C" _returnvalue))
  (Variables|Default|SetMainMenuWidget _returnvalue_7)
  (bind _returnvalue_8 (UserInterface|CreateWidget "/Game/Dynamic/UserInterface/WBPs/Gameplay/WBP_GameOverCampaign.WBP_GameOverCampaign_C" _returnvalue))
  (Variables|Default|SetGameOverWidget _returnvalue_8)
  (bind _returnvalue_9 (UserInterface|CreateWidget "/Game/Dynamic/UserInterface/WBPs/Gameplay/Mission/WP_MissionScoreResults.WP_MissionScoreResults_C" _returnvalue))
  (Variables|Default|SetMissionEndScreenWidget _returnvalue_9)
  (bind _returnvalue_10 (UserInterface|CreateWidget "/Game/Dynamic/UserInterface/WBPs/MainMenu/WBP_CampaignMenu.WBP_CampaignMenu_C"))
  (Variables|Default|SetCampaignMenuWidget _returnvalue_10))

(fn UpdateOpacityinCombat
  (params (Condition :type Boolean))
  (bind _playerhudwidget (Variables|Default|GetPlayerHUDWidget))
  (bind _wp_playerdata (Variables|/Game/Dynamic/UserInterface/WBPs/Gameplay/WBP_PlayerHUD.WBP_PlayerHUD_C|GetWP_PlayerData _playerhudwidget))
  (if Condition
    (Widget|SetRenderOpacity _wp_playerdata 1.0)
    (else
      (Widget|SetRenderOpacity _wp_playerdata 0.1))))
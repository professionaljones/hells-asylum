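; Save game object that stores the player's stats, suit abilities, campaign and mission profile data, inventories and XP progress.
; SetSavedValues takes whole stat, suit and profile structs plus weapon and item inventories, a weapon array and XP values, and stores them directly.
; GetSavedValues breaks those structs into individual outputs, returned alongside the inventories, weapon array and XP values.
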(fn SetSavedValues
  (params (SG_PlayerStatsStruct :type Character%20Stats%20Data%20Structure) (SG_PlayerSuitStatsStruct :type Goethe%20Suit%20Stats%20Data%20Structure) (SG_ProfileDataStruct :type Save%20Game%20Data%20Structure) (SG_WeaponInventory :type Map%20of%20Integers%20to%20Classs) (SG_ItemInventory :type Map%20of%20Integers%20to%20Classs) (SG_CurrentXP :type Float%20%28single-precision%29) (SG_XPLimit :type Float%20%28single-precision%29) (SG_WeaponArray :type Map%20of%20Integers%20to%20Objects))
  (Variables|DatatoSave|SetSG_PlayerStatsStruct SG_PlayerStatsStruct)
  (Variables|DataToSave|SetSG_PlayerSuitStatsStruct SG_PlayerSuitStatsStruct)
  (Variables|DataToSave|SetSG_ProfileDataStruct SG_ProfileDataStruct)
  (Variables|DataToSave|SetSG_WeaponInventory SG_WeaponInventory)
  (Variables|DataToSave|SetSG_WeaponArray SG_WeaponArray)
  (Variables|DataToSave|SetSG_ItemInventory SG_ItemInventory)
  (Variables|DataToSave|SetSG_CurrentXP SG_CurrentXP)
  (Variables|DataToSave|SetSG_XPLimit SG_XPLimit))

(fn GetSavedValues
  (bind _sg_playerstatsstruct (Variables|DatatoSave|GetSG_PlayerStatsStruct))
  (bind _sg_playersuitstatsstruct (Variables|DataToSave|GetSG_PlayerSuitStatsStruct))
  (bind _sg_profiledatastruct (Variables|DataToSave|GetSG_ProfileDataStruct))
  (bind (_bhasshield _fcurrenthealth _fmaxhealth _fcurrentstamina _fmaxstamina _fcurrentshield _fmaxshield _icurrentcharacterlevel _imaxcharacterlevel _fmovementloudness _fmovementmaxrange _fcrouchmovementloudness _fcrouchmovementmaxrange _ffireresist _ficeresist _fshockresist) (Utilities|Struct|BreakCharacterStatsData _sg_playerstatsstruct))
  (bind (_goetheselectedmainability _goethesuittype _goethepassivepowerone _goethepassivepowertwo _goethepassivepowerboots _goethepassivepowerjet _goetheactivepowerone _goetheactivepowertwo _goetheactivepowerthree _despairorbcurrentlevel _despairorbmaxlevel _harmonyorbcurrentlevel _harmonyorbmaxlevel _teslacurrentlevel _teslamaxlevel _chargercurrentlevel _chargermaxlevel _stormcurrentlevel _stormmaxlevel _tractorcurrentlevel _tractormaxlevel _energydraincurrentlevel _energydrainmaxlevel _weaponpowerscurrentlevel _weaponpowersmaxlevel _currentaragongauge _maxaragongauge _currentaragontanks _aragonregenamount _aragonregenspeed _maxaragontanks _quicksilverslowdownamount _quicksilverplayerspeed _quicksilverconsumptionrate _overdriveconsumptionrate _sacrificeconsumptionrate _sacrificepowerlimit _overdrivespeedboost _energydrainconsumptionrate _discordabilitycooldown _harmonyabilitycooldown _snowabilitycooldown _chargerabilitycooldown _drainabilitycooldown _teslaabilitycooldown _weaponabilitycooldown _scanradius _enemysearchradius) (Utilities|Struct|BreakGoetheSuitStatsData _sg_playersuitstatsstruct))
  (bind (_savedate _currentcampaignmodeact _savedgamedifficulty_campaign _savedgamedifficulty_mission _playercurrentpoints_campaign _playercurrentpoints_mission _saveablecampaigndatamap _saveablemissiondatamap _savedlevelname _playerstartlocation _playersavecheckpointlocation _savedcurrentplayerxp _savedplayerxplimit _playerlifetimepoints_campaign _playerlifetimepoints_mission _playercurrentshardcount _playerlifetimeshardcount) (Utilities|Struct|BreakSaveGameData _sg_profiledatastruct))
  (return _bhasshield _fcurrenthealth _fmaxhealth _fcurrentshield _fmaxshield _icurrentcharacterlevel _imaxcharacterlevel _fmovementloudness _fmovementmaxrange _fcrouchmovementloudness _fcrouchmovementmaxrange (Variables|DataToSave|GetSG_WeaponInventory) (Variables|DataToSave|GetSG_ItemInventory) _ffireresist _ficeresist _fshockresist _goetheselectedmainability _goethesuittype _goethepassivepowerone _goethepassivepowertwo _goethepassivepowerboots _goethepassivepowerjet _goetheactivepowerone _goetheactivepowertwo _goetheactivepowerthree _despairorbcurrentlevel _despairorbmaxlevel _harmonyorbcurrentlevel _harmonyorbmaxlevel _teslacurrentlevel _teslamaxlevel _chargercurrentlevel _chargermaxlevel _stormcurrentlevel _stormmaxlevel _tractorcurrentlevel _tractormaxlevel _energydraincurrentlevel _energydrainmaxlevel _weaponpowerscurrentlevel _weaponpowersmaxlevel _currentaragongauge _maxaragongauge _currentaragontanks _aragonregenamount _aragonregenspeed _maxaragontanks _quicksilverslowdownamount _quicksilverplayerspeed _quicksilverconsumptionrate _overdriveconsumptionrate _sacrificeconsumptionrate _sacrificepowerlimit _overdrivespeedboost _energydrainconsumptionrate _discordabilitycooldown _harmonyabilitycooldown _snowabilitycooldown _chargerabilitycooldown _drainabilitycooldown _teslaabilitycooldown _weaponabilitycooldown _scanradius _enemysearchradius _currentcampaignmodeact _savedgamedifficulty_campaign _savedgamedifficulty_mission _playercurrentpoints_campaign _playercurrentpoints_mission _saveablecampaigndatamap _saveablemissiondatamap _savedlevelname _playersavecheckpointlocation _playerstartlocation _playerlifetimepoints_campaign _playerlifetimepoints_mission _playercurrentshardcount _playerlifetimeshardcount _savedate _fcurrentstamina _fmaxstamina (Variables|DataToSave|GetSG_CurrentXP) (Variables|DataToSave|GetSG_XPLimit) (Variables|DataToSave|GetSG_WeaponArray)))
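; Mission player state that tracks score, crit multiplier and boost drop chance during a level.
; Enemy kills add points, multiply the whole running total, raise drop chance, and update the HUD, player character and game state.
; Crits reset drop chance and set a multiplier with a looping countdown timer.
; It registers the level in save data, pushes mission stats to the game instance, checks placement thresholds, and saves on level exit.
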(event EventBeginPlay
  (bind _returnvalue (CallFunction|GetProjectInstance))
  (bind _savedatastruct (Variables|/Script/HellsAsylum.AsylumGameInstance|GetSaveDataStruct _returnvalue))
  (bind _saveablemissiondatamap (Utilities|Struct|BreakSaveGameData _savedatastruct))
  (bind _returnvalue_2 (Game|GetCurrentLevelName true))
  (if (not (.ReturnValue (Utilities|Map|Find _saveablemissiondatamap _returnvalue_2)))
    (Utilities|Map|Add _saveablemissiondatamap _returnvalue_2 (.Value (Utilities|Map|Find _saveablemissiondatamap _returnvalue_2)))))

(event EventOnLevelExit
  (bind _returnvalue (Game|GetGameInstance))
  (Class|BPIAsylumGameInterface|OnUpdateMissionDataMap(Message) _returnvalue (Variables|/Script/HellsAsylum.AsylumGameStateBase|GetCurrentMissionLevelData (CallFunction|GetMissionGameState)))
  (Class|BPIAsylumGameInterface|OnGameMissionSave(Message) _returnvalue "MissionSave01"))

(event EventOnCalculatePlayerScore
  (Class|BPIAsylumGameInterface|OnUpdateMissionDataMap(Message) (Game|GetGameInstance) (Variables|/Script/HellsAsylum.AsylumGameStateBase|GetCurrentMissionLevelData (CallFunction|GetMissionGameState)))
  (Utilities|LVMinScoreCheck
    (:true
      (Utilities|ThirdPlaceScoreCheck
        (:true
          (Utilities|SecondPlaceScoreCheck
            (:true
              (Utilities|FirstPlaceScoreCheck))))))))

(event EventCopyProperties
  (params (NewPlayerState :type Player%20State%20Object%20Reference))
  (|CallParentFunction NewPlayerState))

(event EventOnMissionEnemyKill
  (params (PointsToAdd :type Float%20%28single-precision%29))
  (bind _returnvalue (Game|GetGameState))
  (bind _playercurrentscore (Variables|Default|GetPlayerCurrentScore))
  (Utilities|UpdatePlayerScore PointsToAdd
    (:Exit
      (Class|BPIHUD|UpdatePlayerScoreText(Message) (Variables|/Game/Static/UI_Kit/Widgets/WBP_PlayerHUD_N.WBP_PlayerHUD_N_C|GetWP_MissionPanel (Variables|/Game/Dynamic/UserInterface/BP_AsylumHUD_Base.BP_AsylumHUD_Base_C|GetPlayerHUDWidget_N (CallFunction|GetGameHUD))) _playercurrentscore)
      (Default|CallOnPlayerUpdate (.AsBP%20Player%20Character%20Melanie (Utilities|Casting|CastToBP_PlayerCharacter_Melanie (Utilities|ResolveSoftReference (Variables|Default|GetPC_SO)))))
      (Class|AsylumHUDInterface|OnUpdateRPCMission(Message) _returnvalue _playercurrentscore)
      (Variables|Default|SetPlayerBoostDropChance (+ (Variables|Default|GetPlayerBoostDropChance) 0.03))
      (bind _structout (Utilities|Struct|SetmembersinMissionLevelStats (Variables|/Script/HellsAsylum.AsylumGameStateBase|GetCurrentMissionLevelData (CallFunction|GetMissionGameState)) _playercurrentscore))
      (Class|BPIAsylumGameInterface|OnUpdateMissionDataMap(Message) _returnvalue _structout))))

(event EventOnCritStart
  (params (NewMultiplierAmount :type Float%20%28single-precision%29) (MultiplierTimeLimit :type Float%20%28single-precision%29))
  (Variables|Default|SetPlayerBoostDropChance 0.0)
  (bind _output_get (Variables|Default|SetPlayerCurrentScoreMultiplier NewMultiplierAmount))
  (Variables|Default|SetScoreMultiplierTimeLimit MultiplierTimeLimit)
  (Rendering|Components|TextRender|SetText (Variables|/Game/Dynamic/UserInterface/WBPs/Gameplay/Mission/WP_MissionPanel.WP_MissionPanel_C|GetMultiplierText (Variables|/Game/Static/UI_Kit/Widgets/WBP_PlayerHUD_N.WBP_PlayerHUD_N_C|GetWP_MissionPanel (Variables|/Game/Dynamic/UserInterface/BP_AsylumHUD_Base.BP_AsylumHUD_Base_C|GetPlayerHUDWidget_N (CallFunction|GetGameHUD)))) (Utilities|Text|ToText(Float) _output_get "HalfToEven"))
  (bind _returnvalue (Utilities|Time|SetTimerbyEvent (EventDispatchers|CreateEvent :!event MultiplierCountdown) 1.0 true))
  (Variables|Default|SetMultiplierTimerHandle _returnvalue))

(event EventOnCritEnd
  (bind _output_get (Variables|Default|SetPlayerCurrentScoreMultiplier 1.0))
  (Variables|Default|SetScoreMultiplierTimeLimit 0.0)
  (Rendering|Components|TextRender|SetText (Variables|/Game/Dynamic/UserInterface/WBPs/Gameplay/Mission/WP_MissionPanel.WP_MissionPanel_C|GetMultiplierText (Variables|/Game/Static/UI_Kit/Widgets/WBP_PlayerHUD_N.WBP_PlayerHUD_N_C|GetWP_MissionPanel (Variables|/Game/Dynamic/UserInterface/BP_AsylumHUD_Base.BP_AsylumHUD_Base_C|GetPlayerHUDWidget_N (CallFunction|GetGameHUD)))) (Utilities|Text|ToText(Float) _output_get "HalfToEven")))

(fn ConstructionScript
  (|CallParentFunction))

(fn MultiplierCountdown
  (bind _output_get (Variables|Default|SetScoreMultiplierTimeLimit (- (Variables|Default|GetScoreMultiplierTimeLimit) 1.0)))
  (if (<= _output_get 0.0)
    (Utilities|Time|ClearandInvalidateTimerbyHandle (Variables|Default|GetMultiplierTimerHandle))))
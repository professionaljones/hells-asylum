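; Campaign game mode that handles player spawning, game-type start messages and pickup drops.
; BeginPlay notifies the HUD and non-player AsylumCharacterInterface actors whether campaign or mission play is active.
; Pawn spawning uses the saved checkpoint when one exists, otherwise the given transform.
; Drops depend on player health, shield and equipped-weapon ammo, plus a mission-only multiplier; inverted threshold ordering leaves medium and high tiers unreachable.
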(event EventBeginPlay
  (bind _returnvalue (CallFunction|GetGameHUD))
  (switch Utilities|FlowControl|Switch|SwitchonEGameType (Variables|Default|GetCurrentGameType)
    (:MGT_Campaign
      (Class|AsylumHUDInterface|OnCampaignStart(Message) _returnvalue)
      (bind _outactors (Actor|GetAllActorswithInterface "/Script/HellsAsylum.AsylumCharacterInterface"))
      (for _array_element _outactors
        (if (!= _array_element (Game|GetPlayerCharacter 0))
          (Class|AsylumCharacterInterface|OnMissionMode(Message) _array_element false))))
    (:MGT_MissionStandard
      (Class|AsylumHUDInterface|OnMissionStart(Message) _returnvalue :!label _label)
      (bind _outactors_2 (Actor|GetAllActorswithInterface "/Script/HellsAsylum.AsylumCharacterInterface"))
      (for _array_element_2 _outactors_2
        (if (!= _array_element_2 (Game|GetPlayerCharacter 0))
          (Class|AsylumCharacterInterface|OnMissionMode(Message) _array_element_2 true))))
    (:MGT_MissionStealth
      (goto _label))
    (:MGT_MissionAttack
      (goto _label))
    (:MGT_MissionSurvival
      (goto _label))
    (:MGT_BossRush
      (goto _label))
    (:MGT_Variety
      (goto _label))))

(event EventOnSpawnPickup
  (params (SpawnLocation :type Vector :default "0, 0, 0"))
  (CallFunction|SpawnRandomPickup SpawnLocation))

(event EventOnSpawnItemPickup
  (params (SpawnPoint :type Vector :default "0, 0, 0") (ItemToSpawn :type Item%20Pickup%20Base%20Class%20Reference))
  (CallFunction|SpawnItemPickup SpawnPoint ItemToSpawn))

(fn ConstructionScript)

(fn SpawnDefaultPawnatTransform
  (params (NewPlayer :type Controller%20Object%20Reference) (SpawnTransform :type Transform%20%28by%20ref%29))
  (bind _player_save_checkpoint_location (CallFunction|GetCheckpointLocation))
  (if (CallFunction|GetSaveStatus)
    (if (== _player_save_checkpoint_location (Math|Transform|MakeTransform "0, 0, 0"))
      _
      (else
        ;[1 1 1] Pawn should spawn at Player Start
        (bind _returnvalue (|CallParentFunction NewPlayer _player_save_checkpoint_location))
        (return _returnvalue))))
  ;[1 1 1] Pawn will spawn at saved location
  (bind _returnvalue_2 (|CallParentFunction NewPlayer SpawnTransform))
  (return _returnvalue_2))

(fn SpawnRandomPickup
  (params (SpawnLocation :type Vector))
  (bind _returnvalue (CallFunction|GetPC))
  (Utilities|FlowControl|Sequence
    (:then_0
      (CallFunction|SpawnHealthPickup _returnvalue SpawnLocation))
    (:then_1
      (CallFunction|SpawnShieldPickup _returnvalue SpawnLocation))
    (:then_2
      (CallFunction|SpawnAmmoPickup _returnvalue SpawnLocation))
    (:then_3
      (if (Variables|Default|GetbIsMissionMode)
        (if (>= (Variables|/Script/HellsAsylum.AsylumPlayerState|GetPlayerBoostDropChance (.AsBP%20Asylum%20Player%20State%20Mission (Utilities|Casting|CastToBP_AsylumPlayerState_Mission (CallFunction|GetCurrentPlayerState)))) 0.2)
          (Game|SpawnActorfromClass "/Game/Dynamic/Pickups/Mission/MultiplierPickup_2X.MultiplierPickup_2X_C" (Math|Transform|MakeTransform SpawnLocation "0, 0, 0" "1,1,1") "Undefined" 0 0))))))

(fn SpawnHealthPickup
  (params (PC :type Asylum%20Player%20Character%20Object%20Reference) (SpawnLocation :type Vector))
  (bind _returnvalue (Class|AsylumPlayerCharacter|GetPlayerHealthPercentage PC))
  (if (<= _returnvalue 0.75)
    (Game|SpawnActorfromClass "/Game/Dynamic/Pickups/Health/HealthPickup_Low.HealthPickup_Low_C" (Math|Transform|MakeTransform SpawnLocation "0, 0, 0" "1,1,1") "Undefined" 0 0)
    (elif (<= _returnvalue 0.5)
      (Game|SpawnActorfromClass "/Game/Dynamic/Pickups/Health/HealthPickup_Medium.HealthPickup_Medium_C" (Math|Transform|MakeTransform SpawnLocation "0, 0, 0" "1,1,1") "Undefined" 0 0)
      (elif (<= _returnvalue 0.25)
        (Game|SpawnActorfromClass "/Game/Dynamic/Pickups/Health/HealthPickup_High.HealthPickup_High_C" (Math|Transform|MakeTransform SpawnLocation "0, 0, 0" "1,1,1") "Undefined" 0 0)))))

(fn SpawnShieldPickup
  (params (PC :type Asylum%20Player%20Character%20Object%20Reference) (SpawnLocation :type Vector))
  (bind _returnvalue (Class|AsylumPlayerCharacter|GetPlayerShieldPercentage PC))
  (if (<= _returnvalue 0.75)
    (Game|SpawnActorfromClass "/Game/Dynamic/Pickups/Shield/ShieldPickup_Low.ShieldPickup_Low_C" (Math|Transform|MakeTransform SpawnLocation "0, 0, 0" "1,1,1") "Undefined" 0 0)
    (elif (<= _returnvalue 0.5)
      (Game|SpawnActorfromClass "/Game/Dynamic/Pickups/Shield/ShieldPickup_Medium.ShieldPickup_Medium_C" (Math|Transform|MakeTransform SpawnLocation "0, 0, 0" "1,1,1") "Undefined" 0 0))))

(fn SpawnAmmoPickup
  (params (PC :type Asylum%20Player%20Character%20Object%20Reference) (SpawnLocation :type Vector))
  (bind _currentequippedweapon (Variables|/Script/HellsAsylum.AsylumCharacter|GetCurrentEquippedWeapon PC))
  (Utilities|IsValid _currentequippedweapon
    (:Is%20Valid
      (if (<= (Class|AsylumWeapon|GetAmmoPercentage _currentequippedweapon) 0.75)
        (Game|SpawnActorfromClass "/Game/Dynamic/Pickups/Weapons/AmmoPickup.AmmoPickup_C" (Math|Transform|MakeTransform SpawnLocation "0, 0, 0" "1,1,1") "Undefined" 0 0)))))

(fn SpawnItemPickup
  (params (SpawnLocation :type Vector) (Class :type Actor%20Class%20Reference))
  (Game|SpawnActorfromClass Class (Math|Transform|MakeTransform SpawnLocation "0, 0, 0" "1,1,1") "Undefined" 0 0))
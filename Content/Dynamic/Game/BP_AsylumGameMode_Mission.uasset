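; Mission game mode that sets up Discord rich presence and announces mission start when play begins.
; BeginPlay loops over existing DiscordRPCActor instances and caches valid ones, spawning one only for an invalid element, so an empty result spawns nothing.
; A second sequence branch waits briefly, then calls OnMissionStartMessage on the first player's HUD.
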(event EventBeginPlay
  (Utilities|FlowControl|Sequence
    (:then_0
      (bind _outactors (Actor|GetAllActorsOfClass "/Game/Dynamic/LevelAssets/DiscordRPCActor.DiscordRPCActor_C"))
      (for _array_element _outactors
        (Utilities|IsValid _array_element
          (:Is%20Valid
            (Variables|Default|SetDRPC_Reference _array_element))
          (:Is%20Not%20Valid
            (bind _returnvalue (Game|SpawnActorfromClass "/Game/Dynamic/LevelAssets/DiscordRPCActor.DiscordRPCActor_C" (Math|Transform|MakeTransform "0, 0, 0") "Undefined" 0 0))
            (Variables|Default|SetDRPC_Reference _returnvalue)))))
    (:then_1
      (Utilities|FlowControl|Delay 0.2)
      (Class|AsylumHUDInterface|OnMissionStart(Message) (HUD|GetHUD (Game|GetPlayerController 0))))))

(fn ConstructionScript)
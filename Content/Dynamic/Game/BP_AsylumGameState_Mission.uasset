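; Mission game state that tracks living and dead enemies and relays score updates to Discord Rich Presence.
; BeginPlay registers every AsylumCharacterInterface actor except player 0 as a remaining enemy in the mission level data.
; It also caches a DiscordRPCActor; the spawn fallback sits inside the search loop, so it never runs when none exist.
; UpdateEnemyArray moves killed enemies to the dead list, while OnUpdateRPCMission forwards the new score to that actor.
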(event EventBeginPlay
  (|CallParentFunction)
  (Utilities|FlowControl|Sequence
    (:then_0
      (bind _outactors (Actor|GetAllActorswithInterface "/Script/HellsAsylum.AsylumCharacterInterface"))
      (for _array_element _outactors
        (if (!= _array_element (Game|GetPlayerCharacter 0))
          (Utilities|Array|Add (Utilities|Struct|BreakMissionLevelStats (Variables|Default|GetCurrentMissionLevelData)) _array_element))))
    (:then_1
      (bind _outactors_2 (Actor|GetAllActorsOfClass "/Game/Dynamic/LevelAssets/DiscordRPCActor.DiscordRPCActor_C"))
      (for _array_element_2 _outactors_2
        (Utilities|IsValid _array_element_2
          (:Is%20Valid
            (Variables|Default|SetDRPCReference _array_element_2))
          (:Is%20Not%20Valid
            (bind _returnvalue (Game|SpawnActorfromClass "/Game/Dynamic/LevelAssets/DiscordRPCActor.DiscordRPCActor_C" (Math|Transform|MakeTransform "0, 0, 0") "Undefined" 0 0))
            (Variables|Default|SetDRPCReference _returnvalue)))))))

(event EventUpdateEnemyArray
  (params (EnemyKilled :type Actor%20Object%20Reference))
  (bind _currentmissionleveldata (Variables|Default|GetCurrentMissionLevelData))
  (bind (_missionenemiesremaining _missionenemiesdead) (Utilities|Struct|BreakMissionLevelStats _currentmissionleveldata))
  (bind _returnvalue (Utilities|Array|RemoveItem _missionenemiesremaining EnemyKilled))
  (if _returnvalue
    (Utilities|Array|Add _missionenemiesdead EnemyKilled)
    (Utilities|Struct|SetmembersinMissionLevelStats _currentmissionleveldata _missionenemiesdead)))

(event EventOnUpdateRPCMission
  (params (NewPlayerScore :type Float%20%28single-precision%29))
  (Default|UpdateRPforMission (Variables|Default|GetDRPCReference) NewPlayerScore))

(fn ConstructionScript
  (|CallParentFunction))
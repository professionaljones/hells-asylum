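; Blueprint function library of shared helpers for the Asylum game's campaign and mission modes.
; Typed getters wrap casts to the game instance, game modes, game states, HUD and player, exposing save data such as difficulty, checkpoint, stats and inventories.
; Utilities handle floored damage math, desktop platform checks and gathering non-player characters by interface.
; Setters start a new campaign at the prologue with a chosen difficulty and write mission score thresholds.
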(fn IsRunningonPlatform
  (switch string (Game|GetPlatformName)
    (:Windows
      _)
    (:Mac
      _)
    (:Linux
      _)
    (:PS4
      (return false))
    (:XboxOne
      (return false))
    (:HTML5
      (return false))
    (:Android
      (return false)))
  (return true))

(fn DamageCalculation
  (params (BaseDamageAmount :type Float%20%28single-precision%29) (DamageMultiplierAmount :type Float%20%28single-precision%29) (DamageModiferAmount :type Float%20%28single-precision%29))
  (return (Math|Conversions|ToFloat(Integer) (Math|Float|Floor (* BaseDamageAmount (+ DamageMultiplierAmount 1.0) (+ DamageModiferAmount 1.0))))))

(fn GetMissionGameState
  (return (.AsBP%20Asylum%20Game%20State%20Mission (Utilities|Casting|CastToBP_AsylumGameState_Mission (Game|GetGameState)))))

(fn GetPC
  (return (.AsBP%20Player%20Character%20Melanie (Utilities|Casting|CastToBP_PlayerCharacter_Melanie (Game|GetPlayerCharacter 0)))))

(fn GetGameDifficulty
  (bind _returnvalue (CallFunction|GetProjectInstance))
  (bind _savedatastruct (Variables|/Script/HellsAsylum.AsylumGameInstance|GetSaveDataStruct _returnvalue))
  (bind _savedgamedifficulty_campaign (Utilities|Struct|BreakSaveGameData _savedatastruct))
  (Utilities|IsValid _returnvalue
    (:Is%20Valid
      (if (== _savedgamedifficulty_campaign 1)
        (return "Easy")
        (elif (== _savedgamedifficulty_campaign 2)
          (return "Normal")
          (elif (== _savedgamedifficulty_campaign 3)
            (return "Hard")
            (elif (== _savedgamedifficulty_campaign 4)
              (return "Extreme")
              (elif (== _savedgamedifficulty_campaign 5)
                (return "Huntress")
                (elif (== _savedgamedifficulty_campaign 6)
                  (return "Easy+")
                  (elif (== _savedgamedifficulty_campaign 7)
                    (return "Normal+")
                    (elif (== _savedgamedifficulty_campaign 8)
                      (return "Hard+")
                      (elif (== _savedgamedifficulty_campaign 9)
                        (return "Extreme+")
                        (elif (== _savedgamedifficulty_campaign 10)
                          (return "Huntress+"))))))))))))))

(fn GetProjectInstance
  (return (.AsBP%20Asylum%20Game%20Instance (Utilities|Casting|CastToBP_AsylumGameInstance (Game|GetGameInstance)))))

(fn LoadingfromSave?
  (bind _returnvalue (CallFunction|GetProjectInstance))
  (Utilities|IsValid _returnvalue
    (:Is%20Valid
      (return (Variables|/Script/HellsAsylum.AsylumGameInstance|GetbWasSaveLoaded _returnvalue)))))

(fn GetPlayerStatsfromSave
  (bind _returnvalue (CallFunction|GetProjectInstance))
  (return (Variables|/Script/HellsAsylum.AsylumGameInstance|GetSavedPlayerSuitStats _returnvalue) (Variables|/Script/HellsAsylum.AsylumGameInstance|GetSavedPlayerCharacterStats _returnvalue) (Variables|/Script/HellsAsylum.AsylumGameInstance|GetSavedPlayerItemInventory _returnvalue) (Variables|/Script/HellsAsylum.AsylumGameInstance|GetSavedPlayerWeaponInventory _returnvalue)))

(fn GetMissionModeStatus
  (bind _returnvalue (CallFunction|GetStoryGameMode))
  (bind _returnvalue_2 (CallFunction|GetMissionGameMode))
  (Utilities|IsValid _returnvalue
    (:Is%20Valid
      (return (Variables|/Script/HellsAsylum.AsylumGameModeBase|GetbIsMissionMode _returnvalue)))
    (:Is%20Not%20Valid
      (Utilities|IsValid _returnvalue_2
        (:Is%20Valid
          (return (Variables|/Script/HellsAsylum.AsylumGameModeBase|GetbIsMissionMode _returnvalue_2)))))))

(fn GetStoryGameMode
  (return (.AsBP%20Asylum%20Game%20Mode%20Campaign (Utilities|Casting|CastToBP_AsylumGameMode_Campaign (Game|GetGameMode)))))

(fn GetMissionGameMode
  (return (.AsBP%20Asylum%20Game%20Mode%20Mission (Utilities|Casting|CastToBP_AsylumGameMode_Mission (Game|GetGameMode)))))

(fn StartNewGame
  (params (Saved%20Game%20Difficulty%20Campaign :type Integer))
  (bind _returnvalue (CallFunction|GetProjectInstance))
  (Game|OpenLevel(byName) _returnvalue "CM_Prologue")
  (Utilities|Struct|SetmembersinSaveGameData (Variables|/Script/HellsAsylum.AsylumGameInstance|GetSaveDataStruct _returnvalue) Saved%20Game%20Difficulty%20Campaign))

(fn GetGameHUD
  (return (.AsBP%20Asylum%20HUD%20Base (Utilities|Casting|CastToBP_AsylumHUD_Base (HUD|GetHUD (Game|GetPlayerController 0))))))

(fn GetSaveStatus
  (bind _returnvalue (CallFunction|GetProjectInstance))
  (Utilities|IsValid _returnvalue
    (:Is%20Valid
      (return (Variables|/Script/HellsAsylum.AsylumGameInstance|GetbWasSaveLoaded _returnvalue)))))

(fn GetCheckpointLocation
  (return (.PlayerSaveCheckpointLocation (Utilities|Struct|BreakSaveGameData (Variables|/Script/HellsAsylum.AsylumGameInstance|GetSaveDataStruct (CallFunction|GetProjectInstance))))))

(fn GetPlayerItemInventory
  (return (Variables|/Script/HellsAsylum.AsylumPlayerCharacter|GetItemInventory (.AsAsylum%20Player%20Character (Utilities|Casting|CastToAsylumPlayerCharacter (Game|GetPlayerCharacter 0))))))

(fn IsPlayerOtherActor?
  (params (ActorToCheck :type Actor%20Object%20Reference))
  (return (== ActorToCheck (Game|GetPlayerCharacter 0))))

(fn SetMissionLevelStats
  (params (LVMinScore :type Float%20%28single-precision%29) (TPScore :type Float%20%28single-precision%29) (SPScore :type Float%20%28single-precision%29) (FPScore :type Float%20%28single-precision%29))
  (bind _returnvalue (Game|GetPlayerController 0))
  (bind _playerstate (Variables|/Script/Engine.Controller|GetPlayerState _returnvalue))
  (bind _asbp_asylum_player_state_mission (Utilities|Casting|CastToBP_AsylumPlayerState_Mission _playerstate))
  (Class|AsylumGameStateBase|SetLevelScores (.AsAsylum%20Game%20State%20Base (Utilities|Casting|CastToAsylumGameStateBase (Game|GetGameState))) LVMinScore TPScore SPScore FPScore)
  (bind _structout (Utilities|Struct|SetmembersinMissionLevelStats (Variables|/Game/Dynamic/Game/BP_AsylumPlayerState_Mission.BP_AsylumPlayerState_Mission_C|GetCurrentLevelStats _asbp_asylum_player_state_mission) LVMinScore TPScore SPScore FPScore))
  (Variables|/Game/Dynamic/Game/BP_AsylumPlayerState_Mission.BP_AsylumPlayerState_Mission_C|SetCurrentLevelStats _asbp_asylum_player_state_mission _structout))

(fn GetCurrentPlayerState
  (return (Variables|/Script/Engine.Controller|GetPlayerState (Game|GetPlayerController 0))))

(fn GetDifficultyModfier
  (return (.SavedGameDifficulty_Campaign (Utilities|Struct|BreakSaveGameData (Variables|/Script/HellsAsylum.AsylumGameInstance|GetSaveDataStruct (CallFunction|GetProjectInstance))))))

(fn AddEnemiestoArray
  (params (TargetArray :type Array%20of%20Actor%20Object%20References))
  (bind _outactors (Actor|GetAllActorswithInterface 0 "/Script/HellsAsylum.AsylumCharacterInterface"))
  (for _array_element _outactors
    (if (!= _array_element (Game|GetPlayerCharacter 0))
      (Utilities|Array|Add TargetArray _array_element))))

(fn GetCampaignGameState
  (return (.AsBP%20Asylum%20Game%20State%20Campaign (Utilities|Casting|CastToBP_AsylumGameState_Campaign (Game|GetGameState)))))
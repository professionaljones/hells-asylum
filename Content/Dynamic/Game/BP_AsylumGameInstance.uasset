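; Game instance that owns persistent campaign and mission progress: points, shards, per-level data maps and cached player stats, suit and inventories.
; Events update SaveDataStruct, which save functions write with player data to BP_AsylumSaveGame slots, with separate functions for missions.
; Loading refills these cached structs and can reopen the saved level; Init loads a hard save if found.
; Slot-existence checks return on the first array entry.
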(event EventOnGameSave
  (params (SlotName :type String))
  (if (Utilities|Enum|Equal(Enum) SlotName "")
    (CallFunction|SaveGame (Variables|Default|GetCurrentSave))
    (else
      (CallFunction|SaveGame SlotName))))

(event EventOnCampaignEnemyDeath
  (params (f_PointsToAdd :type Float%20%28single-precision%29))
  (bind _savedatastruct (Variables|Default|GetSaveDataStruct))
  (bind (_savedate _playercurrentpoints_campaign _playerlifetimepoints_campaign) (Utilities|Struct|BreakSaveGameData _savedatastruct))
  (bind _returnvalue (+ _playercurrentpoints_campaign f_PointsToAdd))
  (Utilities|Struct|SetmembersinSaveGameData _savedatastruct _returnvalue (+ _playerlifetimepoints_campaign _returnvalue)))

(event EventAdjustSoundClassVolume
  (params (SoundMixInUse :type Sound%20Mix%20Object%20Reference) (SoundClassInUse :type Sound%20Class%20Object%20Reference) (NewValue :type Float%20%28single-precision%29) (bApplyToChildren :type Boolean))
  (Audio|SetSoundMixClassOverride SoundMixInUse SoundClassInUse NewValue 1.0 1.0 bApplyToChildren))

(event EventOnNewGameStart
  (bind _savedatastruct (Variables|Default|GetSaveDataStruct))
  (bind _saveablecampaigndatamap (Utilities|Struct|BreakSaveGameData _savedatastruct))
  (for _array_element (Class|MapNamesBPLibrary|GetBaseStoryMapNamesP)
    (for _array_element_2 (Variables|Default|GetCampaignLevelEventArray)
      (Utilities|Map|Add _saveablecampaigndatamap _array_element _array_element_2)
      (Utilities|Struct|SetmembersinSaveGameData _savedatastruct _saveablecampaigndatamap))))

(event EventOnShardPickup
  (bind _savedatastruct (Variables|Default|GetSaveDataStruct))
  (Class|BPIHUD|SetMessagewithTime(Message) (CallFunction|GetGameHUD) "Aragon Shard Collected!" 3.0)
  (bind _result (Math|Integer|IncrementInt (Utilities|Struct|BreakSaveGameData _savedatastruct))
    (:%20%20
      (Utilities|Struct|SetmembersinSaveGameData _savedatastruct _result)
      (Class|AsylumPlayerInterface|OnPlayerRecoverFullStats(Message) (Game|GetPlayerCharacter 0)))))

(event EventOnDFragPickup)

(event EventOnMissionEnemyDeath
  (params (f_PointsToAdd :type Float%20%28single-precision%29))
  (bind _savedatastruct (Variables|Default|GetSaveDataStruct))
  (bind (_savedate _playercurrentpoints_mission _playerlifetimepoints_mission) (Utilities|Struct|BreakSaveGameData _savedatastruct))
  (bind _returnvalue (+ _playercurrentpoints_mission f_PointsToAdd))
  (Utilities|Struct|SetmembersinSaveGameData _savedatastruct _returnvalue (+ _playerlifetimepoints_mission _returnvalue))
  (Class|AslyumMissionModeInterface|OnMissionEnemyKill(Message) (Variables|/Script/Engine.Controller|GetPlayerState (Game|GetPlayerController 0)) f_PointsToAdd))

(event EventOnGameLoad
  (params (SlotName :type String) (bShouldLoadNewLevel? :type Boolean))
  (CallFunction|LoadGame SlotName)
  (Variables|Default|SetbWasSaveLoaded true)
  (if bShouldLoadNewLevel?
    (Game|OpenLevel(byName) (Utilities|String|StringToName (.SavedLevelName (Utilities|Struct|BreakSaveGameData (Variables|Default|GetSaveDataStruct)))))))

(event EventInit
  (bind (_returnvalue _array_element) (CallFunction|DoHardSavesExist))
  (Variables|Default|SetGameStartDate (Math|DateTime|MakeDateTime (Class|KismetMathLibrary|GetYear (Variables|Default|GetGameStartDate)) (Class|KismetMathLibrary|GetMonth (Variables|Default|GetGameStartDate)) (Class|KismetMathLibrary|GetDay (Variables|Default|GetGameStartDate))))
  (if _returnvalue
    (CallFunction|LoadGame _array_element)))

(event EventOnUpdateCampaignDataMap
  (params (Struct :type Saveable%20Level%20Event%20Data%20Structure))
  (CallFunction|UpdateCampaignDataMap Struct))

(event EventOnCreateAutoSave
  (params (SaveName :type String))
  (CallFunction|SaveGame SaveName))

(event EventOnLoadfromAutoSave
  (bind (_returnvalue _array_element) (CallFunction|DoAutoSavesExist))
  (if _returnvalue
    (CallFunction|LoadGame _array_element)
    (Variables|Default|SetbWasSaveLoaded _returnvalue)
    (Game|OpenLevel(byName) (Utilities|String|StringToName (.SavedLevelName (Utilities|Struct|BreakSaveGameData (Variables|Default|GetSaveDataStruct)))))))

(event EventOnUpdateMissionDataMap
  (params (Struct :type Mission%20Level%20Stats%20Structure))
  (CallFunction|UpdateMissionDataMap Struct))

(event EventOnGameMissionSave
  (params (SlotName :type String))
  (CallFunction|SaveGameMission SlotName))

(fn SaveGame
  (params (SlotName :type String))
  (bind _returnvalue (Game|GetPlayerCharacter 0))
  (bind _asasylum_player_character (Utilities|Casting|CastToAsylumPlayerCharacter _returnvalue))
  (bind _returnvalue_2 (SaveGame|CreateSaveGameObject "/Game/Dynamic/Game/SaveGame/BP_AsylumSaveGame.BP_AsylumSaveGame_C"))
  (bind _output_get (Variables|Default|SetSaveGameInstance _returnvalue_2))
  (Utilities|FlowControl|Sequence
    (:then_0
      (if (not (CallFunction|GetMissionModeStatus))
        (bind _returnvalue_3 (Game|GetCurrentLevelName true))
        (Utilities|Struct|SetmembersinSaveGameData (Variables|Default|GetSaveDataStruct) _returnvalue_3)))
    (:then_1
      (bind _structout (Utilities|Struct|SetmembersinSaveGameData (Variables|Default|GetSaveDataStruct) (Math|DateTime|Now) (.CurrentCampaignModeAct (Utilities|Struct|BreakSaveGameData (Variables|Default|GetSaveDataStruct))) (.SavedGameDifficulty_Campaign (Utilities|Struct|BreakSaveGameData (Variables|Default|GetSaveDataStruct))) (.SavedGameDifficulty_Mission (Utilities|Struct|BreakSaveGameData (Variables|Default|GetSaveDataStruct))) (.PlayerCurrentPoints_Campaign (Utilities|Struct|BreakSaveGameData (Variables|Default|GetSaveDataStruct))) (.PlayerCurrentPoints_Mission (Utilities|Struct|BreakSaveGameData (Variables|Default|GetSaveDataStruct))) (.SaveableCampaignDataMap (Utilities|Struct|BreakSaveGameData (Variables|Default|GetSaveDataStruct))) (.SaveableMissionDataMap (Utilities|Struct|BreakSaveGameData (Variables|Default|GetSaveDataStruct))) (Transformation|GetActorTransform _returnvalue) (.PlayerLifetimePoints_Campaign (Utilities|Struct|BreakSaveGameData (Variables|Default|GetSaveDataStruct))) (.PlayerLifetimePoints_Mission (Utilities|Struct|BreakSaveGameData (Variables|Default|GetSaveDataStruct)))))
      (bind _output_get_2 (Variables|Default|SetSaveDataStruct _structout))
      (bind _output_get_3 (Variables|Default|SetSavedPlayerCharacterStats (Variables|/Script/HellsAsylum.AsylumStatsComponent|GetCharacterStatsDataStruct (Variables|/Script/HellsAsylum.AsylumPlayerCharacter|GetPlayerStatsComponent _asasylum_player_character))))
      (bind _output_get_4 (Variables|Default|SetSavedPlayerSuitStats (Variables|/Script/HellsAsylum.AsylumSuitComponent|GetSuitStatsData (Variables|/Script/HellsAsylum.AsylumPlayerCharacter|GetGoetheSuitComponent _asasylum_player_character))))
      (bind _output_get_5 (Variables|Default|SetSavedPlayerWeaponInventory (Variables|/Script/HellsAsylum.AsylumPlayerCharacter|GetPlayerWeaponInventory _asasylum_player_character)))
      (bind _output_get_6 (Variables|Default|SetSavedPlayerItemInventory (Variables|/Script/HellsAsylum.AsylumPlayerCharacter|GetItemInventory _asasylum_player_character)))
      (Default|SetSavedValues _output_get _output_get_3 _output_get_4 _output_get_2 _output_get_5 _output_get_6)
      (bind _returnvalue_4 (SaveGame|SaveGametoSlot _output_get SlotName))
      ;[1 1 1] Maybe insert a success sound
      (if _returnvalue_4
        (Audio|PlaySound2D "/Game/Static/ArtAssets/SFX/Interact/Success_2a.Success_2a" 1.0 1.0 0.0 0 0)
        (Variables|Default|SetCurrentSave SlotName)))))

(fn LoadGame
  (params (SlotName :type String))
  (bind _returnvalue (SaveGame|DoesSaveGameExist SlotName))
  (if _returnvalue
    (bind _returnvalue_2 (SaveGame|LoadGamefromSlot SlotName))
    (Variables|Default|SetCurrentSave SlotName)
    (bind _asbp_asylum_save_game (Utilities|Casting|CastToBP_AsylumSaveGame _returnvalue_2))
    (bind _structout (Utilities|Struct|SetmembersinGoetheSuitStatsData (Variables|Default|GetSavedPlayerSuitStats) (.Goethe%20Selected%20Main%20Ability (Default|GetSavedValues _asbp_asylum_save_game)) (.Goethe%20Suit%20Type (Default|GetSavedValues _asbp_asylum_save_game)) (.Goethe%20Passive%20Power%20One (Default|GetSavedValues _asbp_asylum_save_game)) (.Goethe%20Passive%20Power%20Two (Default|GetSavedValues _asbp_asylum_save_game)) (.Goethe%20Passive%20Power%20Boots (Default|GetSavedValues _asbp_asylum_save_game)) (.Goethe%20Passive%20Power%20Jet (Default|GetSavedValues _asbp_asylum_save_game)) (.Goethe%20Active%20Power%20One (Default|GetSavedValues _asbp_asylum_save_game)) (.Goethe%20Active%20Power%20Two (Default|GetSavedValues _asbp_asylum_save_game)) (.Goethe%20Active%20Power%20Three (Default|GetSavedValues _asbp_asylum_save_game)) (.Despair%20Orb%20Current%20Level (Default|GetSavedValues _asbp_asylum_save_game)) (.Despair%20Orb%20Max%20Level (Default|GetSavedValues _asbp_asylum_save_game)) (.Harmony%20Orb%20Current%20Level (Default|GetSavedValues _asbp_asylum_save_game)) (.Harmony%20Orb%20Max%20Level (Default|GetSavedValues _asbp_asylum_save_game)) (.Tesla%20Current%20Level (Default|GetSavedValues _asbp_asylum_save_game)) (.Tesla%20Max%20Level (Default|GetSavedValues _asbp_asylum_save_game)) (.Charger%20Current%20Level (Default|GetSavedValues _asbp_asylum_save_game)) (.Charger%20Max%20Level (Default|GetSavedValues _asbp_asylum_save_game)) (.Storm%20Current%20Level (Default|GetSavedValues _asbp_asylum_save_game)) (.Storm%20Max%20Level (Default|GetSavedValues _asbp_asylum_save_game)) (.Tractor%20Current%20Level (Default|GetSavedValues _asbp_asylum_save_game)) (.Tractor%20Max%20Level (Default|GetSavedValues _asbp_asylum_save_game)) (.Energy%20Drain%20Current%20Level (Default|GetSavedValues _asbp_asylum_save_game)) (.Energy%20Drain%20Max%20Level (Default|GetSavedValues _asbp_asylum_save_game)) (.Weapon%20Powers%20Current%20Level (Default|GetSavedValues _asbp_asylum_save_game)) (.Weapon%20Powers%20Max%20Level (Default|GetSavedValues _asbp_asylum_save_game)) (.Current%20Aragon%20Gauge (Default|GetSavedValues _asbp_asylum_save_game)) (.Max%20Aragon%20Gauge (Default|GetSavedValues _asbp_asylum_save_game)) (.Current%20Aragon%20Tanks (Default|GetSavedValues _asbp_asylum_save_game)) (.Aragon%20Regen%20Amount (Default|GetSavedValues _asbp_asylum_save_game)) (.Aragon%20Regen%20Speed (Default|GetSavedValues _asbp_asylum_save_game)) (.Max%20Aragon%20Tanks (Default|GetSavedValues _asbp_asylum_save_game)) (.Quicksilver%20Slow%20Down%20Amount (Default|GetSavedValues _asbp_asylum_save_game)) (.Quicksilver%20Player%20Speed (Default|GetSavedValues _asbp_asylum_save_game)) (.Quicksilver%20Consumption%20Rate (Default|GetSavedValues _asbp_asylum_save_game)) (.Overdrive%20Consumption%20Rate (Default|GetSavedValues _asbp_asylum_save_game)) (.Sacrifice%20Consumption%20Rate (Default|GetSavedValues _asbp_asylum_save_game)) (.Sacrifice%20Power%20Limit (Default|GetSavedValues _asbp_asylum_save_game)) (.Overdrive%20Speed%20Boost (Default|GetSavedValues _asbp_asylum_save_game)) (.Energy%20Drain%20Consumption%20Rate (Default|GetSavedValues _asbp_asylum_save_game)) (.Discord%20Ability%20Cooldown (Default|GetSavedValues _asbp_asylum_save_game)) (.Harmony%20Ability%20Cooldown (Default|GetSavedValues _asbp_asylum_save_game)) (.Snow%20Ability%20Cooldown (Default|GetSavedValues _asbp_asylum_save_game)) (.Charger%20Ability%20Cooldown (Default|GetSavedValues _asbp_asylum_save_game)) (.Drain%20Ability%20Cooldown (Default|GetSavedValues _asbp_asylum_save_game)) (.Tesla%20Ability%20Cooldown (Default|GetSavedValues _asbp_asylum_save_game)) (.Weapon%20Ability%20Cooldown (Default|GetSavedValues _asbp_asylum_save_game)) (.Scan%20Radius (Default|GetSavedValues _asbp_asylum_save_game)) (.Enemy%20Search%20Radius (Default|GetSavedValues _asbp_asylum_save_game))))
    (Variables|Default|SetSavedPlayerSuitStats _structout)
    (Variables|Default|SetSavedPlayerWeaponInventory (.Weapon%20Inventory (Default|GetSavedValues _asbp_asylum_save_game)))
    (Variables|Default|SetSavedPlayerItemInventory (.temInventory (Default|GetSavedValues _asbp_asylum_save_game)))
    (bind _structout_2 (Utilities|Struct|SetmembersinCharacterStatsData (Variables|Default|GetSavedPlayerCharacterStats) (.Has%20Shield (Default|GetSavedValues _asbp_asylum_save_game)) (.F%20Current%20Health (Default|GetSavedValues _asbp_asylum_save_game)) (.F%20Max%20Health (Default|GetSavedValues _asbp_asylum_save_game)) (.fCurrentStamina (Default|GetSavedValues _asbp_asylum_save_game)) (.fMaxStamina (Default|GetSavedValues _asbp_asylum_save_game)) (.F%20Current%20Shield (Default|GetSavedValues _asbp_asylum_save_game)) (.F%20Max%20Shield (Default|GetSavedValues _asbp_asylum_save_game)) (.I%20Current%20Character%20Level (Default|GetSavedValues _asbp_asylum_save_game)) (.I%20Max%20Character%20Level (Default|GetSavedValues _asbp_asylum_save_game)) (.F%20Movement%20Loudness (Default|GetSavedValues _asbp_asylum_save_game)) (.F%20Movement%20Max%20Range (Default|GetSavedValues _asbp_asylum_save_game)) (.F%20Crouch%20Movement%20Loudness (Default|GetSavedValues _asbp_asylum_save_game)) (.F%20Crouch%20Movement%20Max%20Range (Default|GetSavedValues _asbp_asylum_save_game)) (.F%20Fire%20Resist (Default|GetSavedValues _asbp_asylum_save_game)) (.F%20Ice%20Resist (Default|GetSavedValues _asbp_asylum_save_game)) (.F%20Shock%20Resist (Default|GetSavedValues _asbp_asylum_save_game))))
    (Variables|Default|SetSavedPlayerCharacterStats _structout_2)
    (bind _structout_3 (Utilities|Struct|SetmembersinSaveGameData (Variables|Default|GetSaveDataStruct) (.SaveDate (Default|GetSavedValues _asbp_asylum_save_game)) (.Current%20Campaign%20Mode%20Act (Default|GetSavedValues _asbp_asylum_save_game)) (.Saved%20Game%20Difficulty%20Campaign (Default|GetSavedValues _asbp_asylum_save_game)) (.Saved%20Game%20Difficulty%20Mission (Default|GetSavedValues _asbp_asylum_save_game)) (.Player%20Current%20Points%20Campaign (Default|GetSavedValues _asbp_asylum_save_game)) (.Player%20Current%20Points%20Mission (Default|GetSavedValues _asbp_asylum_save_game)) (.Saveable%20Campaign%20Data%20Map (Default|GetSavedValues _asbp_asylum_save_game)) (.Saveable%20Mission%20Data%20Map (Default|GetSavedValues _asbp_asylum_save_game)) (.Saved%20Level%20Name (Default|GetSavedValues _asbp_asylum_save_game)) (.Player%20Start%20Location (Default|GetSavedValues _asbp_asylum_save_game)) (.Player%20Save%20Checkpoint%20Location (Default|GetSavedValues _asbp_asylum_save_game)) (.Player%20Lifetime%20Points%20Campaign (Default|GetSavedValues _asbp_asylum_save_game)) (.Player%20Lifetime%20Points%20Mission (Default|GetSavedValues _asbp_asylum_save_game)) (.PlayerCurrentShardCount (Default|GetSavedValues _asbp_asylum_save_game)) (.PlayerTotalShardCount (Default|GetSavedValues _asbp_asylum_save_game))))
    (Variables|Default|SetSaveDataStruct _structout_3)))

(fn DoHardSavesExist
  (for _array_element (Variables|Default|GetHardSaveArray)
    (bind _returnvalue (SaveGame|DoesSaveGameExist _array_element))
    (return _returnvalue _array_element)))

(fn DoAutoSavesExist
  (for _array_element (Variables|Default|GetAutoSaveArray)
    (bind _returnvalue (SaveGame|DoesSaveGameExist _array_element))
    (return _returnvalue _array_element))
  (Development|PrintString "Completed Array"))

(fn UpdateCampaignDataMap
  (params (Value :type Saveable%20Level%20Event%20Data%20Structure%20%28by%20ref%29))
  (bind _returnvalue (Game|GetCurrentLevelName true))
  (Utilities|Map|Add (Utilities|Struct|BreakSaveGameData (Variables|Default|GetSaveDataStruct)) _returnvalue Value))

(fn UpdateMissionDataMap
  (params (Value :type Mission%20Level%20Stats%20Structure%20%28by%20ref%29))
  (bind _returnvalue (Game|GetCurrentLevelName true))
  (Utilities|Map|Add (Utilities|Struct|BreakSaveGameData (Variables|Default|GetSaveDataStruct)) _returnvalue Value))

(fn GetMissionLevelLastScore
  (params (Key :type String%20%28by%20ref%29))
  (bind _returnvalue (SaveGame|DoesSaveGameExist "MissionSave01"))
  (if _returnvalue
    (bind _returnvalue_2 (SaveGame|LoadGamefromSlot "MissionSave01"))
    (bind _asbp_asylum_save_game (Utilities|Casting|CastToBP_AsylumSaveGame _returnvalue_2))
    (if (.ReturnValue (Utilities|Map|Find (Utilities|Struct|BreakSaveGameData (Variables|/Game/Dynamic/Game/SaveGame/BP_AsylumSaveGame.BP_AsylumSaveGame_C|GetSG_ProfileDataStruct _asbp_asylum_save_game)) Key))
      (return (Utilities|Struct|BreakMissionLevelStats (.Value (Utilities|Map|Find (Utilities|Struct|BreakSaveGameData (Variables|/Game/Dynamic/Game/SaveGame/BP_AsylumSaveGame.BP_AsylumSaveGame_C|GetSG_ProfileDataStruct _asbp_asylum_save_game)) Key))))
      (else
        (return 0.0)))))

(fn SaveGameMission
  (params (SlotName :type String))
  (bind _returnvalue (Game|GetPlayerCharacter 0))
  (bind _asasylum_player_character (Utilities|Casting|CastToAsylumPlayerCharacter _returnvalue))
  (bind _returnvalue_2 (SaveGame|CreateSaveGameObject "/Game/Dynamic/Game/SaveGame/BP_AsylumSaveGame.BP_AsylumSaveGame_C"))
  (bind _output_get (Variables|Default|SetSaveGameInstance _returnvalue_2))
  (bind _output_get_2 (Variables|Default|SetCurrentMissionSave SlotName))
  (bind _returnvalue_3 (Game|GetCurrentLevelName true))
  (bind _structout (Utilities|Struct|SetmembersinSaveGameData (Variables|Default|GetSaveDataStruct) (.SaveDate (Utilities|Struct|BreakSaveGameData (Variables|Default|GetSaveDataStruct))) (.SavedGameDifficulty_Mission (Utilities|Struct|BreakSaveGameData (Variables|Default|GetSaveDataStruct))) (.PlayerCurrentPoints_Mission (Utilities|Struct|BreakSaveGameData (Variables|Default|GetSaveDataStruct))) (.SaveableMissionDataMap (Utilities|Struct|BreakSaveGameData (Variables|Default|GetSaveDataStruct))) _returnvalue_3 (.PlayerLifetimePoints_Mission (Utilities|Struct|BreakSaveGameData (Variables|Default|GetSaveDataStruct)))))
  (bind _output_get_3 (Variables|Default|SetSaveDataStruct _structout))
  (bind _output_get_4 (Variables|Default|SetSavedPlayerCharacterStats (Variables|/Script/HellsAsylum.AsylumStatsComponent|GetCharacterStatsDataStruct (Variables|/Script/HellsAsylum.AsylumPlayerCharacter|GetPlayerStatsComponent _asasylum_player_character))))
  (bind _output_get_5 (Variables|Default|SetSavedPlayerSuitStats (Variables|/Script/HellsAsylum.AsylumSuitComponent|GetSuitStatsData (Variables|/Script/HellsAsylum.AsylumPlayerCharacter|GetGoetheSuitComponent _asasylum_player_character))))
  (Default|SetSavedValues _output_get _output_get_4 _output_get_5 _output_get_3 (Variables|Default|GetSavedPlayerWeaponInventory) (Variables|Default|GetSavedPlayerItemInventory))
  (bind _returnvalue_4 (SaveGame|SaveGametoSlot _output_get _output_get_2))
  ;[1 1 1] Maybe insert a success sound
  (if _returnvalue_4
    (Audio|PlaySound2D "/Game/Static/ArtAssets/SFX/Interact/Success_2a.Success_2a" 1.0 1.0 0.0 0 0)))

(fn LoadGameMission
  (params (SlotName :type String))
  (bind _returnvalue (SaveGame|DoesSaveGameExist SlotName))
  (if _returnvalue
    (bind _returnvalue_2 (SaveGame|LoadGamefromSlot SlotName))
    (Variables|Default|SetCurrentMissionSave SlotName)
    (bind _asbp_asylum_save_game (Utilities|Casting|CastToBP_AsylumSaveGame _returnvalue_2))
    (bind _structout (Utilities|Struct|SetmembersinGoetheSuitStatsData (Variables|Default|GetSavedPlayerSuitStats) (.Goethe%20Selected%20Main%20Ability (Default|GetSavedValues _asbp_asylum_save_game)) (.Goethe%20Suit%20Type (Default|GetSavedValues _asbp_asylum_save_game)) (.Goethe%20Passive%20Power%20One (Default|GetSavedValues _asbp_asylum_save_game)) (.Goethe%20Passive%20Power%20Two (Default|GetSavedValues _asbp_asylum_save_game)) (.Goethe%20Passive%20Power%20Boots (Default|GetSavedValues _asbp_asylum_save_game)) (.Goethe%20Passive%20Power%20Jet (Default|GetSavedValues _asbp_asylum_save_game)) (.Goethe%20Active%20Power%20One (Default|GetSavedValues _asbp_asylum_save_game)) (.Goethe%20Active%20Power%20Two (Default|GetSavedValues _asbp_asylum_save_game)) (.Goethe%20Active%20Power%20Three (Default|GetSavedValues _asbp_asylum_save_game)) (.Despair%20Orb%20Current%20Level (Default|GetSavedValues _asbp_asylum_save_game)) (.Despair%20Orb%20Max%20Level (Default|GetSavedValues _asbp_asylum_save_game)) (.Harmony%20Orb%20Current%20Level (Default|GetSavedValues _asbp_asylum_save_game)) (.Harmony%20Orb%20Max%20Level (Default|GetSavedValues _asbp_asylum_save_game)) (.Tesla%20Current%20Level (Default|GetSavedValues _asbp_asylum_save_game)) (.Tesla%20Max%20Level (Default|GetSavedValues _asbp_asylum_save_game)) (.Charger%20Current%20Level (Default|GetSavedValues _asbp_asylum_save_game)) (.Charger%20Max%20Level (Default|GetSavedValues _asbp_asylum_save_game)) (.Storm%20Current%20Level (Default|GetSavedValues _asbp_asylum_save_game)) (.Storm%20Max%20Level (Default|GetSavedValues _asbp_asylum_save_game)) (.Tractor%20Current%20Level (Default|GetSavedValues _asbp_asylum_save_game)) (.Tractor%20Max%20Level (Default|GetSavedValues _asbp_asylum_save_game)) (.Energy%20Drain%20Current%20Level (Default|GetSavedValues _asbp_asylum_save_game)) (.Energy%20Drain%20Max%20Level (Default|GetSavedValues _asbp_asylum_save_game)) (.Weapon%20Powers%20Current%20Level (Default|GetSavedValues _asbp_asylum_save_game)) (.Weapon%20Powers%20Max%20Level (Default|GetSavedValues _asbp_asylum_save_game)) (.Current%20Aragon%20Gauge (Default|GetSavedValues _asbp_asylum_save_game)) (.Max%20Aragon%20Gauge (Default|GetSavedValues _asbp_asylum_save_game)) (.Current%20Aragon%20Tanks (Default|GetSavedValues _asbp_asylum_save_game)) (.Aragon%20Regen%20Amount (Default|GetSavedValues _asbp_asylum_save_game)) (.Aragon%20Regen%20Speed (Default|GetSavedValues _asbp_asylum_save_game)) (.Max%20Aragon%20Tanks (Default|GetSavedValues _asbp_asylum_save_game)) (.Quicksilver%20Slow%20Down%20Amount (Default|GetSavedValues _asbp_asylum_save_game)) (.Quicksilver%20Player%20Speed (Default|GetSavedValues _asbp_asylum_save_game)) (.Quicksilver%20Consumption%20Rate (Default|GetSavedValues _asbp_asylum_save_game)) (.Overdrive%20Consumption%20Rate (Default|GetSavedValues _asbp_asylum_save_game)) (.Sacrifice%20Consumption%20Rate (Default|GetSavedValues _asbp_asylum_save_game)) (.Sacrifice%20Power%20Limit (Default|GetSavedValues _asbp_asylum_save_game)) (.Overdrive%20Speed%20Boost (Default|GetSavedValues _asbp_asylum_save_game)) (.Energy%20Drain%20Consumption%20Rate (Default|GetSavedValues _asbp_asylum_save_game)) (.Discord%20Ability%20Cooldown (Default|GetSavedValues _asbp_asylum_save_game)) (.Harmony%20Ability%20Cooldown (Default|GetSavedValues _asbp_asylum_save_game)) (.Snow%20Ability%20Cooldown (Default|GetSavedValues _asbp_asylum_save_game)) (.Charger%20Ability%20Cooldown (Default|GetSavedValues _asbp_asylum_save_game)) (.Drain%20Ability%20Cooldown (Default|GetSavedValues _asbp_asylum_save_game)) (.Tesla%20Ability%20Cooldown (Default|GetSavedValues _asbp_asylum_save_game)) (.Weapon%20Ability%20Cooldown (Default|GetSavedValues _asbp_asylum_save_game)) (.Scan%20Radius (Default|GetSavedValues _asbp_asylum_save_game)) (.Enemy%20Search%20Radius (Default|GetSavedValues _asbp_asylum_save_game))))
    (Variables|Default|SetSavedPlayerSuitStats _structout)
    (Variables|Default|SetSavedPlayerWeaponInventory (.Weapon%20Inventory (Default|GetSavedValues _asbp_asylum_save_game)))
    (Variables|Default|SetSavedPlayerItemInventory (.temInventory (Default|GetSavedValues _asbp_asylum_save_game)))
    (bind _structout_2 (Utilities|Struct|SetmembersinCharacterStatsData (Variables|Default|GetSavedPlayerCharacterStats) (.Has%20Shield (Default|GetSavedValues _asbp_asylum_save_game)) (.F%20Current%20Health (Default|GetSavedValues _asbp_asylum_save_game)) (.F%20Max%20Health (Default|GetSavedValues _asbp_asylum_save_game)) (.F%20Current%20Shield (Default|GetSavedValues _asbp_asylum_save_game)) (.F%20Max%20Shield (Default|GetSavedValues _asbp_asylum_save_game)) (.I%20Current%20Character%20Level (Default|GetSavedValues _asbp_asylum_save_game)) (.I%20Max%20Character%20Level (Default|GetSavedValues _asbp_asylum_save_game)) (.F%20Movement%20Loudness (Default|GetSavedValues _asbp_asylum_save_game)) (.F%20Movement%20Max%20Range (Default|GetSavedValues _asbp_asylum_save_game)) (.F%20Crouch%20Movement%20Loudness (Default|GetSavedValues _asbp_asylum_save_game)) (.F%20Crouch%20Movement%20Max%20Range (Default|GetSavedValues _asbp_asylum_save_game)) (.F%20Fire%20Resist (Default|GetSavedValues _asbp_asylum_save_game)) (.F%20Ice%20Resist (Default|GetSavedValues _asbp_asylum_save_game)) (.F%20Shock%20Resist (Default|GetSavedValues _asbp_asylum_save_game))))
    (Variables|Default|SetSavedPlayerCharacterStats _structout_2)
    (bind _structout_3 (Utilities|Struct|SetmembersinSaveGameData (Variables|Default|GetSaveDataStruct) (.Current%20Campaign%20Mode%20Act (Default|GetSavedValues _asbp_asylum_save_game)) (.Saved%20Game%20Difficulty%20Campaign (Default|GetSavedValues _asbp_asylum_save_game)) (.Saved%20Game%20Difficulty%20Mission (Default|GetSavedValues _asbp_asylum_save_game)) (.Player%20Current%20Points%20Campaign (Default|GetSavedValues _asbp_asylum_save_game)) (.Player%20Current%20Points%20Mission (Default|GetSavedValues _asbp_asylum_save_game)) (.Saveable%20Campaign%20Data%20Map (Default|GetSavedValues _asbp_asylum_save_game)) (.Saveable%20Mission%20Data%20Map (Default|GetSavedValues _asbp_asylum_save_game)) (.Saved%20Level%20Name (Default|GetSavedValues _asbp_asylum_save_game)) (.Player%20Start%20Location (Default|GetSavedValues _asbp_asylum_save_game)) (.Player%20Save%20Checkpoint%20Location (Default|GetSavedValues _asbp_asylum_save_game)) (.Player%20Lifetime%20Points%20Campaign (Default|GetSavedValues _asbp_asylum_save_game)) (.Player%20Lifetime%20Points%20Mission (Default|GetSavedValues _asbp_asylum_save_game))))
    (Variables|Default|SetSaveDataStruct _structout_3)))

(fn FindMostRecentHardSave
  (bind (_returnvalue _array_element) (CallFunction|DoHardSavesExist))
  (if _returnvalue
    (bind _returnvalue_2 (SaveGame|LoadGamefromSlot _array_element))
    (if (>= (.SaveDate (Utilities|Struct|BreakSaveGameData (Variables|/Game/Dynamic/Game/SaveGame/BP_AsylumSaveGame.BP_AsylumSaveGame_C|GetSG_ProfileDataStruct (.AsBP%20Asylum%20Save%20Game (Utilities|Casting|CastToBP_AsylumSaveGame _returnvalue_2))))) (Variables|Default|GetGameStartDate))
      (return _array_element)
      (else
        (return "")))))
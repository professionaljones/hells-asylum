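; Campaign game state that holds the level's world music player and exposes events to control its playback.
; BeginPlay caches the BP_WorldMusicPlayer, spawning one only for invalid search results, and caches the elevator on the Oridona map.
; Events forward single-track play, repeat and restore-settings requests to that player.
; UpdateEnemyArray is an empty stub, with its array logic left disconnected.
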(event EventBeginPlay
  (bind _outactors (Actor|GetAllActorsOfClass "/Game/Dynamic/World/BP_WorldMusicPlayer.BP_WorldMusicPlayer_C"))
  (for _array_element _outactors
    (Utilities|IsValid _array_element
      (:Is%20Valid
        (Variables|Default|SetCurrentMusicPlayer _array_element))
      (:Is%20Not%20Valid
        (bind _returnvalue (Game|SpawnActorfromClass "/Game/Dynamic/World/BP_WorldMusicPlayer.BP_WorldMusicPlayer_C" (Math|Transform|MakeTransform "0, 0, 0") "Undefined" 0 0))
        (Variables|Default|SetCurrentMusicPlayer _returnvalue))))
  (bind _returnvalue_2 (Game|GetCurrentLevelName true))
  (if (Utilities|Enum|Equal(Enum) _returnvalue_2 "CM_Oridona_P")
    (bind _outactors_2 (Actor|GetAllActorsOfClass "/Game/Dynamic/LevelAssets/Elevators/BP_OridonaElevator.BP_OridonaElevator_C"))
    (for _array_element_2 _outactors_2
      (Utilities|IsValid _array_element_2
        (:Is%20Valid
          (Variables|Default|SetOriElevator _array_element_2))))))

(event EventUpdateEnemyArray
  (params (EnemyKilled :type Actor%20Object%20Reference)))

(event EventOnMusicPlayerPlayOneTrack
  (params (TrackDesiredAtIndex :type Integer))
  (bind _currentmusicplayer (Variables|Default|GetCurrentMusicPlayer))
  (Variables|/Game/Dynamic/World/BP_WorldMusicPlayer.BP_WorldMusicPlayer_C|SetSpecificTrackDesired _currentmusicplayer TrackDesiredAtIndex)
  (Variables|/Game/Dynamic/World/BP_WorldMusicPlayer.BP_WorldMusicPlayer_C|SetPlayOneTrack? _currentmusicplayer true)
  (Default|PlaybackHandler _currentmusicplayer))

(event EventOnMusicPlayerRestoreOriginalSettings
  (Default|RestoreOriginalSettings (Variables|Default|GetCurrentMusicPlayer)))

(event EventOnMusicPlayerRepeatOneTrack
  (params (TrackDesiredAtIndex :type Integer))
  (bind _currentmusicplayer (Variables|Default|GetCurrentMusicPlayer))
  (Variables|/Game/Dynamic/World/BP_WorldMusicPlayer.BP_WorldMusicPlayer_C|SetSpecificTrackDesired _currentmusicplayer TrackDesiredAtIndex)
  (Variables|/Game/Dynamic/World/BP_WorldMusicPlayer.BP_WorldMusicPlayer_C|SetPlayOneTrack? _currentmusicplayer true)
  (Variables|/Game/Dynamic/World/BP_WorldMusicPlayer.BP_WorldMusicPlayer_C|SetRepeatPlaylist? _currentmusicplayer true)
  (Default|PlaybackHandler _currentmusicplayer))

(fn ConstructionScript)
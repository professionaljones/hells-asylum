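; BP_EnemyReSpawner is a spawner that periodically creates an enemy at a random spawn point and displays a countdown.
; A looping one-second timer decrements the delay from its maximum, playing a countdown cue near zero.
; On expiry it calls SpawnEnemy, plays a portal sound and resets, with separate random picks for the validity check and spawn transform.
; Tick writes the remaining delay to a text render.
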(event Custom|RespawnEnemy
  (bind _spawnpoints (Variables|Default|GetSpawnPoints))
  (bind _returnvalue (Utilities|Array|Length _spawnpoints))
  (bind _returnvalue_2 (Math|Random|RandomInteger _returnvalue))
  (bind _output (Utilities|Array|Get(acopy) _spawnpoints _returnvalue_2))
  (bind _output_get (Variables|Default|SetTimerDelay (- (Variables|Default|GetTimerDelay) 1.0)))
  (Utilities|FlowControl|Sequence
    (:then_0
      (if (== (Variables|Default|GetTimerDelay) 5.0)
        (Audio|PlaySoundatLocation "/Game/Static/ArtAssets/SFX/Countdown_From_5_Cue.Countdown_From_5_Cue" (Transformation|GetActorLocation) "0, 0, 0" 1.0 1.0 0.0 0 0 0)))
    (:then_1
      (if (<= _output_get 0.0)
        (Utilities|IsValid _output
          (:Is%20Valid
            (CallFunction|SpawnEnemy (Transformation|GetActorTransform _output))
            (Variables|Default|SetTimerDelay (Variables|Default|GetMaxDelay))
            (Audio|PlaySoundatLocation "/Game/Static/ArtAssets/SFX/PM_FN_Spawns_Portals_Teleports_1_Cue.PM_FN_Spawns_Portals_Teleports_1_Cue" (Transformation|GetActorLocation) "0, 0, 0" 1.0 1.0 0.0 0 0 0)))))))

(event EventBeginPlay
  (|CallParentFunction)
  (Variables|Default|SetTimerDelay (Variables|Default|GetMaxDelay))
  (Utilities|Time|SetTimerbyEvent (EventDispatchers|CreateEvent :!event Custom|RespawnEnemy) 1.0 true))

(event Collision|EventActorBeginOverlap
  (params (OtherActor :type Actor%20Object%20Reference))
  (|CallParentFunction OtherActor) ; This node is disabled and will not be called.\nDrag off pins to build functionality.
)

(event EventTick
  (params (DeltaSeconds :type Float%20%28single-precision%29))
  (|CallParentFunction DeltaSeconds)
  (Rendering|Components|TextRender|SetText (Variables|Default|GetTextRender) (Utilities|Text|ToText(Float) (Variables|Default|GetTimerDelay) "HalfToEven")))

(fn ConstructionScript
  (|CallParentFunction))
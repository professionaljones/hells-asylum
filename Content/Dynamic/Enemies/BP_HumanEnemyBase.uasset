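; Base character for armed human AI enemies, handling stats, combat, damage reactions and death rewards for mission or campaign play.
; Setup loads stats from a DataTable, equips a difficulty-scaled weapon and starts a looping sphere-trace vision timer that feeds the AI controller's blackboard.
; Damage drains shield before health, with freeze and stun draining stamina to stun the enemy and incendiary applying burn ticks.
; Lock-on shows a stat-bar widget and toggles a Chameleon highlight actor.
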(event EventBeginPlay
  (CallFunction|AICharacterSetup)
  (Utilities|FlowControl|Delay 0.2)
  (Default|CallUpdateBlackboardData (Variables|Default|GetAICon_Reference))
  (Default|CallOnCharacterUpdate)
  (Audio|Components|Audio|Stop (Variables|Default|GetAudio))
  (Variables|/Game/Static/Chameleon/Chameleon.Chameleon_C|SetEnabled (Variables|Default|GetChamRef) false))

(event EventOnPlayerLockon
  (params (bIsLockedOn :type Boolean))
  (if bIsLockedOn
    (CallFunction|ShowWidget)
    (CallFunction|StartWidgetTimer)
    (Variables|/Game/Static/Chameleon/Chameleon.Chameleon_C|SetEnabled (Variables|Default|GetChamRef) true)
    (else
      (CallFunction|HideWidget)
      (Utilities|Time|ClearandInvalidateTimerbyHandle (Variables|Default|GetWidgetTimer))
      (Variables|/Game/Static/Chameleon/Chameleon.Chameleon_C|SetEnabled (Variables|Default|GetChamRef) false))))

(event EventOnStaminaDamage
  (params (DamageAmount :type Float%20%28single-precision%29))
  (bind _enemystatscomponent (Variables|Default|GetEnemyStatsComponent))
  (bind _characterstatsdatastruct (Variables|/Script/HellsAsylum.AsylumStatsComponent|GetCharacterStatsDataStruct _enemystatscomponent))
  (bind _fcurrentstamina (Utilities|Struct|BreakCharacterStatsData _characterstatsdatastruct))
  (Utilities|Struct|SetmembersinCharacterStatsData _characterstatsdatastruct (- _fcurrentstamina DamageAmount))
  (Default|CallOnCharacterUpdate)
  (if (<= _fcurrentstamina 0.0)
    (Class|AsylumCharacterInterface|OnStaminaDrained)))

(event EventOnAIFire
  (CallFunction|WeaponAttack)
  (Default|CallUpdateBlackboardData (Variables|Default|GetAICon_Reference)))

(event Game|Damage|EventAnyDamage
  (params (Damage :type Float%20%28single-precision%29) (DamageType :type Damage%20Type%20Object%20Reference) (InstigatedBy :type Controller%20Object%20Reference) (DamageCauser :type Actor%20Object%20Reference))
  (CallFunction|TakeDamage Damage DamageType))

(event EventOnAIReload
  (bind _currentequippedweapon (Variables|Default|GetCurrentEquippedWeapon))
  (Utilities|IsValid _currentequippedweapon
    (:Is%20Valid
      (Class|AsylumWeapon|StartReload _currentequippedweapon)
      (Default|CallUpdateBlackboardData (Variables|Default|GetAICon_Reference)))))

(event EventOnDifficultyModifier
  (params (GameDifficulty :type Float%20%28single-precision%29))
  (if (== GameDifficulty 1.0)
    (CallFunction|ModifiyDamageModifier 1.0)
    (elif (== GameDifficulty 2.0)
      (CallFunction|ModifiyDamageModifier 1.1)
      (elif (== GameDifficulty 3.0)
        (CallFunction|ModifiyDamageModifier 1.25)
        (elif (== GameDifficulty 4.0)
          (CallFunction|ModifiyDamageModifier 1.75)
          (elif (== GameDifficulty 5.0)
            (CallFunction|ModifiyDamageModifier 2.0)))))))

(event EventDestroyed
  (bind _currentequippedweapon (Variables|Default|GetCurrentEquippedWeapon))
  (bind _asbp_asylum_weapon_base (Utilities|Casting|CastToBP_AsylumWeaponBase _currentequippedweapon))
  (Utilities|IsValid _currentequippedweapon
    (:Is%20Valid
      (Default|ToggleCollider _asbp_asylum_weapon_base true)
      (Actor|SetLifeSpan _asbp_asylum_weapon_base 2.0))))

(event EventUnpossessed
  (params (OldController :type Controller%20Object%20Reference))
  (Utilities|FlowControl|Delay 2.0)
  (Actor|DestroyActor)
  (Utilities|Time|ClearandInvalidateTimerbyHandle (Variables|Default|GetVisionTimer)))

(event EventOnStaminaDrained
  (Class|BPIAIAnimation|OnAIStunned(Message) (Variables|Default|GetEnemyABP))
  (Pawn|Components|CharacterMovement|SetMovementMode (Variables|Character|GetCharacterMovement) "MOVE_None" 0)
  (Variables|/Script/HellsAsylum.AsylumWeapon|SetbCanWeaponFire (Variables|Default|GetCurrentEquippedWeapon) false)
  (Class|AsylumCharacterInterface|OnRecoverStamina)
  (AI|Navigation|StopMovement (AI|GetAIController self)))

(event EventOnRecoverStamina
  (bind _returnvalue (Utilities|Time|SetTimerbyEvent (EventDispatchers|CreateEvent :!event RecoverStamina) 1.0 true))
  (Variables|Default|SetStaminaRegenTimer _returnvalue))

(fn ConstructionScript)

(fn TakeDamage
  (params (DamageApplied :type Float%20%28single-precision%29) (DamageType :type Damage%20Type%20Object%20Reference))
  (bind _asasylum_damage_type (Utilities|Casting|CastToAsylumDamageType DamageType))
  (bind _enemystatscomponent (Variables|Default|GetEnemyStatsComponent))
  (bind _audio (Variables|Default|GetAudio))
  (bind _hitfx (Variables|/Script/HellsAsylum.AsylumDamageType|GetHitFX _asasylum_damage_type))
  (bind _characterstatsdatastruct (Variables|/Script/HellsAsylum.AsylumStatsComponent|GetCharacterStatsDataStruct _enemystatscomponent))
  (bind _characterstatsdatastruct_2 (Variables|/Script/HellsAsylum.AsylumStatsComponent|GetCharacterStatsDataStruct _enemystatscomponent))
  (bind _characterstatsdatastruct_3 (Variables|/Script/HellsAsylum.AsylumStatsComponent|GetCharacterStatsDataStruct _enemystatscomponent))
  (bind (_bhasshield _fcurrenthealth _fcurrentstamina _fmaxstamina _fcurrentshield) (Utilities|Struct|BreakCharacterStatsData _characterstatsdatastruct_2))
  (bind _fcurrentstamina_2 (Utilities|Struct|BreakCharacterStatsData _characterstatsdatastruct_3))
  (Utilities|FlowControl|Sequence
    (:then_0
      (if (!= (Variables|/Script/Engine.AudioComponent|GetSound _audio) "/Game/Static/ArtAssets/SFX/Character/Soldiers/SoundCue_SoldierDamage.SoundCue_SoldierDamage")
        (Audio|Components|Audio|SetSound _audio "/Game/Static/ArtAssets/SFX/Character/Soldiers/SoundCue_SoldierDamage.SoundCue_SoldierDamage")))
    (:then_1
      (Default|CallOnCharacterUpdate)
      (Audio|Components|Audio|Play (Variables|Default|GetAudio) 0.0)
      (Default|CallUpdateBlackboardData (Variables|Default|GetAICon_Reference))
      (if _bhasshield
        (bind _structout (Utilities|Struct|SetmembersinCharacterStatsData _characterstatsdatastruct_2 (- _fcurrentshield DamageApplied)))
        (Default|CallOnCharacterUpdate)
        (if (<= (.fCurrentShield (Utilities|Struct|BreakCharacterStatsData _structout)) 0.0)
          (Utilities|Struct|SetmembersinCharacterStatsData _structout false 0.0)
          (Default|CallOnCharacterUpdate))
        (else
          (bind _structout_2 (Utilities|Struct|SetmembersinCharacterStatsData _characterstatsdatastruct_2 (- _fcurrenthealth DamageApplied)))
          (if (<= (.fCurrentHealth (Utilities|Struct|BreakCharacterStatsData _structout_2)) 0.0)
            (Variables|/Script/HellsAsylum.AsylumStatsComponent|SetbIsCharacterDead _enemystatscomponent true)
            (Default|CallOnCharacterDeath)))))
    (:then_2
      (Utilities|IsValid _hitfx
        (:Is%20Valid
          (Effects|SpawnEmitterAttached _hitfx (Variables|Default|GetParticleSystem) "spine_02" "0, 0, 0" "0, 0, 0" "1.000000,1.000000,1.000000" "SnapToTarget"))))
    (:then_3
      (if (== DamageType "/Game/Dynamic/Weapons/DamageType/DT_Freeze.DT_Freeze")
        (Class|AsylumCharacterInterface|OnStaminaDamage (/ DamageApplied 2.0))
        (if (<= (Utilities|Struct|BreakCharacterStatsData _characterstatsdatastruct) 0.0)
          (Effects|SpawnEmitterAttached "/Game/Static/FXVarietyPack/Particles/P_ky_stunBall.P_ky_stunBall" (Variables|Default|GetParticleSystem) "spine_03" "0, 0, 0" "0, 0, 0" "1.000000,1.000000,1.000000" "SnapToTarget"))
        (elif (== DamageType "/Game/Dynamic/Weapons/DamageType/DT_Incendiary.DT_Incendiary")
          (CallFunction|Ignite)
          (elif (== DamageType "/Game/Dynamic/Weapons/DamageType/DT_Stun.DT_Stun")
            (Utilities|Struct|SetmembersinCharacterStatsData _characterstatsdatastruct (- _fcurrentstamina_2 DamageApplied))
            (if (<= _fcurrentstamina_2 0.0)
              (Class|AsylumCharacterInterface|OnStaminaDrained))))))))

(fn CharacterDeathEvent
  (bind _returnvalue (Game|GetGameInstance))
  (bind _returnvalue_2 (Transformation|GetActorLocation))
  (bind _enemystatscomponent (Variables|Default|GetEnemyStatsComponent))
  (bind _itemtospawn (Variables|Default|GetItemToSpawn))
  (bind _audio (Variables|Default|GetAudio))
  (bind _visiontimer (Variables|Default|GetVisionTimer))
  (bind _widgettimer (Variables|Default|GetWidgetTimer))
  (bind _currentequippedweapon (Variables|Default|GetCurrentEquippedWeapon))
  (bind _bischaracterdead (Variables|/Script/HellsAsylum.AsylumStatsComponent|GetbIsCharacterDead _enemystatscomponent))
  (if _bischaracterdead
    (Pawn|Components|CharacterMovement|SetMovementMode (Variables|Character|GetCharacterMovement) "MOVE_None" 0)
    (Class|Pawn|DetachfromControllerPendingDestroy)
    (Variables|Default|SetbCanBeDamaged false)
    (Class|BPIAIAnimation|OnAIDeath(Message) (Variables|Default|GetEnemyABP) _bischaracterdead)
    (Rendering|SetVisibility (Variables|Default|GetEnemyDataWidget) false false)
    (Audio|Components|Audio|SetSound _audio "/Game/Static/ArtAssets/SFX/Character/Soldiers/SoundCue_SoldierDeath.SoundCue_SoldierDeath")
    (Audio|Components|Audio|Play _audio 0.0)
    (Class|BPIAsylumGameInterface|OnSpawnPickup(Message) (Game|GetGameMode) _returnvalue_2)
    (Effects|SpawnEmitteratLocation "/Game/Static/VFX_Toolkit_V1/ParticleSystems/356Days/Par_DiamondSpawn_Enemy.Par_DiamondSpawn_Enemy" _returnvalue_2 "0, 0, 0" "3.000000,3.000000,3.000000")
    (Utilities|FlowControl|Sequence
      (:then_0
        (if (CallFunction|GetMissionModeStatus)
          (Class|AsylumDataCommInterface|OnMissionEnemyDeath(Message) _returnvalue (Variables|Default|Getf_MissionPointsToAdd))
          (Class|AsylumHUDInterface|UpdateEnemyArray(Message) (Game|GetGameState) self)
          (else
            (Class|AsylumDataCommInterface|OnCampaignEnemyDeath(Message) _returnvalue (Variables|Default|Getf_CampaignPointsToAdd))
            (Class|AsylumPlayerInterface|OnPlayerUpdateXP(Message) (Game|GetPlayerCharacter 0) (Variables|Default|GetPlayerExpMod))
            ;[1 1 1] This will spawn 'key' items
            (if (Utilities|IsValidClass _itemtospawn)
              (Class|BPIAsylumGameInterface|OnSpawnItemPickup(Message) (Game|GetGameMode) (Transformation|GetActorLocation) _itemtospawn)))))
      (:then_1
        (if (Class|KismetSystemLibrary|TimerExistsHandle _visiontimer)
          (Utilities|Time|ClearandInvalidateTimerbyHandle _visiontimer)))
      (:then_2
        (if (Class|KismetSystemLibrary|TimerExistsHandle _widgettimer)
          (Utilities|Time|ClearandInvalidateTimerbyHandle _widgettimer)))
      (:then_3
        (Utilities|IsValid _currentequippedweapon
          (:Is%20Valid
            (Default|ToggleCollider (.AsBP%20Asylum%20Weapon%20Base (Utilities|Casting|CastToBP_AsylumWeaponBase _currentequippedweapon)) true)))))))

(fn AICharacterSetup
  (EventDispatchers|BindEventtoOnCharacterDeath (EventDispatchers|CreateEvent :!event CharacterDeathEvent))
  (CallFunction|SetupAIConReference)
  (CallFunction|SetupABPReference)
  (CallFunction|SetupStatValues)
  (CallFunction|AIWeaponEquip)
  (CallFunction|SetupWidget)
  (bind _returnvalue (Utilities|Time|SetTimerbyEvent (EventDispatchers|CreateEvent :!event HumanoidVisionRaycast) 0.9 true))
  (Variables|Default|SetVisionTimer _returnvalue)
  (CallFunction|HideWidget)
  (bind _outactors (Actor|GetAllActorsOfClass "/Game/Static/Chameleon/Chameleon_CustDepth.Chameleon_CustDepth_C"))
  (bind _arrayelement (Utilities|Array|ReverseforEachLoop _outactors)
    (:LoopBody
      (Utilities|IsValid _arrayelement
        (:Is%20Valid
          (Variables|Default|SetChamRef _arrayelement))))))

(fn AIWeaponEquip
  (bind _ai_weapontoequip (Variables|Default|GetAI_WeaponToEquip))
  (if (Utilities|IsValidClass _ai_weapontoequip)
    (bind _returnvalue (Game|SpawnActorfromClass _ai_weapontoequip (Math|Transform|MakeTransform "0, 0, 0") "Undefined" self (Game|GetInstigator)))
    (bind _output_get (Variables|Default|SetCurrentEquippedWeapon _returnvalue))
    (Transformation|AttachComponentToComponent _output_get (Variables|Character|GetMesh) (Variables|/Script/HellsAsylum.AsylumWeapon|GetWeaponAttachPoint _output_get) "SnapToTarget" "SnapToTarget" "SnapToTarget" true)
    (Class|BPIAIAnimation|OnAIEquipNewWeapon(Message) (Variables|Default|GetEnemyABP) (Utilities|Struct|BreakWeaponStatsData (Variables|/Script/HellsAsylum.AsylumWeapon|GetWeaponStatsData _output_get)))
    (Class|AsylumCharacterInterface|OnDifficultyModifier (Math|Conversions|ToFloat(Integer) (CallFunction|GetDifficultyModfier)))))

(fn SetupWidget
  (bind _enemydatawidget (Variables|Default|GetEnemyDataWidget))
  (bind _output_get (Variables|Default|SetWidgetReference (.AsWBP%20AI%20Lock-%20on%20Data (Utilities|Casting|CastToWBP_AI_Lock-OnData (UserInterface|GetUserWidgetObject _enemydatawidget)))))
  (Rendering|Components|TextRender|SetText (Variables|/Game/Dynamic/UserInterface/WBPs/AI/WBP_AI_Lock-OnData.WBP_AI_Lock-OnData_C|GetEnemyNameText _output_get) (Utilities|Text|ToText(Name) (Variables|Default|GetCharacterName)))
  (Rendering|SetVisibility _enemydatawidget false false)
  (bind _returnvalue (Appearance|GetDynamicMaterial (Variables|/Game/Dynamic/UserInterface/WBPs/AI/WBP_AI_Lock-OnData.WBP_AI_Lock-OnData_C|GetHealthBar (Variables|Default|GetWidgetReference)) :!class /Script/UMG.Image))
  (Variables|Default|SetHealthBar_MI _returnvalue)
  (bind _returnvalue_2 (Appearance|GetDynamicMaterial (Variables|/Game/Dynamic/UserInterface/WBPs/AI/WBP_AI_Lock-OnData.WBP_AI_Lock-OnData_C|GetShieldBar (Variables|Default|GetWidgetReference)) :!class /Script/UMG.Image))
  (Variables|Default|SetShieldBar_MI _returnvalue_2)
  (bind _returnvalue_3 (Appearance|GetDynamicMaterial (Variables|/Game/Dynamic/UserInterface/WBPs/AI/WBP_AI_Lock-OnData.WBP_AI_Lock-OnData_C|GetStaminaBar (Variables|Default|GetWidgetReference)) :!class /Script/UMG.Image))
  (Variables|Default|SetStaminaBar_MI _returnvalue_3)
  (EventDispatchers|BindEventtoOnCharacterUpdate (EventDispatchers|CreateEvent :!event UpdateWidget)))

(fn HumanoidVisionRaycast
  (bind _aicon_reference (Variables|Default|GetAICon_Reference))
  (bind _scene (Variables|Default|GetScene))
  (bind _returnvalue (Transformation|GetWorldLocation _scene))
  (if (not (Variables|/Script/HellsAsylum.AsylumStatsComponent|GetbIsCharacterDead (Variables|Default|GetEnemyStatsComponent)))
    (bind _outhit (Collision|SphereTraceForObjects _returnvalue (+ _returnvalue (* (Math|Vector|GetForwardVector _scene) (Variables|Default|GetMaxVisionDistance))) (Variables|Default|GetVisionFOV) (Utilities|Array|MakeArray "ObjectTypeQuery2" "ObjectTypeQuery9") true (Utilities|Array|MakeArray self) "None" true "(R=1.000000,G=0.000000,B=0.000000,A=1.000000)" "(R=0.000000,G=1.000000,B=0.000000,A=1.000000)" 2.0))
    (if (and (.bBlockingHit (Collision|BreakHitResult _outhit)) (Utilities|DoesObjectImplementInterface (.HitActor (Collision|BreakHitResult _outhit)) "/Script/HellsAsylum.AsylumPlayerInterface"))
      (Utilities|IsValid (.HitActor (Collision|BreakHitResult _outhit))
        (:Is%20Valid
          (AI|Components|Blackboard|SetValueasObject (Variables|/Script/AIModule.AIController|GetBlackboard _aicon_reference) (Variables|/Script/HellsAsylum.AsylumAIController|GetAttackerKey _aicon_reference) (.HitActor (Collision|BreakHitResult _outhit)))
          (Default|CallUpdateBlackboardData _aicon_reference))))))

(fn SetupStatValues
  (bind _enemystatscomponent (Variables|Default|GetEnemyStatsComponent))
  (bind _returnvalue (Utilities|GetDataTableRow (Variables|/Script/HellsAsylum.AsylumStatsComponent|GetCharacterDataTable _enemystatscomponent) "NG")
    (:then
      (Utilities|Struct|SetmembersinCharacterStatsData (Variables|/Script/HellsAsylum.AsylumStatsComponent|GetCharacterStatsDataStruct _enemystatscomponent) (.bHasShield (Utilities|Struct|BreakCharacterStatsData _returnvalue)) (.fCurrentHealth (Utilities|Struct|BreakCharacterStatsData _returnvalue)) (.fMaxHealth (Utilities|Struct|BreakCharacterStatsData _returnvalue)) (.fCurrentStamina (Utilities|Struct|BreakCharacterStatsData _returnvalue)) (.fMaxStamina (Utilities|Struct|BreakCharacterStatsData _returnvalue)) (.fCurrentShield (Utilities|Struct|BreakCharacterStatsData _returnvalue)) (.fMaxShield (Utilities|Struct|BreakCharacterStatsData _returnvalue)) (.iCurrentCharacterLevel (Utilities|Struct|BreakCharacterStatsData _returnvalue)) (.iMaxCharacterLevel (Utilities|Struct|BreakCharacterStatsData _returnvalue)) (.fMovementLoudness (Utilities|Struct|BreakCharacterStatsData _returnvalue)) (.fMovementMaxRange (Utilities|Struct|BreakCharacterStatsData _returnvalue)) (.fCrouchMovementLoudness (Utilities|Struct|BreakCharacterStatsData _returnvalue)) (.fCrouchMovementMaxRange (Utilities|Struct|BreakCharacterStatsData _returnvalue)) (.fFireResist (Utilities|Struct|BreakCharacterStatsData _returnvalue)) (.fIceResist (Utilities|Struct|BreakCharacterStatsData _returnvalue)) (.fShockResist (Utilities|Struct|BreakCharacterStatsData _returnvalue))))))

(fn SetupABPReference
  (Variables|Default|SetEnemyABP (Components|SkeletalMesh|GetAnimInstance (Variables|Character|GetMesh))))

(fn SetupAIConReference
  (Variables|Default|SetAICon_Reference (.AsBP%20AICon%20Humanoid%20Base (Utilities|Casting|CastToBP_AICon_HumanoidBase (AI|GetAIController self)))))

(fn KeepWidgetinView
  (bind _enemydatawidget (Variables|Default|GetEnemyDataWidget))
  (Transformation|SetWorldRotation _enemydatawidget (Math|Rotator|FindLookatRotation (Transformation|GetWorldLocation _enemydatawidget) (Camera|GetCameraLocation (Game|GetPlayerCameraManager 0))) false false))

(fn HideWidget
  (Rendering|SetVisibility (Variables|Default|GetEnemyDataWidget) false false))

(fn StartWidgetTimer
  (bind _returnvalue (Utilities|Time|SetTimerbyEvent (EventDispatchers|CreateEvent :!event KeepWidgetinView) 0.05 true))
  (Variables|Default|SetWidgetTimer _returnvalue))

(fn ShowWidget
  (Rendering|SetVisibility (Variables|Default|GetEnemyDataWidget) true false))

(fn UpdateWidget
  (bind _shieldbar_mi (Variables|Default|GetShieldBar_MI))
  (bind _widgetreference (Variables|Default|GetWidgetReference))
  (bind _enemystatscomponent (Variables|Default|GetEnemyStatsComponent))
  (bind _shieldbar (Variables|/Game/Dynamic/UserInterface/WBPs/AI/WBP_AI_Lock-OnData.WBP_AI_Lock-OnData_C|GetShieldBar _widgetreference))
  (bind _characterstatsdatastruct (Variables|/Script/HellsAsylum.AsylumStatsComponent|GetCharacterStatsDataStruct _enemystatscomponent))
  (bind (_bhasshield _fcurrenthealth _fmaxhealth _fcurrentstamina _fmaxstamina _fcurrentshield _fmaxshield) (Utilities|Struct|BreakCharacterStatsData _characterstatsdatastruct))
  (if (not (Variables|/Script/HellsAsylum.AsylumStatsComponent|GetbIsCharacterDead _enemystatscomponent))
    (Rendering|Material|SetScalarParameterValue (Variables|Default|GetHealthBar_MI) "Progress" (/ _fcurrenthealth _fmaxhealth) :!class /Script/Engine.MaterialInstanceDynamic)
    (Rendering|Components|TextRender|SetText (Variables|/Game/Dynamic/UserInterface/WBPs/AI/WBP_AI_Lock-OnData.WBP_AI_Lock-OnData_C|GetHealthText _widgetreference) (Utilities|Text|ToText(Float) _fcurrenthealth "HalfToEven"))
    (Utilities|FlowControl|Sequence
      (:then_0
        (Rendering|Material|SetScalarParameterValue (Variables|Default|GetStaminaBar_MI) "Progress" (/ _fcurrentstamina _fmaxstamina) :!class /Script/Engine.MaterialInstanceDynamic))
      (:then_1
        (if _bhasshield
          (Rendering|Material|SetScalarParameterValue _shieldbar_mi "Progress" (/ _fcurrentshield _fmaxshield) :!class /Script/Engine.MaterialInstanceDynamic)
          (if (not (Widget|IsVisible _shieldbar))
            (Widget|SetVisibility _shieldbar "HitTestInvisible"))
          (else
            (Rendering|Material|SetScalarParameterValue _shieldbar_mi "Progress" 0.0 :!class /Script/Engine.MaterialInstanceDynamic)
            (Widget|SetVisibility _shieldbar "Hidden")))))))

(fn WeaponAttack
  (bind _currentequippedweapon (Variables|Default|GetCurrentEquippedWeapon))
  (bind _currentequippedweapon_2 (Variables|Default|GetCurrentEquippedWeapon))
  (bind _weaponstatsdata (Variables|/Script/HellsAsylum.AsylumWeapon|GetWeaponStatsData _currentequippedweapon))
  (bind _rootcomponent (Variables|/Script/Engine.Actor|GetRootComponent _currentequippedweapon_2))
  (bind (_or_weapondamagetype _c_weapondamagetype _currentmagazineammo _ammoconsumptionamount _maxmagazineammo _damageamountsum) (Utilities|Struct|BreakWeaponStatsData _weaponstatsdata))
  (bind _returnvalue (Transformation|GetWorldLocation _rootcomponent))
  (bind _outhit (Collision|LineTraceForObjects _returnvalue (+ _returnvalue (* (Math|Vector|GetForwardVector (Variables|/Script/Engine.Actor|GetRootComponent _currentequippedweapon_2)) (Variables|Default|GetMaxVisionDistance))) (Utilities|Array|MakeArray "ObjectTypeQuery9") false 0 "None"))
  (if (and (.bBlockingHit (Collision|BreakHitResult _outhit)) (Utilities|DoesObjectImplementInterface (.HitActor (Collision|BreakHitResult _outhit)) "/Script/HellsAsylum.AsylumPlayerInterface"))
    (Game|Damage|ApplyPointDamage (.HitActor (Collision|BreakHitResult _outhit)) _damageamountsum (.ImpactPoint (Collision|BreakHitResult _outhit)) _outhit (Variables|Default|GetAICon_Reference) _currentequippedweapon)
    (Utilities|Struct|SetmembersinWeaponStatsData _weaponstatsdata (- _currentmagazineammo (Math|Conversions|ToFloat(Integer) _ammoconsumptionamount)))
    (Class|AsylumWeapon|FinishFire _currentequippedweapon)))

(fn ModifiyDamageModifier
  (params (Damage%20Modifier%20Amount :type Float%20%28single-precision%29))
  (bind _currentequippedweapon (Variables|Default|GetCurrentEquippedWeapon))
  (bind _weaponstatsdata (Variables|/Script/HellsAsylum.AsylumWeapon|GetWeaponStatsData _currentequippedweapon))
  (bind (_or_weapondamagetype _c_weapondamagetype _maxmagazineammo _basedamageamount _damagemultiplieramount) (Utilities|Struct|BreakWeaponStatsData _weaponstatsdata))
  (Utilities|IsValid _currentequippedweapon
    (:Is%20Valid
      (Utilities|Struct|SetmembersinWeaponStatsData _weaponstatsdata Damage%20Modifier%20Amount (CallFunction|DamageCalculation _basedamageamount _damagemultiplieramount Damage%20Modifier%20Amount)))))

(fn RecoverStamina
  (bind _enemystatscomponent (Variables|Default|GetEnemyStatsComponent))
  (bind _characterstatsdatastruct (Variables|/Script/HellsAsylum.AsylumStatsComponent|GetCharacterStatsDataStruct _enemystatscomponent))
  (bind (_fcurrentstamina _fmaxstamina) (Utilities|Struct|BreakCharacterStatsData _characterstatsdatastruct))
  (if (<= _fcurrentstamina _fmaxstamina)
    (bind _structout (Utilities|Struct|SetmembersinCharacterStatsData _characterstatsdatastruct (+ _fcurrentstamina 2.0)))
    (if (>= (.fCurrentStamina (Utilities|Struct|BreakCharacterStatsData _structout)) (.fMaxStamina (Utilities|Struct|BreakCharacterStatsData _structout)))
      (Utilities|Struct|SetmembersinCharacterStatsData _structout (.fMaxStamina (Utilities|Struct|BreakCharacterStatsData _structout)))
      (Utilities|Time|ClearandInvalidateTimerbyHandle (Variables|Default|GetStaminaRegenTimer))
      (Pawn|Components|CharacterMovement|SetMovementMode (Variables|Character|GetCharacterMovement) "MOVE_Walking" 0)
      (Variables|/Script/HellsAsylum.AsylumWeapon|SetbCanWeaponFire (Variables|Default|GetCurrentEquippedWeapon) true))))

(fn Ignite
  (if (not (Variables|Default|GetbIsOnFire?))
    (Effects|SpawnEmitterAttached "/Game/Static/M5VFXVOL2/Particles/Fire/Fire_01.Fire_01" (Variables|Default|GetParticleSystem) "spine_03" "0, 0, 0" "0, 0, 0" "1.000000,1.000000,1.000000" "SnapToTarget")
    (Utilities|Time|SetTimerbyEvent (EventDispatchers|CreateEvent :!event TakeFireDamage) 3.0 true)
    (Variables|Default|SetbIsOnFire? true)))

(fn TakeFireDamage
  (Game|Damage|ApplyDamage self 3.0 (Game|GetInstigatorController) (Game|GetInstigator) "/Game/Dynamic/Weapons/DamageType/DT_Incendiary.DT_Incendiary_C"))
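; Enemy turret that turns to face the player and is destroyed when its health runs out; it has no firing logic.
; A looping timer is set on BeginPlay, and Raycaster sphere-traces forward for an actor implementing AsylumPlayerInterface.
; On a hit, mesh yaw is set by interpolating from the AI controller's control rotation toward player character 0.
; Damage reduces health stored in the AsylumStats component.
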(event Custom|Raycaster
  (bind _scene (Variables|Default|GetScene))
  (bind _staticmesh (Variables|Default|GetStaticMesh))
  (bind _returnvalue (Transformation|GetWorldLocation _scene))
  (bind _returnvalue_2 (Transformation|GetWorldRotation _staticmesh))
  (bind (_roll _pitch) (Math|Rotator|BreakRotator _returnvalue_2))
  (if (not (Variables|/Script/HellsAsylum.AsylumStatsComponent|GetbIsCharacterDead (Variables|Default|GetAsylumStats)))
    (bind _outhit (Collision|SphereTraceForObjects _returnvalue (+ _returnvalue (* (Math|Vector|GetForwardVector _scene) 5e+03)) 3.6e+02 (Utilities|Array|MakeArray "ObjectTypeQuery9") true (Utilities|Array|MakeArray self) "ForOneFrame" true "(R=1.000000,G=0.000000,B=0.000000,A=1.000000)" "(R=0.000000,G=1.000000,B=0.000000,A=1.000000)" 2.0))
    (if (and (.bBlockingHit (Collision|BreakHitResult _outhit)) (Utilities|DoesObjectImplementInterface (.HitActor (Collision|BreakHitResult _outhit)) "/Script/HellsAsylum.AsylumPlayerInterface"))
      (Transformation|SetWorldRotation (Variables|Default|GetStaticMesh) (Math|Rotator|MakeRotator _roll _pitch (.Yaw (Math|Rotator|BreakRotator (Math|Interpolation|RInterpTo (Pawn|GetControlRotation (AI|GetAIController self) :!class /Script/Engine.Controller) (Math|Rotator|FindLookatRotation (Transformation|GetActorLocation) (Transformation|GetActorLocation (Game|GetPlayerCharacter 0))) (Utilities|Time|GetWorldDeltaSeconds) 1e+01)))) false false))))

(event EventBeginPlay
  (Utilities|Time|SetTimerbyEvent (EventDispatchers|CreateEvent :!event Custom|Raycaster) 0.5 true)
  (Utilities|Struct|SetmembersinCharacterStatsData (Variables|/Script/HellsAsylum.AsylumStatsComponent|GetCharacterStatsDataStruct (Variables|Default|GetAsylumStats)) 2e+02))

(event Game|Damage|EventAnyDamage
  (params (Damage :type Float%20%28single-precision%29) (DamageType :type Damage%20Type%20Object%20Reference) (InstigatedBy :type Controller%20Object%20Reference) (DamageCauser :type Actor%20Object%20Reference))
  (bind _asylumstats (Variables|Default|GetAsylumStats))
  (bind _characterstatsdatastruct (Variables|/Script/HellsAsylum.AsylumStatsComponent|GetCharacterStatsDataStruct _asylumstats))
  (bind _structout (Utilities|Struct|SetmembersinCharacterStatsData _characterstatsdatastruct (- (Utilities|Struct|BreakCharacterStatsData _characterstatsdatastruct) Damage)))
  (if (<= (Utilities|Struct|BreakCharacterStatsData _structout) 0.0)
    (Actor|DestroyActor)))

(fn ConstructionScript)
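; World music player Blueprint that plays tracks from an indexed playlist map through a music component.
; PlaybackHandler starts playback on BeginPlay, choosing a specific, shuffled or sequential track, with optional fades.
; When audio finishes, it repeats the playlist, stops or fades a single track, or advances the index, optionally fading out at list end.
; Startup caches repeat, one-track, shuffle and fade-in flags for RestoreOriginalSettings, which only partially restores them.
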(event OnAudioFinished(MusicComponent)
  (if (Variables|Settings|GetRepeatPlaylist?)
    (CallFunction|RepeatPlaylist)
    (elif (Variables|Settings|GetPlayOneTrack?)
      (if (Variables|Settings|GetShouldFadeOut?)
        (CallFunction|FadeOutMusic)
        (else
          (Audio|Components|Audio|Stop (Variables|Default|GetMusicComponent))))
      (else
        (CallFunction|IncrementPlayIndex)
        (CallFunction|PlaybackHandler)))))

(event EventBeginPlay
  (CallFunction|PlaybackHandler)
  (CallFunction|FadeOutatEnd)
  (CallFunction|CacheSettingsonStart))

(fn ConstructionScript)

(fn FadeinPlaylist
  (params (FadeInDuration :type Float%20%28single-precision%29) (FadeVolumeLevel :type Float%20%28single-precision%29))
  (bind _musiccomponent (Variables|Default|GetMusicComponent))
  (Audio|Components|Audio|SetSound _musiccomponent (CallFunction|FindTracktoPlay))
  (Audio|Components|Audio|FadeIn _musiccomponent FadeInDuration FadeVolumeLevel 0.0 :!class /Script/Engine.AudioComponent)
  (Utilities|IsValid (Variables|/Script/Engine.AudioComponent|GetSound _musiccomponent)))

(fn FindTracktoPlay
  (bind _musicplaylistmap (Variables|Playlists|GetMusicPlaylistMap))
  (bind _desiredsongindex (Variables|Playlists|GetDesiredSongIndex))
  (bind (_value _returnvalue) (Utilities|Map|Find _musicplaylistmap _desiredsongindex))
  (bind _tracktoplay (Utilities|Struct|BreakBPS_BGM_Object _value))
  (if _returnvalue
    (Variables|Default|SetCurrentTrack _tracktoplay)
    (return _tracktoplay)))

(fn ShufflePlaylist
  (Variables|Playlists|SetDesiredSongIndex (Math|Random|RandomInteger (Utilities|Map|Length (Variables|Playlists|GetMusicPlaylistMap)))))

(fn PlaybackHandler
  (bind _musiccomponent (Variables|Default|GetMusicComponent))
  (bind _musiccomponent_2 (Variables|Default|GetMusicComponent))
  (bind _fadein_duration (Variables|Settings|Audio|GetFadein_Duration))
  (bind _fadein_volumelevel (Variables|Settings|Audio|GetFadein_VolumeLevel))
  (CallFunction|CheckPlaylistLength)
  (CallFunction|FadeOutatEnd)
  (if (Variables|Settings|GetShouldFadeOut?)
    (CallFunction|FadeOutMusic)
    (elif (Variables|Settings|GetPlayOneTrack?)
      (Audio|Components|Audio|SetSound _musiccomponent_2 (CallFunction|FindSpecificTracktoPlay (Variables|Playlists|GetSpecificTrackDesired)))
      (if (Variables|Settings|GetShouldFadeIn?)
        (Audio|Components|Audio|FadeIn _musiccomponent_2 _fadein_duration _fadein_volumelevel 0.0 :!class /Script/Engine.AudioComponent)
        (else
          (Audio|Components|Audio|Play _musiccomponent_2 0.0)))
      (elif (Variables|Settings|GetShuffle?)
        (CallFunction|ShufflePlaylist)
        (if (Variables|Settings|GetShouldFadeIn?)
          (CallFunction|FadeinPlaylist _fadein_duration _fadein_volumelevel)
          (else
            (Audio|Components|Audio|Play _musiccomponent 0.0)))
        (elif (Variables|Settings|GetShouldFadeIn?)
          (CallFunction|FadeinPlaylist _fadein_duration _fadein_volumelevel)
          (else
            (Audio|Components|Audio|SetSound _musiccomponent (CallFunction|FindTracktoPlay))
            (Audio|Components|Audio|Play _musiccomponent 0.0)))))))

(fn ReachedEndOfPlaylist?
  (return (>= (Variables|Playlists|GetDesiredSongIndex) (Utilities|Map|Length (Variables|Playlists|GetMusicPlaylistMap)))))

(fn IncrementPlayIndex
  (bind _result (Math|Integer|IncrementInt (Variables|Playlists|GetDesiredSongIndex))
    (:%20%20
      (Variables|Playlists|SetDesiredSongIndex _result))))

(fn FadeOutMusic
  (Audio|Components|Audio|FadeOut (Variables|Default|GetMusicComponent) (Variables|Settings|Audio|GetFadeOut_Duration) (Variables|Settings|Audio|GetFadeOut_VolumeLevel) :!class /Script/Engine.AudioComponent))

(fn FadeOutatEnd
  (if (Variables|Settings|GetFadeAtEndOfList?)
    (if (CallFunction|ReachedEndOfPlaylist?)
      (bind _output_get (Variables|Settings|SetShouldFadeOut? true))
      (if _output_get
        (CallFunction|FadeOutMusic)))))

(fn CheckPlaylistLength
  (if (<= (Utilities|Map|Length (Variables|Playlists|GetMusicPlaylistMap)) 0)
    (Development|PrintString "The playlist is empty!" true true "(R=1.000000,G=0.003975,B=0.000000,A=1.000000)" 99999.0)))

(fn RepeatPlaylist
  (if (CallFunction|ReachedEndOfPlaylist?)
    (Variables|Playlists|SetDesiredSongIndex 1)
    (CallFunction|PlaybackHandler)
    (else
      (CallFunction|IncrementPlayIndex)
      (CallFunction|PlaybackHandler))))

(fn FindSpecificTracktoPlay
  (params (Key :type Integer%20%28by%20ref%29))
  (bind _musicplaylistmap (Variables|Playlists|GetMusicPlaylistMap))
  (bind (_value _returnvalue) (Utilities|Map|Find _musicplaylistmap Key))
  (bind _tracktoplay (Utilities|Struct|BreakBPS_BGM_Object _value))
  (if _returnvalue
    (Variables|Default|SetCurrentTrack _tracktoplay)
    (return _tracktoplay)))

(fn CacheSettingsonStart
  (Utilities|FlowControl|Sequence
    (:then_0
      (if (Variables|Settings|GetRepeatPlaylist?)
        (Variables|Settings|Original|SetS_Repeat? true)
        (else
          (Variables|Settings|Original|SetS_Repeat? false))))
    (:then_1
      (if (Variables|Settings|GetPlayOneTrack?)
        (Variables|Settings|Original|SetS_OneTrack? true)
        (else
          (Variables|Settings|Original|SetS_OneTrack? false))))
    (:then_2
      (if (Variables|Settings|GetShuffle?)
        (Variables|Settings|Original|SetS_Shuffle? true)
        (else
          (Variables|Settings|Original|SetS_Shuffle? false))))
    (:then_3
      (if (Variables|Settings|GetShouldFadeIn?)
        (Variables|Settings|Original|SetS_FadeIn? true)
        (else
          (Variables|Settings|Original|SetS_FadeIn? false))))))

(fn RestoreOriginalSettings
  (Utilities|FlowControl|Sequence
    (:then_0
      (if (Variables|Settings|Original|GetS_Repeat?)
        (Variables|Settings|SetRepeatPlaylist? true)
        (else
          (Variables|Settings|SetRepeatPlaylist? false))))
    (:then_1
      (if (Variables|Settings|Original|GetS_Shuffle?)
        (Variables|Settings|SetShuffle? true)
        (else
          (Variables|Settings|SetShuffle? false))))
    (:then_2
      (if (Variables|Settings|Original|GetS_FadeIn?)
        (Variables|Settings|Original|SetS_FadeIn? true)
        (else
          (Variables|Settings|Original|SetS_FadeIn? false))))
    (:then_3
      (if (Variables|Settings|Original|GetS_OneTrack?)
        (Variables|Settings|Original|SetS_OneTrack? true)
        (else
          (Variables|Settings|Original|SetS_OneTrack? false)))))
  (CallFunction|PlaybackHandler))
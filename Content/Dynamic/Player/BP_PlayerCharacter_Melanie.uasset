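; Player character Blueprint for Melanie, handling stat setup, weapon slots, attacking and damage.
; BeginPlay configures lock-on and loads character and Goethe suit stats from a save or difficulty-keyed DataTable rows.
; Inventory weapons spawn hidden on mesh sockets in three slots; equipping reveals one, attacking messages it, and both notify the anim Blueprint.
; Damage drains the shield, otherwise health, firing the death dispatcher at zero.
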(event EventBeginPlay
  (CallFunction|CharacterSetup))

(event EventOnWeaponPickup
  (params (WeaponToAdd :type Asylum%20Weapon%20Class%20Reference) (KeyToOccupy :type Integer))
  (CallFunction|AddWeapon KeyToOccupy WeaponToAdd))

(event Game|Damage|EventAnyDamage
  (params (Damage :type Float%20%28single-precision%29) (DamageType :type Damage%20Type%20Object%20Reference) (InstigatedBy :type Controller%20Object%20Reference) (DamageCauser :type Actor%20Object%20Reference))
  (CallFunction|TakeDamage Damage))

(event Input|ActionEvents|InputActionAttack
  (params (Key :type Key%20Structure))
  (:Pressed
    (CallFunction|WeaponAttack))
  (:Released
    (CallFunction|WeaponStopAttack)))

(event Input|ActionEvents|InputActionSelectPrimaryWeaponOne
  (params (Key :type Key%20Structure))
  (:Pressed
    (CallFunction|EquipWeapon (Variables|Default|GetWeaponSlotOne))))

(event Input|ActionEvents|InputActionSelectSecondaryWeapon
  (params (Key :type Key%20Structure))
  (:Pressed
    (CallFunction|EquipWeapon (Variables|Default|GetWeaponSlotTwo))))

(event Input|ActionEvents|InputActionSelectSecondaryWeapon
  (params (Key :type Key%20Structure))
  (:Pressed
    (CallFunction|EquipWeapon (Variables|Default|GetWeaponSlotThree))))

(event Input|KeyboardEvents|Slash
  (params (Key :type Key%20Structure))
  (:Pressed
    (Game|Damage|ApplyDamage self 2e+01 0 0)))

(event Input|KeyboardEvents|NumPadEight
  (params (Key :type Key%20Structure))
  (:Pressed
    (bind _output_get (Variables|Default|SetNewVar_0 (+ (Variables|Default|GetNewVar_0) 5e+02)))
    (Default|CallNewEventDispatcher0 _output_get)))

(fn ConstructionScript)

(fn EquipWeapon
  (params (DesiredWeapon :type Asylum%20Weapon%20Object%20Reference))
  (if (!= DesiredWeapon (Variables|Default|GetCurrentEquippedWeapon))
    (Utilities|IsValid DesiredWeapon
      (:Is%20Valid
        (CallFunction|ShowWeapon DesiredWeapon)
        (bind _output_get (Variables|Default|SetCurrentEquippedWeapon DesiredWeapon))
        (bind _output_get_2 (Variables|Default|SetCurrentWeaponType (Utilities|Struct|BreakWeaponStatsData (Variables|/Script/HellsAsylum.AsylumWeapon|GetWeaponStatsData _output_get))))
        (Class|BPICharacterAnimation|OnCharacterWeaponEquip(Message) (Variables|Default|GetABP_Player) _output_get_2)
        (Variables|Default|SetbIsInCombat true)))))

(fn ShowWeapon
  (params (WeaponDesired :type Asylum%20Weapon%20Object%20Reference))
  (bind _weaponslotone (Variables|Default|GetWeaponSlotOne))
  (bind _weaponslottwo (Variables|Default|GetWeaponSlotTwo))
  (bind _weaponslotthree (Variables|Default|GetWeaponSlotThree))
  (Utilities|IsValid WeaponDesired
    (:Is%20Valid
      (if (and (== WeaponDesired _weaponslotone) (Utilities|IsValid _weaponslotone))
        (Rendering|SetActorHiddenInGame _weaponslotone false)
        (elif (and (== WeaponDesired _weaponslottwo) (Utilities|IsValid _weaponslottwo))
          (Rendering|SetActorHiddenInGame _weaponslottwo false)
          (elif (and (== WeaponDesired _weaponslotthree) (Utilities|IsValid _weaponslotthree))
            (Rendering|SetActorHiddenInGame _weaponslotthree false)))))))

(fn AssignWeapons
  (bind _values (Utilities|Map|Values (Utilities|Struct|BreakCharacterStatsData (Variables|/Script/HellsAsylum.AsylumStatsComponent|GetCharacterStatsDataStruct (Variables|Default|GetPlayerStatsComponent)))))
  (for (_array_element _array_index) _values
    (switch int _array_index
      (:1
        (bind _returnvalue (Game|SpawnActorfromClass _array_element (Transformation|GetActorTransform) "Undefined" (Game|Player|GetPlayerPawn 0) 0))
        (Utilities|IsValid _returnvalue
          (:Is%20Valid
            (switch Utilities|FlowControl|Switch|SwitchonEWeaponSlotType (Utilities|Struct|BreakWeaponStatsData (Variables|/Script/HellsAsylum.AsylumWeapon|GetWeaponStatsData _returnvalue))
              (:ST_Primary
                (bind _output_get (Variables|Default|SetWeaponSlotOne _returnvalue))
                (Transformation|AttachComponentToComponent _output_get (Variables|Character|GetMesh) (Variables|/Script/HellsAsylum.AsylumWeapon|GetWeaponAttachPoint _output_get) "SnapToTarget" "SnapToTarget" "SnapToTarget" true))))))
      (:2
        (bind _returnvalue_2 (Game|SpawnActorfromClass _array_element (Transformation|GetActorTransform) "Undefined" (Game|Player|GetPlayerPawn 0) 0))
        (Utilities|IsValid _returnvalue_2
          (:Is%20Valid
            (switch Utilities|FlowControl|Switch|SwitchonEWeaponSlotType (Utilities|Struct|BreakWeaponStatsData (Variables|/Script/HellsAsylum.AsylumWeapon|GetWeaponStatsData _returnvalue_2))
              (:ST_Secondary
                (bind _output_get_2 (Variables|Default|SetWeaponSlotTwo _returnvalue_2))
                (Transformation|AttachComponentToComponent _output_get_2 (Variables|Character|GetMesh) (Variables|/Script/HellsAsylum.AsylumWeapon|GetWeaponAttachPoint _output_get_2) "SnapToTarget" "SnapToTarget" "SnapToTarget" true))))))
      (:3
        (bind _returnvalue_3 (Game|SpawnActorfromClass _array_element (Transformation|GetActorTransform) "Undefined" (Game|Player|GetPlayerPawn 0) 0))
        (Utilities|IsValid 0
          (:Is%20Valid
            (bind _output_get_3 (Variables|Default|SetWeaponSlotThree _returnvalue_3))
            (switch Utilities|FlowControl|Switch|SwitchonEWeaponSlotType (Utilities|Struct|BreakWeaponStatsData (Variables|/Script/HellsAsylum.AsylumWeapon|GetWeaponStatsData _output_get_3))
              (:ST_Tertiary
                (Transformation|AttachComponentToComponent _output_get_3 (Variables|Character|GetMesh) (Variables|/Script/HellsAsylum.AsylumWeapon|GetWeaponAttachPoint _output_get_3) "SnapToTarget" "SnapToTarget" "SnapToTarget" true))))))))
  (CallFunction|HideWeapons))

(fn HideWeapons
  (bind _weaponslotone (Variables|Default|GetWeaponSlotOne))
  (bind _weaponslottwo (Variables|Default|GetWeaponSlotTwo))
  (bind _weaponslotthree (Variables|Default|GetWeaponSlotThree))
  (Utilities|FlowControl|Sequence
    (:then_0
      (Utilities|IsValid _weaponslotone
        (:Is%20Valid
          (Rendering|SetActorHiddenInGame _weaponslotone true))))
    (:then_1
      (Utilities|IsValid _weaponslottwo
        (:Is%20Valid
          (Rendering|SetActorHiddenInGame _weaponslottwo true))))
    (:then_2
      (Utilities|IsValid _weaponslotthree
        (:Is%20Valid
          (Rendering|SetActorHiddenInGame _weaponslotthree true))))))

(fn CharacterSetup
  (bind _playerstatscomponent (Variables|Default|GetPlayerStatsComponent))
  (bind _characterstatsdatastruct (Variables|/Script/HellsAsylum.AsylumStatsComponent|GetCharacterStatsDataStruct _playerstatscomponent))
  (bind _weaponinventory (Utilities|Struct|BreakCharacterStatsData _characterstatsdatastruct))
  (CallFunction|SetupLockon)
  (Variables|Default|SetABP_Player (Components|SkeletalMesh|GetAnimInstance (Variables|Character|GetMesh)))
  (Utilities|FlowControl|Sequence
    (:then_0
      (if (CallFunction|LoadingfromSave?)
        (CallFunction|SetCharacterStatsfromSave)
        (else
          (CallFunction|SetStartingCharacterStats))))
    (:then_1
      (Utilities|Map|Add _weaponinventory 1 0)
      (Utilities|Map|Add _weaponinventory 2 0)
      (Utilities|Map|Add _weaponinventory 3 0)
      (Utilities|Struct|SetmembersinCharacterStatsData _characterstatsdatastruct)
      (CallFunction|AssignWeapons))))

(fn SetupLockon
  (Variables|Default|SetTValidLockOnObjects (Utilities|Array|MakeArray "ObjectTypeQuery3" "ObjectTypeQuery8" "ObjectTypeQuery2"))
  (Variables|Default|SetLockOnActorsToIgnore (Utilities|Array|MakeArray self)))

(fn WeaponAttack
  (bind _currentequippedweapon (Variables|Default|GetCurrentEquippedWeapon))
  (Utilities|IsValid _currentequippedweapon
    (:Is%20Valid
      (Class|AsylumWeaponInterface|OnStartFire(Message) _currentequippedweapon)
      (Class|BPICharacterAnimation|OnCharacterWeaponAttack(Message) (Variables|Default|GetABP_Player) (Variables|Default|GetCurrentWeaponType)))))

(fn WeaponStopAttack
  (bind _currentequippedweapon (Variables|Default|GetCurrentEquippedWeapon))
  (Utilities|IsValid _currentequippedweapon
    (:Is%20Valid
      (Class|AsylumWeaponInterface|OnFinishFire(Message) _currentequippedweapon))))

(fn SetStartingCharacterStats
  (bind _returndifficulty (CallFunction|GetGameDifficulty))
  (bind _playerstatscomponent (Variables|Default|GetPlayerStatsComponent))
  (bind _goethesuitcomponent (Variables|Default|GetGoetheSuitComponent))
  (bind _returnvalue (Utilities|GetDataTableRow (Variables|/Script/HellsAsylum.AsylumStatsComponent|GetCharacterDataTable _playerstatscomponent) _returndifficulty)
    (:then
      (Utilities|Struct|SetmembersinCharacterStatsData (Variables|/Script/HellsAsylum.AsylumStatsComponent|GetCharacterStatsDataStruct _playerstatscomponent) (.bHasShield (Utilities|Struct|BreakCharacterStatsData _returnvalue)) (.fCurrentHealth (Utilities|Struct|BreakCharacterStatsData _returnvalue)) (.fMaxHealth (Utilities|Struct|BreakCharacterStatsData _returnvalue)) (.fCurrentShield (Utilities|Struct|BreakCharacterStatsData _returnvalue)) (.fMaxShield (Utilities|Struct|BreakCharacterStatsData _returnvalue)) (.iCurrentCharacterLevel (Utilities|Struct|BreakCharacterStatsData _returnvalue)) (.iMaxCharacterLevel (Utilities|Struct|BreakCharacterStatsData _returnvalue)) (.fMovementLoudness (Utilities|Struct|BreakCharacterStatsData _returnvalue)) (.fMovementMaxRange (Utilities|Struct|BreakCharacterStatsData _returnvalue)) (.fCrouchMovementLoudness (Utilities|Struct|BreakCharacterStatsData _returnvalue)) (.fCrouchMovementMaxRange (Utilities|Struct|BreakCharacterStatsData _returnvalue)) (.fFireResist (Utilities|Struct|BreakCharacterStatsData _returnvalue)) (.fIceResist (Utilities|Struct|BreakCharacterStatsData _returnvalue)) (.fShockResist (Utilities|Struct|BreakCharacterStatsData _returnvalue)))
      (bind _returnvalue_2 (Utilities|GetDataTableRow (Variables|/Script/HellsAsylum.AsylumSuitComponent|GetSuitStatsDataTable _goethesuitcomponent) _returndifficulty)
        (:then
          (Utilities|Struct|SetmembersinGoetheSuitStatsData (Variables|/Script/HellsAsylum.AsylumSuitComponent|GetSuitStatsData _goethesuitcomponent) (.GoetheSelectedMainAbility (Utilities|Struct|BreakGoetheSuitStatsData _returnvalue_2)) (.GoetheSuitType (Utilities|Struct|BreakGoetheSuitStatsData _returnvalue_2)) (.GoethePassivePowerOne (Utilities|Struct|BreakGoetheSuitStatsData _returnvalue_2)) (.GoethePassivePowerTwo (Utilities|Struct|BreakGoetheSuitStatsData _returnvalue_2)) (.GoetheActivePowerOne (Utilities|Struct|BreakGoetheSuitStatsData _returnvalue_2)) (.GoetheActivePowerTwo (Utilities|Struct|BreakGoetheSuitStatsData _returnvalue_2)) (.GoetheActivePowerThree (Utilities|Struct|BreakGoetheSuitStatsData _returnvalue_2)) (.DespairOrbCurrentLevel (Utilities|Struct|BreakGoetheSuitStatsData _returnvalue_2)) (.DespairOrbMaxLevel (Utilities|Struct|BreakGoetheSuitStatsData _returnvalue_2)) (.HarmonyOrbCurrentLevel (Utilities|Struct|BreakGoetheSuitStatsData _returnvalue_2)) (.HarmonyOrbMaxLevel (Utilities|Struct|BreakGoetheSuitStatsData _returnvalue_2)) (.TeslaCurrentLevel (Utilities|Struct|BreakGoetheSuitStatsData _returnvalue_2)) (.TeslaMaxLevel (Utilities|Struct|BreakGoetheSuitStatsData _returnvalue_2)) (.ChargerCurrentLevel (Utilities|Struct|BreakGoetheSuitStatsData _returnvalue_2)) (.ChargerMaxLevel (Utilities|Struct|BreakGoetheSuitStatsData _returnvalue_2)) (.StormCurrentLevel (Utilities|Struct|BreakGoetheSuitStatsData _returnvalue_2)) (.StormMaxLevel (Utilities|Struct|BreakGoetheSuitStatsData _returnvalue_2)) (.TractorCurrentLevel (Utilities|Struct|BreakGoetheSuitStatsData _returnvalue_2)) (.TractorMaxLevel (Utilities|Struct|BreakGoetheSuitStatsData _returnvalue_2)) (.EnergyDrainCurrentLevel (Utilities|Struct|BreakGoetheSuitStatsData _returnvalue_2)) (.EnergyDrainMaxLevel (Utilities|Struct|BreakGoetheSuitStatsData _returnvalue_2)) (.WeaponPowersCurrentLevel (Utilities|Struct|BreakGoetheSuitStatsData _returnvalue_2)) (.WeaponPowersMaxLevel (Utilities|Struct|BreakGoetheSuitStatsData _returnvalue_2)) (.CurrentAragonGauge (Utilities|Struct|BreakGoetheSuitStatsData _returnvalue_2)) (.MaxAragonGauge (Utilities|Struct|BreakGoetheSuitStatsData _returnvalue_2)) (.CurrentAragonTanks (Utilities|Struct|BreakGoetheSuitStatsData _returnvalue_2)) (.MaxAragonTanks (Utilities|Struct|BreakGoetheSuitStatsData _returnvalue_2)) (.QuicksilverSlowDownAmount (Utilities|Struct|BreakGoetheSuitStatsData _returnvalue_2)) (.QuicksilverPlayerSpeed (Utilities|Struct|BreakGoetheSuitStatsData _returnvalue_2)) (.QuicksilverConsumptionRate (Utilities|Struct|BreakGoetheSuitStatsData _returnvalue_2)) (.OverdriveConsumptionRate (Utilities|Struct|BreakGoetheSuitStatsData _returnvalue_2)) (.SacrificeConsumptionRate (Utilities|Struct|BreakGoetheSuitStatsData _returnvalue_2)) (.SacrificePowerLimit (Utilities|Struct|BreakGoetheSuitStatsData _returnvalue_2)) (.OverdriveSpeedBoost (Utilities|Struct|BreakGoetheSuitStatsData _returnvalue_2)) (.EnergyDrainConsumptionRate (Utilities|Struct|BreakGoetheSuitStatsData _returnvalue_2)) (.DiscordAbilityCooldown (Utilities|Struct|BreakGoetheSuitStatsData _returnvalue_2)) (.HarmonyAbilityCooldown (Utilities|Struct|BreakGoetheSuitStatsData _returnvalue_2)) (.SnowAbilityCooldown (Utilities|Struct|BreakGoetheSuitStatsData _returnvalue_2)) (.ChargerAbilityCooldown (Utilities|Struct|BreakGoetheSuitStatsData _returnvalue_2)) (.DrainAbilityCooldown (Utilities|Struct|BreakGoetheSuitStatsData _returnvalue_2)) (.TeslaAbilityCooldown (Utilities|Struct|BreakGoetheSuitStatsData _returnvalue_2)) (.WeaponAbilityCooldown (Utilities|Struct|BreakGoetheSuitStatsData _returnvalue_2)) (.ScanRadius (Utilities|Struct|BreakGoetheSuitStatsData _returnvalue_2)) (.EnemySearchRadius (Utilities|Struct|BreakGoetheSuitStatsData _returnvalue_2)))
          (Default|CallOnPlayerUpdate))))))

(fn SetCharacterStatsfromSave
  (bind (_savedplayersuitstats _savedplayercharacterstats) (CallFunction|GetPlayerStatsfromSave))
  (bind (_bhasshield _fcurrenthealth _fmaxhealth _fcurrentshield _fmaxshield _icurrentcharacterlevel _imaxcharacterlevel _fmovementloudness _fmovementmaxrange _fcrouchmovementloudness _fcrouchmovementmaxrange _ffireresist _ficeresist _fshockresist) (Utilities|Struct|BreakCharacterStatsData _savedplayercharacterstats))
  (bind (_goetheselectedmainability _goethesuittype _goethepassivepowerone _goethepassivepowertwo _goetheactivepowerone _goetheactivepowertwo _goetheactivepowerthree _despairorbcurrentlevel _despairorbmaxlevel _harmonyorbcurrentlevel _harmonyorbmaxlevel _teslacurrentlevel _teslamaxlevel _chargercurrentlevel _chargermaxlevel _stormcurrentlevel _stormmaxlevel _tractorcurrentlevel _tractormaxlevel _energydraincurrentlevel _energydrainmaxlevel _weaponpowerscurrentlevel _weaponpowersmaxlevel _currentaragongauge _maxaragongauge _currentaragontanks _maxaragontanks _quicksilverslowdownamount _quicksilverplayerspeed _quicksilverconsumptionrate _overdriveconsumptionrate _sacrificeconsumptionrate _sacrificepowerlimit _overdrivespeedboost _energydrainconsumptionrate _discordabilitycooldown _harmonyabilitycooldown _snowabilitycooldown _chargerabilitycooldown _drainabilitycooldown _teslaabilitycooldown _weaponabilitycooldown _scanradius _enemysearchradius) (Utilities|Struct|BreakGoetheSuitStatsData _savedplayersuitstats))
  (Utilities|Struct|SetmembersinCharacterStatsData (Variables|/Script/HellsAsylum.AsylumStatsComponent|GetCharacterStatsDataStruct (Variables|Default|GetPlayerStatsComponent)) _bhasshield _fcurrenthealth _fmaxhealth _fcurrentshield _fmaxshield _icurrentcharacterlevel _imaxcharacterlevel _fmovementloudness _fmovementmaxrange _fcrouchmovementloudness _fcrouchmovementmaxrange _ffireresist _ficeresist _fshockresist)
  (Utilities|Struct|SetmembersinGoetheSuitStatsData (Variables|/Script/HellsAsylum.AsylumSuitComponent|GetSuitStatsData (Variables|Default|GetGoetheSuitComponent)) _goetheselectedmainability _goethesuittype _goethepassivepowerone _goethepassivepowertwo _goetheactivepowerone _goetheactivepowertwo _goetheactivepowerthree _despairorbcurrentlevel _despairorbmaxlevel _harmonyorbcurrentlevel _harmonyorbmaxlevel _teslacurrentlevel _teslamaxlevel _chargercurrentlevel _chargermaxlevel _stormcurrentlevel _stormmaxlevel _tractorcurrentlevel _tractormaxlevel _energydraincurrentlevel _energydrainmaxlevel _weaponpowerscurrentlevel _weaponpowersmaxlevel _currentaragongauge _maxaragongauge _currentaragontanks _maxaragontanks _quicksilverslowdownamount _quicksilverplayerspeed _quicksilverconsumptionrate _overdriveconsumptionrate _sacrificeconsumptionrate _sacrificepowerlimit _overdrivespeedboost _energydrainconsumptionrate _discordabilitycooldown _harmonyabilitycooldown _snowabilitycooldown _chargerabilitycooldown _drainabilitycooldown _teslaabilitycooldown _weaponabilitycooldown _scanradius _enemysearchradius)
  (Default|CallOnPlayerUpdate))

(fn AddWeapon
  (params (Key :type Integer%20%28by%20ref%29) (Value :type Asylum%20Weapon%20Class%20Reference%20%28by%20ref%29))
  (bind _playerstatscomponent (Variables|Default|GetPlayerStatsComponent))
  (bind _characterstatsdatastruct (Variables|/Script/HellsAsylum.AsylumStatsComponent|GetCharacterStatsDataStruct _playerstatscomponent))
  (Utilities|Map|Add (Utilities|Struct|BreakCharacterStatsData _characterstatsdatastruct) Key Value)
  (Utilities|Struct|SetmembersinCharacterStatsData _characterstatsdatastruct)
  (CallFunction|AssignWeapons))

(fn TakeDamage
  (params (DamageApplied :type Float%20%28single-precision%29))
  (bind _playerstatscomponent (Variables|Default|GetPlayerStatsComponent))
  (bind _characterstatsdatastruct (Variables|/Script/HellsAsylum.AsylumStatsComponent|GetCharacterStatsDataStruct _playerstatscomponent))
  (bind (_bhasshield _fcurrenthealth _fcurrentshield) (Utilities|Struct|BreakCharacterStatsData _characterstatsdatastruct))
  (Default|CallOnPlayerUpdate)
  (if _bhasshield
    (bind _structout (Utilities|Struct|SetmembersinCharacterStatsData _characterstatsdatastruct (- _fcurrentshield DamageApplied)))
    (if (<= (Utilities|Struct|BreakCharacterStatsData _structout) 0.0)
      (Utilities|Struct|SetmembersinCharacterStatsData _structout false 0.0))
    (else
      (bind _structout_2 (Utilities|Struct|SetmembersinCharacterStatsData _characterstatsdatastruct (- _fcurrenthealth DamageApplied)))
      (if (<= (Utilities|Struct|BreakCharacterStatsData _structout_2) 0.0)
        (Default|CallOnPlayerDeath)))))
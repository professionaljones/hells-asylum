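; Player-controlled flying drone pawn that the player can possess, steer and fire from.
; Axis inputs drive horizontal movement, elevation and look, while Attack spawns a drone projectile at a scene component, facing the actor's rotation.
; Possession events toggle damageability and set actor visibility, and a sphere overlap sends lock-on on/off messages to non-player actors.
; Trace and return-to-character possession logic is left unconnected, and GetLockOnActor is an empty stub.
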(event OnComponentBeginOverlap(Sphere)
  (params (OverlappedComponent :type Primitive%20Component%20Object%20Reference) (OtherActor :type Actor%20Object%20Reference) (OtherComp :type Primitive%20Component%20Object%20Reference) (OtherBodyIndex :type Integer) (bFromSweep :type Boolean) (SweepResult :type Hit%20Result%20Structure%20%28by%20ref%29))
  (if (not (CallFunction|IsPlayerOtherActor? OtherActor))
    (Class|AsylumCharacterInterface|OnPlayerLockon(Message) OtherActor true)))

(event OnComponentEndOverlap(Sphere)
  (params (OverlappedComponent :type Primitive%20Component%20Object%20Reference) (OtherActor :type Actor%20Object%20Reference) (OtherComp :type Primitive%20Component%20Object%20Reference) (OtherBodyIndex :type Integer))
  (if (not (CallFunction|IsPlayerOtherActor? OtherActor))
    (Class|AsylumCharacterInterface|OnPlayerLockon(Message) OtherActor false)))

(event EventBeginPlay
  (Rendering|SetActorHiddenInGame true)
  (Variables|Actor|SetbCanBeDamaged false))

(event EventUnpossessed
  (params (OldController :type Controller%20Object%20Reference))
  (Rendering|SetActorHiddenInGame true)
  (Rendering|SetActorHiddenInGame true)
  (Variables|Actor|SetbCanBeDamaged false))

(event EventPossessed
  (params (NewController :type Controller%20Object%20Reference))
  (Rendering|SetActorHiddenInGame false)
  (Rendering|SetActorHiddenInGame true)
  (Variables|Actor|SetbCanBeDamaged true))

(event Input|ActionEvents|InputActionAttack
  (params (Key :type Key%20Structure))
  (:Pressed
    (Game|SpawnActorfromClass "/Game/Dynamic/Weapons/WeaponDroneProjectile.WeaponDroneProjectile_C" (Math|Transform|MakeTransform (Transformation|GetWorldLocation (Variables|Default|GetScene)) (Transformation|GetActorRotation) "1,1,1") "Undefined" 0 0)))

(event Input|ActionEvents|InputActionActivateDrone
  (params (Key :type Key%20Structure)))

(event Input|AxisEvents|InputAxisLookUpAtRate
  (params (AxisValue :type Float%20%28single-precision%29))
  (Pawn|Input|AddControllerPitchInput AxisValue))

(event Input|AxisEvents|InputAxisTurn
  (params (AxisValue :type Float%20%28single-precision%29))
  (Pawn|Input|AddControllerYawInput AxisValue))

(event Input|AxisEvents|InputAxisLookUp
  (params (AxisValue :type Float%20%28single-precision%29))
  (Pawn|Input|AddControllerPitchInput AxisValue))

(event Input|AxisEvents|InputAxisMoveForward
  (params (AxisValue :type Float%20%28single-precision%29))
  (Pawn|Input|AddMovementInput (* (Math|Vector|GetForwardVector (Transformation|GetActorRotation)) (* AxisValue 1e+02)) 1.0 false))

(event Input|AxisEvents|InputAxisMoveRight
  (params (AxisValue :type Float%20%28single-precision%29))
  (Pawn|Input|AddMovementInput (* (Math|Vector|GetRightVector (Transformation|GetActorRotation)) (* AxisValue 1e+02)) 1.0 false))

(event Input|AxisEvents|InputAxisTurnRate
  (params (AxisValue :type Float%20%28single-precision%29))
  (Pawn|Input|AddControllerYawInput AxisValue))

(event Input|AxisEvents|InputAxisElevation
  (params (AxisValue :type Float%20%28single-precision%29))
  (Pawn|Input|AddMovementInput "0,0.000000,1.000000" (* AxisValue 1e+02) false))

(fn ConstructionScript)

(fn GetLockonActor
  (return 0))
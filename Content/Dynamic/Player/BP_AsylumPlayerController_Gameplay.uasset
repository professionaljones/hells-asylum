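; Gameplay player controller that handles menus, drone switching and debug cheats.
; Input opens pause, journal, cheat console and debug widgets from the game HUD, pausing the game and switching input mode, while debug keys boost drop chance and crit multiplier.
; BeginPlay spawns a drone that can swap possession with the original pawn, and caches windowed resolutions.
; Events drive the animated interact prompt and level-transition fade; UpdateAbilitySlot uses and highlights actionbar slots.
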(event EventBeginPlay
  (Variables|Default|SetMelPawn (Game|Player|GetPlayerPawn 0))
  (bind _returnvalue (Game|SpawnActorfromClass "/Game/Dynamic/Player/BP_PlayerCharacter_Drone.BP_PlayerCharacter_Drone_C" (Math|Transform|MakeTransform "0, 0, 0") "Undefined" 0 0))
  (Variables|Default|SetPlayerDrone _returnvalue)
  (bind _resolutions (Class|KismetSystemLibrary|GetConvenientWindowedResolutions))
  (for _array_element _resolutions
    (Utilities|Array|Add (Variables|Default|GetWindowedResolutions) (Utilities|String|Append (Utilities|String|BuildString(Integer) "" "" (.X (Utilities|Struct|BreakIntPoint _array_element))) " x " (Utilities|String|BuildString(Integer) "" "" (.Y (Utilities|Struct|BreakIntPoint _array_element))))))
  (bind _returnvalue_2 (Settings|GetGameUserSettings))
  (Variables|Default|SetCurrentResolution (Class|GameUserSettings|GetScreenResolution _returnvalue_2)))

(event EventOnLevelTransition
  (CameraFades|StartCameraFade :self (Variables|Default|GetPlayerCameraManager) :ToAlpha 1.0 :Duration 5.0 :bShouldFadeAudio true :bHoldWhenFinished true)
  (Input|DisableInput (Game|GetPlayerCharacter 0) self))

(event EventOnInteractVisible
  (bind _returnvalue (CallFunction|GetGameHUD))
  (bind _playerhudwidget_n (Variables|/Game/Dynamic/UserInterface/BP_AsylumHUD_Base.BP_AsylumHUD_Base_C|GetPlayerHUDWidget_N _returnvalue))
  (bind _wp_interact (Variables|/Game/Static/UI_Kit/Widgets/WBP_PlayerHUD_N.WBP_PlayerHUD_N_C|GetWP_Interact _playerhudwidget_n))
  (Widget|SetVisibility _wp_interact "SelfHitTestInvisible")
  (UserInterface|Animation|PlayAnimation _wp_interact (Variables|/Game/Dynamic/UserInterface/WBPs/Gameplay/Components/WP_Interact.WP_Interact_C|GetStartAnim _wp_interact) 0.0 0 "PingPong" 2.0))

(event EventOnInteractNotVisible
  (bind _returnvalue (CallFunction|GetGameHUD))
  (bind _playerhudwidget_n (Variables|/Game/Dynamic/UserInterface/BP_AsylumHUD_Base.BP_AsylumHUD_Base_C|GetPlayerHUDWidget_N _returnvalue))
  (bind _wp_interact (Variables|/Game/Static/UI_Kit/Widgets/WBP_PlayerHUD_N.WBP_PlayerHUD_N_C|GetWP_Interact _playerhudwidget_n))
  (if (== (Game|GetGameMode) (CallFunction|GetStoryGameMode))
    (Widget|SetVisibility _wp_interact "Hidden")
    (Class|UserWidget|StopAnimation _wp_interact (Variables|/Game/Dynamic/UserInterface/WBPs/Gameplay/Components/WP_Interact.WP_Interact_C|GetStartAnim _wp_interact))))

(event Input|ActionEvents|InputActionPause
  (params (Key :type Key%20Structure))
  (bind _returnvalue (Game|GetPlayerController 0))
  (bind _returnvalue_2 (CallFunction|GetGameHUD))
  (bind _pausewidget (Variables|/Game/Dynamic/UserInterface/BP_AsylumHUD_Base.BP_AsylumHUD_Base_C|GetPauseWidget _returnvalue_2))
  (:Pressed
    (if (Variables|Default|GetbPauseMenuActive?)
      (Widget|RemovefromParent _pausewidget)
      (Variables|Default|SetbPauseMenuActive? false)
      (Input|SetInputModeGameOnly _returnvalue)
      (Game|SetGamePaused false)
      (Variables|Default|SetbShowMouseCursor false)
      (else
        (UserInterface|Viewport|AddtoViewport _pausewidget 0)
        (Variables|Default|SetbPauseMenuActive? true)
        (Game|SetGamePaused true)
        (Variables|Default|SetbShowMouseCursor true)
        (Input|SetInputModeGameandUI _returnvalue (Variables|/Game/Dynamic/UserInterface/WBPs/Gameplay/WBP_PlayerPauseMenu.WBP_PlayerPauseMenu_C|GetResumeButton _pausewidget) "LockInFullscreen" false)))))

(event Input|ActionEvents|InputActionJournal
  (params (Key :type Key%20Structure))
  (bind _returnvalue (CallFunction|GetGameHUD))
  (bind _returnvalue_2 (Game|GetPlayerController 0))
  (bind _journalwidget (Variables|/Game/Dynamic/UserInterface/BP_AsylumHUD_Base.BP_AsylumHUD_Base_C|GetJournalWidget _returnvalue))
  (:Pressed
    (if (not (Variables|Default|GetbPauseMenuActive?))
      (if (Variables|Default|GetbJournalMenuActive?)
        (Widget|RemovefromParent _journalwidget)
        (Variables|Default|SetbJournalMenuActive? false)
        (Input|SetInputModeGameOnly _returnvalue_2)
        (Game|SetGamePaused false)
        (Variables|Default|SetbShowMouseCursor false)
        (else
          (UserInterface|Viewport|AddtoViewport _journalwidget 0)
          (Variables|Default|SetbJournalMenuActive? true)
          (Game|SetGamePaused true)
          (Variables|Default|SetbShowMouseCursor true)
          (Input|SetInputModeGameandUI _returnvalue_2 (Variables|/Game/Dynamic/UserInterface/WBPs/Gameplay/WBP_PlayerJournal.WBP_PlayerJournal_C|GetMapButton _journalwidget) "LockInFullscreen" false))))))

(event Input|ActionEvents|InputActionShowCheatMenu
  (params (Key :type Key%20Structure))
  (bind _returnvalue (CallFunction|GetGameHUD))
  (:Pressed
    (Utilities|FlowControl|FlipFlop
      (:A
        (Class|AsylumHUDInterface|ShowConsoleMenu(Message) _returnvalue)
        (Game|SetGamePaused true)
        (Variables|Default|SetbShowMouseCursor true))
      (:B
        (Widget|RemovefromParent (Variables|/Game/Dynamic/UserInterface/BP_AsylumHUD_Base.BP_AsylumHUD_Base_C|GetConsoleWidget _returnvalue))
        (Input|SetInputModeGameOnly self)
        (Variables|Default|SetbShowMouseCursor false)
        (if (Game|IsGamePaused)
          (Game|SetGamePaused false))))))

(event Input|ActionEvents|InputActionActivateDrone
  (params (Key :type Key%20Structure))
  (:Pressed
    (if (Variables|Default|GetbEnableDrone?)
      (Pawn|UnPossess (Game|GetPlayerController 0))
      (if (Variables|Default|GetbIsDrone)
        (Pawn|Possess (Variables|Default|GetMelPawn))
        (Variables|Default|SetbIsDrone false)
        (else
          (Pawn|Possess (Variables|Default|GetPlayerDrone))
          (Variables|Default|SetbIsDrone true))))))

(event Input|KeyboardEvents|Add
  (params (Key :type Key%20Structure))
  (bind _playerstate (Variables|Default|GetPlayerState))
  (:Pressed
    (Class|AslyumMissionModeInterface|OnCritStart(Message) _playerstate 99.0 999.0)
    (Class|AslyumMissionModeInterface|OnMissionEnemyKill(Message) _playerstate 5e+01)))

(event Input|KeyboardEvents|Divide
  (params (Key :type Key%20Structure))
  (bind _returnvalue (CallFunction|GetCurrentPlayerState))
  (bind _asbp_asylum_player_state_mission (Utilities|Casting|CastToBP_AsylumPlayerState_Mission _returnvalue))
  (:Pressed
    (bind _output_get (Variables|/Script/HellsAsylum.AsylumPlayerState|SetPlayerBoostDropChance _asbp_asylum_player_state_mission (+ (Variables|/Script/HellsAsylum.AsylumPlayerState|GetPlayerBoostDropChance _asbp_asylum_player_state_mission) 0.02)))
    (Development|PrintString (Utilities|String|ToString(Float) _output_get))))

(event Input|KeyboardEvents|Insert
  (params (Key :type Key%20Structure))
  (bind _returnvalue (CallFunction|GetGameHUD))
  (bind _self self)
  (bind _playerhudwidget_n (Variables|/Game/Dynamic/UserInterface/BP_AsylumHUD_Base.BP_AsylumHUD_Base_C|GetPlayerHUDWidget_N _returnvalue))
  (bind _debugwidget (Variables|/Game/Dynamic/UserInterface/BP_AsylumHUD_Base.BP_AsylumHUD_Base_C|GetDebugWidget _returnvalue))
  (:Pressed
    (Utilities|FlowControl|FlipFlop
      (:A
        (UserInterface|Viewport|AddtoViewport _debugwidget 0)
        (Input|SetInputModeGameandUI _self _debugwidget "DoNotLock" false)
        (Variables|Default|SetbShowMouseCursor true)
        (Game|SetGamePaused true)
        (Widget|SetVisibility _playerhudwidget_n "Hidden"))
      (:B
        (Widget|RemovefromParent _debugwidget)
        (Widget|SetVisibility _playerhudwidget_n "SelfHitTestInvisible")
        (Input|SetInputModeGameOnly _self)
        (Variables|Default|SetbShowMouseCursor false)))))

(fn ConstructionScript)

(fn AdjustResolution)

(fn UpdateAbilitySlot
  (params (Slot%20ID :type Name))
  (Default|CallUseActionbarSlot Slot%20ID)
  (Default|CallSetActionbarHighlight Slot%20ID true)
  (return))

(fn GetLockonActor
  (return 0))
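; Player controller that handles the pause menu and journal menu toggles for the game.
; The Pause and Journal inputs add or remove HUD-owned widgets, pausing the game and switching mouse cursor and input mode, with a button focused on open.
; Journal input is ignored while the pause menu is active, but Pause does not check whether the journal is open.
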(event EventBeginPlay)

(event EventTick
  (params (DeltaSeconds :type Float%20%28single-precision%29)))

(event Input|ActionEvents|InputActionPause
  (params (Key :type Key%20Structure))
  (bind _returnvalue (Game|GetPlayerController 0))
  (bind _returnvalue_2 (CallFunction|GetGameHUD))
  (bind _pausewidget (Variables|/Game/Dynamic/UserInterface/BP_AsylumHUD_Base.BP_AsylumHUD_Base_C|GetPauseWidget _returnvalue_2))
  (:Pressed
    (if (Variables|Default|GetbPauseMenuActive?)
      (Widget|RemovefromParent _pausewidget)
      (Variables|Default|SetbPauseMenuActive? false)
      (Input|SetInputModeGameOnly _returnvalue)
      (Game|SetGamePaused false)
      (Variables|Default|SetbShowMouseCursor false)
      (else
        (UserInterface|Viewport|AddtoViewport _pausewidget 0)
        (Variables|Default|SetbPauseMenuActive? true)
        (Game|SetGamePaused true)
        (Variables|Default|SetbShowMouseCursor true)
        (Input|SetInputModeGameandUI _returnvalue (Variables|/Game/Dynamic/UserInterface/WBPs/Gameplay/WBP_PlayerPauseMenu.WBP_PlayerPauseMenu_C|GetResumeButton _pausewidget) "LockInFullscreen" false)))))

(event Input|ActionEvents|InputActionJournal
  (params (Key :type Key%20Structure))
  (bind _returnvalue (CallFunction|GetGameHUD))
  (bind _returnvalue_2 (Game|GetPlayerController 0))
  (bind _journalwidget (Variables|/Game/Dynamic/UserInterface/BP_AsylumHUD_Base.BP_AsylumHUD_Base_C|GetJournalWidget _returnvalue))
  (:Pressed
    (if (not (Variables|Default|GetbPauseMenuActive?))
      (if (Variables|Default|GetbJournalMenuActive?)
        (Widget|RemovefromParent _journalwidget)
        (Variables|Default|SetbJournalMenuActive? false)
        (Input|SetInputModeGameOnly _returnvalue_2)
        (Game|SetGamePaused false)
        (Variables|Default|SetbShowMouseCursor false)
        (else
          (UserInterface|Viewport|AddtoViewport _journalwidget 0)
          (Variables|Default|SetbJournalMenuActive? true)
          (Game|SetGamePaused true)
          (Variables|Default|SetbShowMouseCursor true)
          (Input|SetInputModeGameandUI _returnvalue_2 (Variables|/Game/Dynamic/UserInterface/WBPs/Gameplay/WBP_PlayerJournal.WBP_PlayerJournal_C|GetMapButton _journalwidget) "LockInFullscreen" false))))))

(fn ConstructionScript)
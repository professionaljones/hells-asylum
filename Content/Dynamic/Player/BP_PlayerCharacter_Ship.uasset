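; Player-pilotable ship pawn that flies with floating movement, is shown and damageable while possessed, and turns hidden and undamageable when unpossessed.
; Input axes drive movement and look, with Roll moving it along world Z rather than rolling, and Sprint raising speed and acceleration.
; BeginPlay attaches a spawned drone weapon to the Scene component, but Attack spawns projectiles there directly.
; GetLockOnActor is an empty stub, and the trace and possession-switch logic are disconnected.
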(event EventBeginPlay
  (bind _staticmesh (Variables|Default|GetStaticMesh))
  (bind _returnvalue (Game|SpawnActorfromClass "/Game/Dynamic/Weapons/Player/BP_PlayerWeapon_Drone.BP_PlayerWeapon_Drone_C" (Math|Transform|MakeTransform "0, 0, 0") "Undefined" self 0))
  (bind _output_get (Variables|Default|SetDroneWeapon _returnvalue))
  (Transformation|AttachComponentToComponent _output_get (Variables|Default|GetScene) "None" "SnapToTarget" "SnapToTarget" "SnapToTarget" true)
  (Transformation|AttachComponentToComponent (Variables|Default|GetParticleSystem1) _staticmesh "None" "SnapToTarget" "SnapToTarget" "SnapToTarget" true)
  (Transformation|AttachComponentToComponent (Variables|Default|GetParticleSystem2) _staticmesh "None" "SnapToTarget" "SnapToTarget" "SnapToTarget" true))

(event Collision|EventActorBeginOverlap
  (params (OtherActor :type Actor%20Object%20Reference)))

(event EventTick
  (params (DeltaSeconds :type Float%20%28single-precision%29)))

(event EventUnpossessed
  (params (OldController :type Controller%20Object%20Reference))
  (Rendering|SetActorHiddenInGame true)
  (Variables|Actor|SetbCanBeDamaged false))

(event EventPossessed
  (params (NewController :type Controller%20Object%20Reference))
  (Rendering|SetActorHiddenInGame false)
  (Variables|Actor|SetbCanBeDamaged true))

(event Input|ActionEvents|InputActionAttack
  (params (Key :type Key%20Structure))
  (:Pressed
    (Game|SpawnActorfromClass "/Game/Dynamic/Weapons/WeaponDroneProjectile.WeaponDroneProjectile_C" (Math|Transform|MakeTransform (Transformation|GetWorldLocation (Variables|Default|GetScene)) (Transformation|GetActorRotation) "1,1,1") "Undefined" 0 0)))

(event Input|ActionEvents|InputActionSprint
  (params (Key :type Key%20Structure))
  (bind _floatingpawnmovement (Variables|Default|GetFloatingPawnMovement))
  (:Pressed
    (Variables|/Script/Engine.FloatingPawnMovement|SetMaxSpeed _floatingpawnmovement 6e+03)
    (Variables|/Script/Engine.FloatingPawnMovement|SetAcceleration _floatingpawnmovement 6e+03))
  (:Released
    (Variables|/Script/Engine.FloatingPawnMovement|SetMaxSpeed _floatingpawnmovement 3e+03)
    (Variables|/Script/Engine.FloatingPawnMovement|SetAcceleration _floatingpawnmovement 4e+03)))

(event Input|ActionEvents|InputActionActivateDrone
  (params (Key :type Key%20Structure)))

(event Input|AxisEvents|InputAxisRoll
  (params (AxisValue :type Float%20%28single-precision%29))
  (Pawn|Input|AddMovementInput "0,0.000000,1.000000" (* AxisValue 1e+02) false))

(event Input|AxisEvents|InputAxisTurn
  (params (AxisValue :type Float%20%28single-precision%29))
  (Pawn|Input|AddControllerYawInput AxisValue))

(event Input|AxisEvents|InputAxisLookUp
  (params (AxisValue :type Float%20%28single-precision%29))
  (Pawn|Input|AddControllerPitchInput AxisValue))

(event Input|AxisEvents|InputAxisMoveForward
  (params (AxisValue :type Float%20%28single-precision%29))
  (Pawn|Input|AddMovementInput (* (Math|Vector|GetForwardVector (Transformation|GetActorRotation)) (* AxisValue 1e+02)) 1.0 false))

(event Input|AxisEvents|InputAxisMoveRight
  (params (AxisValue :type Float%20%28single-precision%29))
  (Pawn|Input|AddMovementInput (* (Math|Vector|GetRightVector (Transformation|GetActorRotation)) (* AxisValue 1e+02)) 1.0 false))

(fn ConstructionScript)

(fn GetLockonActor
  (return 0))
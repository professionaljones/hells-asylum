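; Player camera manager that handles screen and audio fades at level start and player death.
; BeginPlay fades in picture and audio over five seconds and binds an event to player combat start.
; UpdateCameraOnDeath fades out and holds while sound mix overrides silence weapons and dialogue.
; UpdateCameraInCombat is effectively empty: its view yaw clamping logic is disconnected and never runs.
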(event EventBeginPlay
  (CameraFades|StartCameraFade :FromAlpha 1.0 :Duration 5.0 :bShouldFadeAudio true)
  (EventDispatchers|BindEventtoOnPlayerCombatStart (EventDispatchers|CreateEvent :!event UpdateCamerainCombat)))

(fn ConstructionScript)

(fn UpdateCamerainCombat
  (params (Condition :type Boolean)))

(fn UpdateCameraonDeath
  (CameraFades|StartCameraFade :ToAlpha 1.0 :Duration 5.0 :bHoldWhenFinished true)
  (Audio|SetSoundMixClassOverride "/Game/Dynamic/Game/Audio/SM_Weapons.SM_Weapons" 0 0.0 1.0 5.0 true)
  (Audio|SetSoundMixClassOverride "/Game/Dynamic/Game/Audio/SM_Dialogue.SM_Dialogue" 0 0.0 1.0 5.0 true))
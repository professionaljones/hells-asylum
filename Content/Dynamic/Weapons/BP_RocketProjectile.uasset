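; Rocket projectile actor that plays audio while alive and explodes when its Sphere overlaps another component.
; DestroyMissile spawns the explosion particles at that component's location and applies radial damage with falloff, destroying the rocket immediately if damage lands, otherwise after a short delay.
; Destruction stops the audio and plays an explosion sound.
; A line-trace impact check exists, but its looping timer setup is disconnected, so it never runs.
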(event OnComponentHit(Sphere)
  (params (HitComponent :type Primitive%20Component%20Object%20Reference) (OtherActor :type Actor%20Object%20Reference) (OtherComp :type Primitive%20Component%20Object%20Reference) (NormalImpulse :type Vector :default "0, 0, 0") (Hit :type Hit%20Result%20Structure%20%28by%20ref%29)))

(event OnComponentBeginOverlap(Sphere)
  (params (OverlappedComponent :type Primitive%20Component%20Object%20Reference) (OtherActor :type Actor%20Object%20Reference) (OtherComp :type Primitive%20Component%20Object%20Reference) (OtherBodyIndex :type Integer) (bFromSweep :type Boolean) (SweepResult :type Hit%20Result%20Structure%20%28by%20ref%29))
  (bind _returnvalue (Transformation|GetWorldLocation OtherComp))
  (bind _bisdestroyed_ (CallFunction|DestroyMissile _returnvalue "0, 0, 0" _returnvalue))
  (if _bisdestroyed_
    _
    (else
      (Utilities|FlowControl|Delay 0.2)
      (Actor|DestroyActor)))
  (Development|PrintString (Utilities|GetDisplayName OtherComp)))

(event Custom|event
  (bind _returnvalue (Transformation|GetActorLocation))
  (bind _outhit (Collision|LineTraceForObjects _returnvalue (+ _returnvalue (* (Transformation|GetActorLocation) 1e+02)) (Utilities|Array|MakeArray "ObjectTypeQuery1" "ObjectTypeQuery2") true 0 "ForDuration"))
  (if (and (.bBlockingHit (Collision|BreakHitResult _outhit)) (!= (.HitActor (Collision|BreakHitResult _outhit)) (Game|GetPlayerCharacter 0)))
    (CallFunction|DestroyMissile (.ImpactPoint (Collision|BreakHitResult _outhit)) (Math|Conversions|RotationFromXVector (.ImpactPoint (Collision|BreakHitResult _outhit))) (.ImpactPoint (Collision|BreakHitResult _outhit)))
    (Utilities|FlowControl|Delay 0.2)
    (Actor|DestroyActor)))

(event EventBeginPlay
  (|CallParentFunction)
  (Audio|Components|Audio|Play (Variables|Default|GetAudio) 0.0))

(event EventTick
  (params (DeltaSeconds :type Float%20%28single-precision%29))
  (|CallParentFunction DeltaSeconds))

(event EventDestroyed
  (Audio|PlaySoundatLocation "/Game/Static/Weapons/SciFiWeapLight/Sound/RocketLauncher/RL_Explosion_Cue.RL_Explosion_Cue" (Transformation|GetActorLocation) "0, 0, 0" 1.0 1.0 0.0 0 0 0)
  (Audio|Components|Audio|Stop (Variables|Default|GetAudio)))

(fn ConstructionScript
  (|CallParentFunction))

(fn DestroyMissile
  (params (Location :type Vector) (Rotation :type Rotator) (Origin :type Vector%20%28by%20ref%29))
  (Effects|SpawnEmitteratLocation "/Game/Static/Weapons/SciFiWeapLight/FX/Particles/P_RocketLauncher_Explosion_Light.P_RocketLauncher_Explosion_Light" Location Rotation)
  (bind _returnvalue (Class|GameplayStatics|ApplyRadialDamagewithFalloff 15.0 3.0 Origin 2.5e+02 5e+02 1.0 0 0 self (Game|GetInstigatorController) "ECC_Visibility"))
  (if _returnvalue
    (Actor|DestroyActor)
    (return _returnvalue)
    (else
      (return false))))
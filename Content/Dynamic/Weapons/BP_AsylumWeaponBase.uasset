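; Base weapon actor for firing, reloading, ammo pickups and level-based upgrades.
; BeginPlay loads data-table stats at level one or below, otherwise applies upgrade-table deltas through a level-to-row map.
; Fire and reload events call inherited logic, broadcast weapon data updates and message the mesh's anim instance.
; Shots and hits report noise and damage to AI perception, with impact particles and an extra headshot effect.
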(event OnComponentBeginOverlap(WeaponMesh)
  (params (OverlappedComponent :type Primitive%20Component%20Object%20Reference) (OtherActor :type Actor%20Object%20Reference) (OtherComp :type Primitive%20Component%20Object%20Reference) (OtherBodyIndex :type Integer) (bFromSweep :type Boolean) (SweepResult :type Hit%20Result%20Structure%20%28by%20ref%29)))

(event OnComponentHit(WeaponMesh)
  (params (HitComponent :type Primitive%20Component%20Object%20Reference) (OtherActor :type Actor%20Object%20Reference) (OtherComp :type Primitive%20Component%20Object%20Reference) (NormalImpulse :type Vector :default "0, 0, 0") (Hit :type Hit%20Result%20Structure%20%28by%20ref%29)))

(event EventBeginPlay
  (bind _weaponstatsdata (Variables|Default|GetWeaponStatsData))
  (bind _currentweaponlevel (Utilities|Struct|BreakWeaponStatsData _weaponstatsdata))
  (if (<= _currentweaponlevel 1)
    (CallFunction|SetStatsonStart (Variables|Default|GetNewGameRowName))
    (else
      (CallFunction|UpgradeWeaponLevel _currentweaponlevel))))

(event EventOnWeaponAmmoPickup
  (params (AmmoToAdd :type Float%20%28single-precision%29))
  (bind _weaponstatsdata (Variables|Default|GetWeaponStatsData))
  (Utilities|Struct|SetmembersinWeaponStatsData _weaponstatsdata (+ (.CurrentWeaponClips (Utilities|Struct|BreakWeaponStatsData _weaponstatsdata)) AmmoToAdd))
  (Default|CallUpdateWeaponData))

(event EventOnUnlimitedClipsToggle
  (Utilities|FlowControl|FlipFlop
    (:A
      _)
    (:B
      _))
  (Class|AsylumWeapon|UnlimitedClipsToggle))

(event EventOnEmptyWeaponFire
  (bind (_returnvalue _animinstance) (CallFunction|HasValidAnimInstance?))
  (Class|AsylumWeapon|WeaponDryFire)
  (if _returnvalue
    (Class|AsylumWeaponInterface|OnEmptyWeaponFire(Message) _animinstance)))

(event EventDestroyed
  (Effects|SpawnEmitteratLocation "/Game/Static/Weapons/SciFiWeapLight/FX/Particles/P_Grenade_Explosion_Dark.P_Grenade_Explosion_Dark" (Transformation|GetActorLocation) (Transformation|GetActorRotation) "0.250000,0.250000,0.250000" true "AutoRelease"))

(event EventOnDamageModify
  (bind _weaponstatsdata (Variables|Default|GetWeaponStatsData))
  (bind (_or_weapondamagetype _c_weapondamagetype _maxmagazineammo _basedamageamount _damagemodifieramount _specialdamagemultiplier) (Utilities|Struct|BreakWeaponStatsData _weaponstatsdata))
  (Utilities|Struct|SetmembersinWeaponStatsData _weaponstatsdata (CallFunction|DamageCalculation _basedamageamount _damagemodifieramount _specialdamagemultiplier)))

(event EventRecalculateBaseWeaponDamage
  (bind _weaponstatsdata (Variables|Default|GetWeaponStatsData))
  (bind (_or_weapondamagetype _c_weapondamagetype _maxmagazineammo _basedamageamount _damagemultiplieramount _damagemodifieramount _specialdamagemultiplier _criticalhitmultiplier _originalbasedamageamount _originaldamagemultiplier _originaldamagemodifier) (Utilities|Struct|BreakWeaponStatsData _weaponstatsdata))
  (Utilities|Struct|SetmembersinWeaponStatsData _weaponstatsdata _basedamageamount _damagemultiplieramount _damagemodifieramount (CallFunction|DamageCalculation _basedamageamount _damagemultiplieramount _damagemodifieramount) _specialdamagemultiplier _criticalhitmultiplier _originalbasedamageamount _originaldamagemultiplier _originaldamagemodifier))

(event EventOnGrantFullAmmo
  (Class|AsylumWeapon|GiveWeaponFullAmmo))

(event EventOnStartFire
  (bind (_returnvalue _animinstance) (CallFunction|HasValidAnimInstance?))
  (bind _weaponstatsdata (Variables|Default|GetWeaponStatsData))
  (bind (_or_weapondamagetype _c_weapondamagetype _maxmagazineammo _weaponfireloudness _weaponfiresoundrange) (Utilities|Struct|BreakWeaponStatsData _weaponstatsdata))
  (Class|AsylumWeapon|StartFire)
  (Class|AISenseHearing|ReportNoiseEvent (Transformation|GetActorLocation) _weaponfireloudness (Game|GetInstigator) _weaponfiresoundrange "None")
  (Default|CallUpdateWeaponData)
  (if _returnvalue
    (Class|AsylumWeaponInterface|OnStartFire(Message) _animinstance)))

(event EventOnStartReload
  (bind (_returnvalue _animinstance) (CallFunction|HasValidAnimInstance?))
  (Class|AsylumWeapon|StartReload)
  (Default|CallUpdateWeaponData)
  (Utilities|FlowControl|Sequence
    (:then_0
      (if _returnvalue
        (Class|AsylumWeaponInterface|OnStartReload(Message) _animinstance)))
    (:then_1
      (Class|AsylumPlayerInterface|OnPlayerReload(Message) (Game|GetPlayerCharacter 0)))))

(event EventOnFinishReload
  (bind (_returnvalue _animinstance) (CallFunction|HasValidAnimInstance?))
  (Default|CallUpdateWeaponData)
  (Utilities|FlowControl|Sequence
    (:then_0
      (Class|AsylumPlayerInterface|OnPlayerReloadFinish(Message) (Game|GetPlayerCharacter 0)))
    (:then_1
      (if _returnvalue
        (Class|AsylumWeaponInterface|OnFinishReload(Message) _animinstance)))))

(event EventOnFire
  (bind (_returnvalue _animinstance) (CallFunction|HasValidAnimInstance?))
  (Default|CallUpdateWeaponData)
  (Utilities|FlowControl|Sequence
    (:then_0
      (Default|CallOnPlayerUpdate (CallFunction|GetPC)))
    (:then_1
      (if (and (Variables|Default|GetbIsAutomatic) (not (Variables|Default|GetbIsWeaponEmpty)))
        (if _returnvalue
          (Class|AsylumWeaponInterface|OnFinishFire(Message) _animinstance))))))

(event EventOnFinishFire
  (bind (_returnvalue _animinstance) (CallFunction|HasValidAnimInstance?))
  (Class|AsylumWeapon|FinishFire)
  (Default|CallUpdateWeaponData)
  (if _returnvalue
    (Class|AsylumWeaponInterface|OnFinishFire(Message) _animinstance)))

(event EventOnHitTarget
  (bind _singlehit (Variables|Default|GetSingleHit))
  (bind (_bblockinghit _binitialoverlap _time _distance _location _impactpoint _normal _impactnormal _physmat _hitactor _hitcomponent _hitbonename) (Collision|BreakHitResult _singlehit))
  (Utilities|FlowControl|Sequence
    (:then_0
      (Class|AISenseDamage|ReportDamageEvent _hitactor (Game|GetInstigator) (.DamageAmountSum (Utilities|Struct|BreakWeaponStatsData (Variables|Default|GetWeaponStatsData))) _impactpoint)
      (Effects|SpawnEmitteratLocation "/Game/Static/VFX_Toolkit_V1/ParticleSystems/356Days/Par_BasicHit.Par_BasicHit" _impactpoint "0, 0, 0" "0.250000,0.250000,0.250000"))
    (:then_1
      (CallFunction|CriticalHitEvent _hitbonename _impactpoint))))

(event EventOnInfiniteAmmoToggle
  (Utilities|FlowControl|FlipFlop
    (:A
      _)
    (:B
      _))
  (Class|AsylumWeapon|InfiniteAmmoToggle))

(fn ConstructionScript)

(fn SetStatsonStart
  (params (RowName :type Name))
  (bind _returnvalue (Utilities|GetDataTableRow (Variables|Default|GetWeaponStatsTable) RowName)
    (:then
      (Utilities|Struct|SetmembersinWeaponStatsData (Variables|Default|GetWeaponStatsData) (.WeaponType (Utilities|Struct|BreakWeaponStatsData _returnvalue)) (.WeaponSlotType (Utilities|Struct|BreakWeaponStatsData _returnvalue)) (.WeaponAmmoType (Utilities|Struct|BreakWeaponStatsData _returnvalue)) (.OR_WeaponDamageType (Utilities|Struct|BreakWeaponStatsData _returnvalue)) (.C_WeaponDamageType (Utilities|Struct|BreakWeaponStatsData _returnvalue)) (.CurrentWeaponLevel (Utilities|Struct|BreakWeaponStatsData _returnvalue)) (.MaxWeaponLevel (Utilities|Struct|BreakWeaponStatsData _returnvalue)) (.FireRate (Utilities|Struct|BreakWeaponStatsData _returnvalue)) (.CurrentMagazineAmmo (Utilities|Struct|BreakWeaponStatsData _returnvalue)) (.AmmoConsumptionAmount (Utilities|Struct|BreakWeaponStatsData _returnvalue)) (.CurrentWeaponClips (Utilities|Struct|BreakWeaponStatsData _returnvalue)) (.MaxMagazineAmmo (Utilities|Struct|BreakWeaponStatsData _returnvalue)) (.MaxWeaponClips (Utilities|Struct|BreakWeaponStatsData _returnvalue)) (.MaxReloadTime (Utilities|Struct|BreakWeaponStatsData _returnvalue)) (.ReloadSpeed (Utilities|Struct|BreakWeaponStatsData _returnvalue)) (.BaseDamageAmount (Utilities|Struct|BreakWeaponStatsData _returnvalue)) (.DamageMultiplierAmount (Utilities|Struct|BreakWeaponStatsData _returnvalue)) (.DamageModifierAmount (Utilities|Struct|BreakWeaponStatsData _returnvalue)) (CallFunction|DamageCalculation (.BaseDamageAmount (Utilities|Struct|BreakWeaponStatsData _returnvalue)) (.DamageMultiplierAmount (Utilities|Struct|BreakWeaponStatsData _returnvalue)) (.DamageModifierAmount (Utilities|Struct|BreakWeaponStatsData _returnvalue))) (.SpecialDamageMultiplier (Utilities|Struct|BreakWeaponStatsData _returnvalue)) (.CriticalHitMultiplier (Utilities|Struct|BreakWeaponStatsData _returnvalue)) (.OriginalBaseDamageAmount (Utilities|Struct|BreakWeaponStatsData _returnvalue)) (.OriginalDamageMultiplier (Utilities|Struct|BreakWeaponStatsData _returnvalue)) (.OriginalDamageModifier (Utilities|Struct|BreakWeaponStatsData _returnvalue)) (.WeaponFireLoudness (Utilities|Struct|BreakWeaponStatsData _returnvalue)) (.WeaponFireSoundRange (Utilities|Struct|BreakWeaponStatsData _returnvalue)) (.WeaponDistanceRange (Utilities|Struct|BreakWeaponStatsData _returnvalue)) (.WeaponChargeLimit (Utilities|Struct|BreakWeaponStatsData _returnvalue)))
      (EventDispatchers|BindEventtoUpdateWeaponData (EventDispatchers|CreateEvent :!event CheckAmmo))
      (CallFunction|ToggleCollider false)
      (if (> (.FireRate (Utilities|Struct|BreakWeaponStatsData _returnvalue)) 0.0)
        (Variables|Default|SetbIsAutomatic true)))))

(fn CriticalHitEvent
  (params (HitBoneName :type Name) (Location :type Vector))
  (if (Utilities|Name|Equal(Name) HitBoneName "head")
    (Effects|SpawnEmitteratLocation "/Game/Static/VFX_Toolkit_V1/ParticleSystems/356Days/Par_CriticalHit.Par_CriticalHit" Location "0, 0, 0" "0.250000,0.250000,0.250000")))

(fn HasValidAnimInstance?
  (bind _weaponmesh (Variables|Default|GetWeaponMesh))
  (bind _returnvalue (Components|SkeletalMesh|GetAnimInstance _weaponmesh))
  (return (Utilities|IsValid _returnvalue) _returnvalue))

(fn ToggleCollider
  (params (Condition :type Boolean))
  (bind _weaponmesh (Variables|Default|GetWeaponMesh))
  (bind _weaponmesh_2 (Variables|Default|GetWeaponMesh))
  (if Condition
    (Collision|SetCollisionEnabled _weaponmesh "QueryAndPhysics")
    (Collision|SetCollisionObjectType _weaponmesh_2 "ECC_WorldDynamic")
    (Physics|SetSimulatePhysics _weaponmesh_2 true)
    (Collision|SetCollisionResponsetoAllChannels _weaponmesh_2 "ECR_Block")
    (else
      (Collision|SetCollisionEnabled _weaponmesh "NoCollision"))))

(fn UpgradeWeaponLevel
  (params (Key :type Integer%20%28by%20ref%29))
  (bind _weaponlevelmap (Variables|Default|GetWeaponLevelMap))
  (bind _weaponstatsdata (Variables|Default|GetWeaponStatsData))
  (bind (_firerate _maxmagazineammo _maxweaponclips _maxreloadtime _reloadspeed _damagemodifieramount _weapondistancerange _weaponchargelimit) (Utilities|Struct|BreakWeaponStatsData _weaponstatsdata))
  (bind (_value _returnvalue) (Utilities|Map|Find _weaponlevelmap Key))
  (if _returnvalue
    (bind _returnvalue_2 (Utilities|GetDataTableRow (Variables|Default|GetWeaponUpgradeDataTable) _value)
      (:then
        (Utilities|Struct|SetmembersinWeaponStatsData _weaponstatsdata (.NewWeaponLevel (Utilities|Struct|BreakWeaponUpgradeData _returnvalue_2)) (- _firerate (.FireRateUpgradeAmount (Utilities|Struct|BreakWeaponUpgradeData _returnvalue_2))) (+ _maxmagazineammo (.MagazineCapacityUpgradeAmount (Utilities|Struct|BreakWeaponUpgradeData _returnvalue_2))) (+ _maxweaponclips (.MaxClipCapacityUpgradeAmount (Utilities|Struct|BreakWeaponUpgradeData _returnvalue_2))) (+ _maxmagazineammo (.MagazineCapacityUpgradeAmount (Utilities|Struct|BreakWeaponUpgradeData _returnvalue_2))) (+ _maxweaponclips (.MaxClipCapacityUpgradeAmount (Utilities|Struct|BreakWeaponUpgradeData _returnvalue_2))) (- _maxreloadtime (.ReloadTimeReduceAmount (Utilities|Struct|BreakWeaponUpgradeData _returnvalue_2))) (+ _reloadspeed (.ReloadSpeedUpgradeAmount (Utilities|Struct|BreakWeaponUpgradeData _returnvalue_2))) (+ (.DamageUpgradeAmount (Utilities|Struct|BreakWeaponUpgradeData _returnvalue_2)) _damagemodifieramount) (+ (.DamageUpgradeAmount (Utilities|Struct|BreakWeaponUpgradeData _returnvalue_2)) _damagemodifieramount) (+ _weapondistancerange (.WeaponRangeUpgradeAmount (Utilities|Struct|BreakWeaponUpgradeData _returnvalue_2))) (+ _weaponchargelimit (.ChargeLimitAmountIncrease (Utilities|Struct|BreakWeaponUpgradeData _returnvalue_2))))
        (Default|CallUpdateWeaponData)
        (Development|PrintString (Utilities|String|ToString(Integer) (.CurrentWeaponLevel (Utilities|Struct|BreakWeaponStatsData (Variables|Default|GetWeaponStatsData)))) true true "(R=0.851307,G=1.000000,B=0.000000,A=1.000000)")))))
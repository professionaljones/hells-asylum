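; BP_PlayerWeapon_Drone is a player weapon that deploys a drone projectile where it is aimed.
; On fire start, it line traces 5000 units along the weapon mesh's forward vector against a single object type.
; It spawns a WeaponDroneProjectile directly at the hit location rather than at the muzzle, without checking whether the trace hit anything.
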(event EventBeginPlay
  (|CallParentFunction) ; This node is disabled and will not be called.\nDrag off pins to build functionality.
)

(event Collision|EventActorBeginOverlap
  (params (OtherActor :type Actor%20Object%20Reference)))

(event EventTick
  (params (DeltaSeconds :type Float%20%28single-precision%29)))

(event EventOnStartFire
  (bind _weaponmesh (Variables|Default|GetWeaponMesh))
  (bind _returnvalue (Transformation|GetWorldLocation _weaponmesh))
  (bind _outhit (Collision|LineTraceForObjects _returnvalue (+ _returnvalue (* (Math|Vector|GetForwardVector _weaponmesh) 5e+03)) (Utilities|Array|MakeArray "ObjectTypeQuery8") false 0 "None"))
  (Game|SpawnActorfromClass "/Game/Dynamic/Weapons/WeaponDroneProjectile.WeaponDroneProjectile_C" (Math|Conversions|ToTransform(Vector) (.Location (Collision|BreakHitResult _outhit))) "Undefined" 0 0))

(fn ConstructionScript
  (|CallParentFunction))
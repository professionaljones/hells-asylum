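; BP_BaseOrb is a suit-ability orb with two modes chosen by IsDespair: Despair damages enemies, Harmony heals the player.
; Looping timers drive periodic effects and per-frame attraction, with sphere traces setting the shared HitActor.
; Harmony lerps toward the player and self-destructs at full health, while Despair's attraction lerp targets its own location.
; Destruction clears stored timers and spawns a mode-specific particle effect; the rotate-around logic is unused.
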(event Custom|RotateAroundPoint)

(event EventBeginPlay
  (if (Variables|Stats|GetbIsDespair)
    (Variables|Stats|SetbShouldApplyDamage true)
    (CallFunction|SearchforEnemies)
    (bind _returnvalue (Utilities|Time|SetTimerbyEvent (EventDispatchers|CreateEvent :!event SearchforEnemies) (Variables|Stats|GetDespairDamageRate) true))
    (Variables|Default|SetDespairDamageTimer _returnvalue)
    (bind _returnvalue_2 (Utilities|Time|SetTimerbyEvent (EventDispatchers|CreateEvent :!event AttracttoEnemies) (Utilities|Time|GetWorldDeltaSeconds) true))
    (Variables|Default|SetDespairAttractTimer _returnvalue_2)
    (else
      (CallFunction|SearchforPlayer)
      (Utilities|Time|SetTimerbyEvent (EventDispatchers|CreateEvent :!event SearchforPlayer) (Variables|Stats|GetHarmonyHealRate) true)
      (bind _returnvalue_3 (Utilities|Time|SetTimerbyEvent (EventDispatchers|CreateEvent :!event AttracttoPlayer) (Utilities|Time|GetWorldDeltaSeconds) true))
      (Variables|Default|SetHarmonyTimer _returnvalue_3))))

(event EventDestroyed
  (bind _returnvalue (Transformation|GetActorTransform))
  (bind _returnvalue_2 (Transformation|GetActorTransform))
  (if (Variables|Stats|GetbIsDespair)
    (Utilities|Time|ClearandInvalidateTimerbyHandle (Variables|Default|GetDespairDamageTimer))
    (Utilities|Time|ClearandInvalidateTimerbyHandle (Variables|Default|GetDespairAttractTimer))
    (Effects|SpawnEmitteratLocation (Variables|Default|GetDespairDestroyPS) (.location _returnvalue_2) (.rotation _returnvalue_2) (.scale _returnvalue_2))
    (else
      (Utilities|Time|ClearandInvalidateTimerbyHandle (Variables|Default|GetHarmonyTimer))
      (Effects|SpawnEmitteratLocation (Variables|Default|GetHarmonyDestroyPS) (.location _returnvalue) (.rotation _returnvalue) (.scale _returnvalue)))))

(fn ConstructionScript
  (if (Variables|Stats|GetbIsDespair)
    (Variables|Stats|SetbShouldApplyDamage true)))

(fn SearchforEnemies
  (bind _returnvalue (Transformation|GetActorTransform))
  (bind _outhit (Collision|SphereTraceForObjects (.location _returnvalue) (+ (.location _returnvalue) (* (Math|Vector|GetForwardVector (.rotation _returnvalue)) (Variables|Stats|GetForwardVectorMod))) (Variables|Stats|GetDespairTraceRadius) (Variables|Default|GetDespairObjectTargets) true 0 "ForDuration" true "(R=1.000000,G=0.000000,B=0.000000,A=1.000000)" "(R=0.474559,G=0.000000,B=1.000000,A=1.000000)"))
  (if (.bBlockingHit (Collision|BreakHitResult _outhit))
    (bind _output_get (Variables|Default|SetHitActor (.HitActor (Collision|BreakHitResult _outhit))))
    (Utilities|IsValid _output_get
      (:Is%20Valid
        (Game|Damage|ApplyDamage (.HitActor (Collision|BreakHitResult _outhit)) (Variables|Stats|GetDamageAmount) (Game|GetInstigatorController) self)))))

(fn AttracttoEnemies
  (bind _returnvalue (Transformation|GetActorTransform))
  (bind _returnvalue_2 (Transformation|GetActorTransform))
  (Utilities|IsValid (Variables|Default|GetHitActor)
    (:Is%20Valid
      (Transformation|SetActorTransform (Math|Transform|MakeTransform (.location (Math|Transform|Lerp(Transform) (Math|Transform|MakeTransform (.location _returnvalue_2) (.rotation _returnvalue_2) "1,1,1") (Math|Transform|MakeTransform (.location _returnvalue) (.rotation _returnvalue) "1,1,1") 0.75 "DualQuatInterp")) "0, 0, 0" "1,1,1") true))))

(fn SearchforPlayer
  (bind _returnvalue (Game|GetPlayerCharacter 0))
  (bind _returnvalue_2 (Transformation|GetActorTransform))
  (bind _asasylum_player_character (Utilities|Casting|CastToAsylumPlayerCharacter _returnvalue))
  (bind _playerstatscomponent (Variables|/Script/HellsAsylum.AsylumPlayerCharacter|GetPlayerStatsComponent _asasylum_player_character))
  (bind _characterstatsdatastruct (Variables|/Script/HellsAsylum.AsylumStatsComponent|GetCharacterStatsDataStruct _playerstatscomponent))
  (bind (_fcurrenthealth _fmaxhealth) (Utilities|Struct|BreakCharacterStatsData _characterstatsdatastruct))
  (Utilities|FlowControl|Sequence
    (:then_0
      (bind _outhits (Collision|MultiSphereTraceForObjects (.location _returnvalue_2) (+ (.location _returnvalue_2) (* (Math|Vector|GetForwardVector (.rotation _returnvalue_2)) 5e+03)) (Variables|Stats|GetHarmonyTraceRadius) (Utilities|Array|MakeArray "ObjectTypeQuery9") true (stale _outactors) "ForDuration" true "(R=0.000000,G=1.000000,B=0.088387,A=1.000000)" "(R=1.000000,G=0.852464,B=0.000000,A=1.000000)"))
      (for _array_element _outhits
        (if (and (.bBlockingHit (Collision|BreakHitResult _array_element)) (== (.HitActor (Collision|BreakHitResult _array_element)) (Game|GetPlayerCharacter 0)))
          (Variables|Default|SetHitActor (.HitActor (Collision|BreakHitResult _array_element)))
          (Utilities|FlowControl|Sequence
            (:then_0
              (Class|AsylumCharacterInterface|OnRecoverHealth(Message) (Game|GetPlayerCharacter 0) (Variables|Stats|GetHealAmount)))
            (:then_1
              (if (>= _fcurrenthealth _fmaxhealth)
                (Actor|DestroyActor)))))))
    (:then_1
      (bind _outactors (Actor|GetAllActorswithInterface 0)))))

(fn AttracttoPlayer
  (bind _returnvalue (Transformation|GetActorTransform))
  (bind _hitactor (Variables|Default|GetHitActor))
  (bind _returnvalue_2 (Transformation|GetActorTransform _hitactor))
  (Utilities|IsValid _hitactor
    (:Is%20Valid
      (Transformation|SetActorTransform (Math|Transform|MakeTransform (.location (Math|Transform|Lerp(Transform) (Math|Transform|MakeTransform (.location _returnvalue) (.rotation _returnvalue) "1,1,1") (Math|Transform|MakeTransform (.location _returnvalue_2) (.rotation _returnvalue_2) "1,1,1") 0.1)) "0, 0, 0" "1,1,1") true)
      (Transformation|AttachComponentToComponent 0 "None" "KeepRelative" "KeepRelative" "KeepRelative" true))))
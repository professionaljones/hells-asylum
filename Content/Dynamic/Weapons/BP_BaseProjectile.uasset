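; Base projectile actor that damages whatever overlaps its sphere, with optional homing.
; BeginPlay enables homing on ProjectileMovement when IsHoming is set, and sphere overlaps apply DamageAmount using the instigator's controller.
; SearchForTarget, not called here, sphere-traces to an endpoint derived from actor location rather than forward vector.
; It makes a hit component the homing target if its actor implements TargetInterface.
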(event OnComponentBeginOverlap(Sphere)
  (params (OverlappedComponent :type Primitive%20Component%20Object%20Reference) (OtherActor :type Actor%20Object%20Reference) (OtherComp :type Primitive%20Component%20Object%20Reference) (OtherBodyIndex :type Integer) (bFromSweep :type Boolean) (SweepResult :type Hit%20Result%20Structure%20%28by%20ref%29))
  (Game|Damage|ApplyDamage OtherActor (Variables|Stats|GetDamageAmount) (Game|GetInstigatorController) (Game|GetInstigator)))

(event EventBeginPlay
  (if (Variables|Properties|GetbIsHoming?)
    (Variables|/Script/Engine.ProjectileMovementComponent|SetbIsHomingProjectile (Variables|Default|GetProjectileMovement) true)))

(event Collision|EventActorBeginOverlap
  (params (OtherActor :type Actor%20Object%20Reference)))

(event EventTick
  (params (DeltaSeconds :type Float%20%28single-precision%29)))

(fn ConstructionScript)

(fn SearchforTarget
  (bind _returnvalue (Transformation|GetActorLocation))
  (bind _outhit (Collision|SphereTraceForObjects _returnvalue (+ _returnvalue (* _returnvalue 5e+03)) (Variables|Properties|GetHomingRadius) (Variables|Properties|GetTargetObjectTypes) true (Variables|Properties|GetActorsToIgnore) "None"))
  (if (and (.bBlockingHit (Collision|BreakHitResult _outhit)) (Utilities|DoesObjectImplementInterface (.HitActor (Collision|BreakHitResult _outhit)) (Variables|Properties|GetTargetInterface)))
    (Variables|/Script/Engine.ProjectileMovementComponent|SetHomingTargetComponent (Variables|Default|GetProjectileMovement) (.HitComponent (Collision|BreakHitResult _outhit)))))
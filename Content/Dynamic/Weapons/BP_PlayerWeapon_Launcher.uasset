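; BP_PlayerWeapon_Launcher is a player rocket launcher weapon that spawns a BP_RocketProjectile on OnStartFire.
; The rocket spawns at the world location of the MyScene component on player 0's AsylumPlayerCharacter, using that player controller's control rotation.
; The Blueprint holds no other active logic beyond calling the parent construction script.
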(event EventBeginPlay
  (|CallParentFunction) ; This node is disabled and will not be called.\nDrag off pins to build functionality.
)

(event Collision|EventActorBeginOverlap
  (params (OtherActor :type Actor%20Object%20Reference)))

(event EventTick
  (params (DeltaSeconds :type Float%20%28single-precision%29)))

(event EventOnStartFire
  (Game|SpawnActorfromClass "/Game/Dynamic/Weapons/BP_RocketProjectile.BP_RocketProjectile_C" (Math|Transform|MakeTransform (.location (Transformation|GetWorldTransform (Variables|/Script/HellsAsylum.AsylumPlayerCharacter|GetMyScene (.AsAsylum%20Player%20Character (Utilities|Casting|CastToAsylumPlayerCharacter (Game|GetPlayerCharacter 0)))))) (Pawn|GetControlRotation (Game|GetPlayerController 0) :!class /Script/Engine.Controller) "1,1,1") "Undefined" 0 0))

(fn ConstructionScript
  (|CallParentFunction))
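; Interactive double gate door that checks the player's inventory when locked, then passes its timeline to CheckDoorState.
; When the player leaves the collision box, it re-locks and calls CloseOnEnter.
; The gate timeline's update slides both panels and restarts a light timeline that rotates a scene component and recolors two point lights.
; Neither timeline has a wired input here; the door-state functions are defined outside this graph.
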(event OnComponentEndOverlap(BoxCollision)
  (params (OverlappedComponent :type Primitive%20Component%20Object%20Reference) (OtherActor :type Actor%20Object%20Reference) (OtherComp :type Primitive%20Component%20Object%20Reference) (OtherBodyIndex :type Integer))
  (if (== OtherActor (Game|GetPlayerCharacter 0))
    (Variables|Default|SetbIsLocked true)
    (CallFunction|CloseonEnter (Variables|Default|GetDoor_GateTimeline))))

(event EventBeginPlay)

(event Collision|EventActorBeginOverlap
  (params (OtherActor :type Actor%20Object%20Reference))
  (|CallParentFunction OtherActor) ; This node is disabled and will not be called.\nDrag off pins to build functionality.
)

(event EventTick
  (params (DeltaSeconds :type Float%20%28single-precision%29))
  (|CallParentFunction DeltaSeconds) ; This node is disabled and will not be called.\nDrag off pins to build functionality.
)

(event EventOnInteractEvent
  (bind _door_gatetimeline (Variables|Default|GetDoor_GateTimeline))
  (if (Variables|Default|GetbIsLocked)
    (CallFunction|CheckPlayerInventory)
    (CallFunction|CheckDoorState _door_gatetimeline)
    (else
      (CallFunction|CheckDoorState _door_gatetimeline))))

(fn ConstructionScript
  (|CallParentFunction))
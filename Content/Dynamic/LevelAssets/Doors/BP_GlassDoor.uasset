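; BP_GlassDoor is an interactable, lockable double glass door built on inherited door logic.
; Interacting checks the player's inventory if locked, then passes GlassDoorTimeline to CheckDoorState either way.
; When the player leaves the box while it is open, it calls CloseOnEnter and LockOnExit.
; The timeline's update slides both panels along X, with no play inputs wired in this graph.
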(event OnComponentEndOverlap(BoxCollision)
  (params (OverlappedComponent :type Primitive%20Component%20Object%20Reference) (OtherActor :type Actor%20Object%20Reference) (OtherComp :type Primitive%20Component%20Object%20Reference) (OtherBodyIndex :type Integer))
  (if (== OtherActor (Game|GetPlayerCharacter 0))
    (if (Variables|Default|GetbIsOpen)
      (CallFunction|CloseonEnter (Variables|Default|GetGlassDoorTimeline))
      (CallFunction|LockonExit))))

(event EventBeginPlay
  (|CallParentFunction))

(event EventOnInteractEvent
  (bind _glassdoortimeline (Variables|Default|GetGlassDoorTimeline))
  (if (Variables|Default|GetbIsLocked)
    (CallFunction|CheckPlayerInventory)
    (CallFunction|CheckDoorState _glassdoortimeline)
    (else
      (CallFunction|CheckDoorState _glassdoortimeline))))

(fn ConstructionScript
  (|CallParentFunction))
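; Sci-fi door Blueprint that streams levels in or out when the player activates it.
; Interaction while locked runs an inventory check, then either unloads the previous level or loads the next and checks door state.
; Unlocked, it toggles a timeline with sound, doing a blocking level load before opening.
; An open door closes when the player leaves its box, using inherited door functions.
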(event OnComponentEndOverlap(BoxCollision)
  (params (OverlappedComponent :type Primitive%20Component%20Object%20Reference) (OtherActor :type Actor%20Object%20Reference) (OtherComp :type Primitive%20Component%20Object%20Reference) (OtherBodyIndex :type Integer))
  (if (== OtherActor (Game|GetPlayerCharacter 0))
    (if (Variables|Default|GetbIsOpen)
      (CallFunction|CloseonEnter (Variables|Default|GetDoor_SciFiTimeline)))))

(event EventBeginPlay
  (|CallParentFunction)
  (EventDispatchers|BindEventtoOnDoorActivate (delegate EventOnInteractEvent)))

(event EventOnInteractEvent
  (bind _door_scifitimeline (Variables|Default|GetDoor_SciFiTimeline))
  (if (Variables|Default|GetbIsLocked)
    (CallFunction|CheckPlayerInventory)
    (if (Variables|Default|GetbUnloadPreviousLevel?)
      (Game|UnloadStreamLevel(byName) (Variables|Default|GetLevelToUnload) true)
      (else
        (Game|LoadStreamLevel(byName) (Variables|Default|GetLevelToLoad) true true)
        (CallFunction|CheckDoorState (Variables|Default|GetDoor_SciFiTimeline))))
    (elif (Variables|Default|GetbIsLocked)
      (Audio|PlaySoundatLocation (Variables|Default|GetDoorLockedSound) (Transformation|GetActorLocation) "0, 0, 0" 1.0 1.0 0.0 0 0 0)
      (Class|BPIHUD|SetMessagewithTime(Message) (HUD|GetHUD (Game|GetPlayerController 0)) "Access Denied" 5.0)
      (elif (Variables|Default|GetbIsOpen)
        (Audio|PlaySoundatLocation (Variables|Default|GetDoorCloseSound) (Transformation|GetActorLocation) "0, 0, 0" 1.0 1.0 0.0 0 0 0)
        (Components|Timeline|ReversefromEnd _door_scifitimeline)
        (Variables|Default|SetbIsOpen false)
        (else
          (Game|LoadStreamLevel(byName) (Variables|Default|GetLevelToLoad) true true)
          (Audio|PlaySoundatLocation (Variables|Default|GetDoorOpenSound) (Transformation|GetActorLocation) "0, 0, 0" 1.0 1.0 0.0 0 0 0)
          (Components|Timeline|PlayfromStart _door_scifitimeline)
          (Variables|Default|SetbIsOpen true))))))

(fn ConstructionScript
  (|CallParentFunction))
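; Base door actor providing shared lock, open/close and key-check logic, with an empty event graph.
; CheckDoorState plays a denial sound and HUD message when locked, otherwise toggles IsOpen with sounds and drives a caller-supplied Timeline forward or in reverse.
; CheckPlayerInventory looks up a given key in the player's item inventory and, if found with a valid class, sends the item-use message to the player character and clears IsLocked.
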(event EventBeginPlay)

(event Collision|EventActorBeginOverlap
  (params (OtherActor :type Actor%20Object%20Reference)))

(event EventTick
  (params (DeltaSeconds :type Float%20%28single-precision%29)))

(fn ConstructionScript)

(fn CheckDoorState
  (params (DoorTimeline :type Timeline%20Component%20Object%20Reference))
  (if (Variables|Conditions|GetbIsLocked)
    (Audio|PlaySoundatLocation (Variables|Feedback|GetDoorLockedSound) (Transformation|GetActorLocation) "0, 0, 0" 1.0 1.0 0.0 0 0 0)
    (Class|BPIHUD|SetMessagewithTime(Message) (CallFunction|GetGameHUD) "Access Denied" 5.0)
    (elif (Variables|Conditions|GetbIsOpen)
      (Audio|PlaySoundatLocation (Variables|Feedback|GetDoorCloseSound) (Transformation|GetActorLocation) "0, 0, 0" 1.0 1.0 0.0 0 0 0)
      (Components|Timeline|ReversefromEnd DoorTimeline)
      (Variables|Conditions|SetbIsOpen false)
      (else
        (Audio|PlaySoundatLocation (Variables|Feedback|GetDoorAcknowledgeSound) (Transformation|GetActorLocation) "0, 0, 0" 1.0 1.0 0.0 0 0 0)
        (Audio|PlaySoundatLocation (Variables|Feedback|GetDoorOpenSound) (Transformation|GetActorLocation) "0, 0, 0" 1.0 1.0 0.0 0 0 0)
        (Components|Timeline|PlayfromStart DoorTimeline)
        (Variables|Conditions|SetbIsOpen true)))))

(fn CheckPlayerInventory
  (params (KeyToFind :type Integer%20%28by%20ref%29))
  (bind _item_inventory (CallFunction|GetPlayerItemInventory))
  (bind (_value _returnvalue) (Utilities|Map|Find _item_inventory KeyToFind))
  (if (and (Utilities|IsValidClass _value) _returnvalue)
    (Class|AsylumPlayerInterface|OnPlayerUseItem(Message) (Game|GetPlayerCharacter 0) _value)
    (if (Variables|Conditions|GetbIsLocked)
      (Variables|Conditions|SetbIsLocked false))))
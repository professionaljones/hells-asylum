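; Sci-fi door Blueprint that slides on interaction and calls a close when the player leaves its collision box.
; Its activate event runs an inventory check if the door is locked, then passes its timeline to CheckDoorState in either case.
; End overlap by the player passes the same timeline to CloseOnEnter if open.
; The timeline's update moves the door mesh's relative location, with no play inputs wired in this graph.
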(event OnComponentEndOverlap(BoxCollision)
  (params (OverlappedComponent :type Primitive%20Component%20Object%20Reference) (OtherActor :type Actor%20Object%20Reference) (OtherComp :type Primitive%20Component%20Object%20Reference) (OtherBodyIndex :type Integer))
  (if (== OtherActor (Game|GetPlayerCharacter 0))
    (if (Variables|Default|GetbIsOpen)
      (CallFunction|CloseonEnter (Variables|Default|GetDoor_SciFiTimeline)))))

(event EventBeginPlay
  (|CallParentFunction)
  (EventDispatchers|BindEventtoOnDoorActivate (delegate EventOnInteractEvent)))

(event EventOnInteractEvent
  (bind _door_scifitimeline (Variables|Default|GetDoor_SciFiTimeline))
  (if (Variables|Default|GetbIsLocked)
    (CallFunction|CheckPlayerInventory)
    (CallFunction|CheckDoorState _door_scifitimeline)
    (else
      (CallFunction|CheckDoorState _door_scifitimeline))))

(fn ConstructionScript
  (|CallParentFunction))
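; BP_DangerDoor is a level actor set up as a timed orb spawner, though its spawning logic is unfinished.
; On BeginPlay it starts a looping timer at OrbSpawnRate, apparently intended to drive SpawnOrbs, whose Sequence node leads nowhere.
; Three SpawnActor nodes target the world locations of Scene, Scene1 and Scene2, but none is wired to execute or shows an actor class, so no orbs spawn.
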(event Custom|SpawnOrbs
  (Utilities|FlowControl|Sequence))

(event EventBeginPlay
  (Utilities|Time|SetTimerbyEvent (EventDispatchers|CreateEvent :!event Custom|SpawnOrbs) (Variables|Default|GetOrbSpawnRate) true))

(fn ConstructionScript)
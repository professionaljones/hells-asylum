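; BP_OridonaElevator is an interactable elevator that travels between the Oridona's Bridge and Captain's Quarters levels.
; It creates a player for the bridge-to-captain Level Sequence on BeginPlay, and interacting opens the WBP_OridonaElevator widget.
; Level-selected events check the current level enum, play that single sequence forward to the quarters or in reverse to the bridge, and update the enum immediately.
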(event EventCaptainLevelSelected
  (switch Utilities|FlowControl|Switch|SwitchonOridonaElevatorSelectEnum (Variables|Default|GetElevatorLevelEnum)
    (:NewEnumerator4
      (Sequencer|Player|Play (Variables|Default|GetLS_BridgeToCaptain) :!class /Script/MovieScene.MovieSceneSequencePlayer)
      (Variables|Default|SetElevatorLevelEnum "NewEnumerator3"))))

(event EventBridgeLevelSelected
  (switch Utilities|FlowControl|Switch|SwitchonOridonaElevatorSelectEnum (Variables|Default|GetElevatorLevelEnum)
    (:NewEnumerator3
      (Class|MovieSceneSequencePlayer|PlayReverse (Variables|Default|GetLS_BridgeToCaptain))
      (Variables|Default|SetElevatorLevelEnum "NewEnumerator4"))))

(event EventOnInteractEvent
  (bind _returnvalue (UserInterface|CreateWidget "/Game/Dynamic/UserInterface/WBPs/Gameplay/WBP_OridonaElevator.WBP_OridonaElevator_C" (Game|GetPlayerController 0)))
  (UserInterface|Viewport|AddtoViewport _returnvalue 0))

(event EventBeginPlay
  (bind (_outactor _returnvalue) (Sequencer|Player|CreateLevelSequencePlayer "/Game/Dynamic/LevelSequences/Oridona/LS_OridonaBridgeToCaptain.LS_OridonaBridgeToCaptain"))
  (Variables|Default|SetNewVar_0 _outactor)
  (Variables|Default|SetLS_BridgeToCaptain _returnvalue))

(fn ConstructionScript)
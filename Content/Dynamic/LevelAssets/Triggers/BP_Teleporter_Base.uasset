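; Base teleporter actor that spawns a wormhole actor at its transform and provides functions to move the player.
; TeleportTwoWay sends the player to a given destination, while TeleportToCheckpoint uses the checkpoint transform loaded from the AutoSave02 save.
; Both disable input, re-enable it only on success, then start a looping one-second cooldown timer.
; Countdown decrements the cooldown, resetting it and clearing the timer at zero.
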(event EventBeginPlay
  (Game|SpawnActorfromClass (Variables|Default|GetHoleClass) (Transformation|GetActorTransform) "AdjustIfPossibleButAlwaysSpawn" 0 0)
  (Variables|Default|SetCurrentCooldown (Variables|Default|GetMaxCooldown)))

(fn ConstructionScript)

(fn TeleportTwoWay
  (params (DestLocation :type Vector))
  (bind _returnvalue (Game|GetPlayerCharacter 0))
  (bind _returnvalue_2 (Game|GetPlayerController 0))
  (Input|DisableInput _returnvalue _returnvalue_2)
  (bind _returnvalue_3 (Transformation|Teleport _returnvalue DestLocation "0, 0, 0"))
  (if _returnvalue_3
    (Development|PrintString "Teleported!")
    (Input|EnableInput _returnvalue _returnvalue_2)
    (Variables|Default|SetbWasUsed? _returnvalue_3)
    (bind _returnvalue_4 (Utilities|Time|SetTimerbyEvent (EventDispatchers|CreateEvent :!event Countdown) 1.0 true))
    (Variables|Default|SetCooldownHandle _returnvalue_4)))

(fn Countdown
  (if (Variables|Default|GetbWasUsed?)
    (bind _output_get (Variables|Default|SetCurrentCooldown (- (Variables|Default|GetCurrentCooldown) 1.0)))
    (if (<= _output_get 0.0)
      (Variables|Default|SetCurrentCooldown (Variables|Default|GetMaxCooldown))
      (Utilities|Time|ClearandInvalidateTimerbyHandle (Variables|Default|GetCooldownHandle)))))

(fn TeleporttoCheckpoint
  (bind _returnvalue (Game|GetPlayerCharacter 0))
  (bind _returnvalue_2 (Game|GetPlayerController 0))
  (Input|DisableInput _returnvalue _returnvalue_2)
  (bind _returnvalue_3 (SaveGame|DoesSaveGameExist "AutoSave02"))
  (if _returnvalue_3
    (bind _returnvalue_4 (SaveGame|LoadGamefromSlot "AutoSave02"))
    (bind _asbp_asylum_save_game (Utilities|Casting|CastToBP_AsylumSaveGame _returnvalue_4))
    (bind _returnvalue_5 (Transformation|Teleport _returnvalue (.Location (Math|Transform|BreakTransform (Utilities|Struct|BreakSaveGameData (Variables|/Game/Dynamic/Game/SaveGame/BP_AsylumSaveGame.BP_AsylumSaveGame_C|GetSG_ProfileDataStruct _asbp_asylum_save_game)))) (.Rotation (Math|Transform|BreakTransform (Utilities|Struct|BreakSaveGameData (Variables|/Game/Dynamic/Game/SaveGame/BP_AsylumSaveGame.BP_AsylumSaveGame_C|GetSG_ProfileDataStruct _asbp_asylum_save_game))))))
    (if _returnvalue_5
      (Development|PrintString "Teleported to checkpoint!")
      (Input|EnableInput _returnvalue _returnvalue_2)
      (Variables|Default|SetbWasUsed? _returnvalue_5)
      (bind _returnvalue_6 (Utilities|Time|SetTimerbyEvent (EventDispatchers|CreateEvent :!event Countdown) 1.0 true))
      (Variables|Default|SetCooldownHandle _returnvalue_6))))
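; BP_AmmoReloadBox is a trigger box that refills the player's weapon ammo when the player overlaps it.
; On overlap it plays a pickup sound and shows a timed "Ammo Recovered" HUD message.
; It then gives full ammo to each valid weapon in the player controller's three slots and calls a player update after each refill.
; It does not destroy or disable itself, so each new overlap triggers it again.
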(event OnComponentBeginOverlap(Box)
  (params (OverlappedComponent :type Primitive%20Component%20Object%20Reference) (OtherActor :type Actor%20Object%20Reference) (OtherComp :type Primitive%20Component%20Object%20Reference) (OtherBodyIndex :type Integer) (bFromSweep :type Boolean) (SweepResult :type Hit%20Result%20Structure%20%28by%20ref%29))
  (bind _returnvalue (CallFunction|GetPC))
  (bind _weaponslotone (Variables|/Script/HellsAsylum.AsylumPlayerCharacter|GetWeaponSlotOne _returnvalue))
  (bind _weaponslottwo (Variables|/Script/HellsAsylum.AsylumPlayerCharacter|GetWeaponSlotTwo _returnvalue))
  (bind _weaponslotthree (Variables|/Script/HellsAsylum.AsylumPlayerCharacter|GetWeaponSlotThree _returnvalue))
  (if (CallFunction|IsPlayerOtherActor? OtherActor)
    (Audio|PlaySound2D "/Game/Static/Weapons/SciFiWeapLight/Sound/Pistol/Wavs/Pistol_AmmoPickup01.Pistol_AmmoPickup01" 1.0 1.0 0.0 0 0)
    (Utilities|FlowControl|Sequence
      (:then_0
        (Class|BPIHUD|SetMessageTwowithTime(Message) (CallFunction|GetGameHUD) "Ammo Recovered" 5.0))
      (:then_1
        (if (Utilities|IsValid _weaponslotone)
          (Class|AsylumWeapon|GiveWeaponFullAmmo _weaponslotone)
          (Default|CallOnPlayerUpdate _returnvalue :!label _label)))
      (:then_2
        (if (Utilities|IsValid _weaponslottwo)
          (Class|AsylumWeapon|GiveWeaponFullAmmo _weaponslottwo)
          (goto _label)))
      (:then_3
        (if (Utilities|IsValid _weaponslotthree)
          (Class|AsylumWeapon|GiveWeaponFullAmmo _weaponslotthree)
          (goto _label))))))

(event EventBeginPlay)

(event Collision|EventActorBeginOverlap
  (params (OtherActor :type Actor%20Object%20Reference)))

(event EventTick
  (params (DeltaSeconds :type Float%20%28single-precision%29)))

(fn ConstructionScript)
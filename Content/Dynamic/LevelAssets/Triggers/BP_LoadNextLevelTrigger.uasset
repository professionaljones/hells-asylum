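; BP_LoadNextLevelTrigger is a box trigger that streams in the next level and signals a game save when the player enters.
; On player overlap it loads LevelToLoad with configurable visibility and blocking, calls the game instance's save message and shows a timed "Game Saved" HUD message.
; When the player leaves the box, it does a blocking unload using the current level name cached at BeginPlay.
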(event OnComponentBeginOverlap(Box)
  (params (OverlappedComponent :type Primitive%20Component%20Object%20Reference) (OtherActor :type Actor%20Object%20Reference) (OtherComp :type Primitive%20Component%20Object%20Reference) (OtherBodyIndex :type Integer) (bFromSweep :type Boolean) (SweepResult :type Hit%20Result%20Structure%20%28by%20ref%29))
  (if (CallFunction|IsPlayerOtherActor? OtherActor)
    (Game|LoadStreamLevel(byName) (Variables|Default|GetLevelToLoad) (Variables|Default|GetMakeVisibleAfterLoad) (Variables|Default|GetShouldBlockOnLoad?))
    (Class|BPIAsylumGameInterface|OnGameSave(Message) (Game|GetGameInstance))
    (Class|BPIHUD|SetMessagewithTime(Message) (CallFunction|GetGameHUD) "Game Saved" 5.0)))

(event OnComponentEndOverlap(Box)
  (params (OverlappedComponent :type Primitive%20Component%20Object%20Reference) (OtherActor :type Actor%20Object%20Reference) (OtherComp :type Primitive%20Component%20Object%20Reference) (OtherBodyIndex :type Integer))
  (if (CallFunction|IsPlayerOtherActor? OtherActor)
    (Game|UnloadStreamLevel(byName) (Utilities|String|StringToName (Variables|Default|GetCurrentLevelName)) true)))

(event EventBeginPlay
  (bind _returnvalue (Game|GetCurrentLevelName true))
  (Variables|Default|SetCurrentLevelName _returnvalue))

(fn ConstructionScript)
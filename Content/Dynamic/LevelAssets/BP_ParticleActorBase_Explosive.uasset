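; Explosive variant of a particle actor that attempts a one-shot radial damage burst where it spawns.
; On BeginPlay it runs a zero-length sphere trace at its location against pawns and one other object type.
; If the single returned hit is blocking and is not the player character, it applies radial damage at its origin; overlap and tick events are unused.
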(event EventBeginPlay
  (bind _returnvalue (Transformation|GetActorLocation))
  (|CallParentFunction)
  (bind _outhit (Collision|SphereTraceForObjects _returnvalue _returnvalue 2e+02 (Utilities|Array|MakeArray "ObjectTypeQuery8" "ObjectTypeQuery3") true 0 "None"))
  (if (and (!= (.HitActor (Collision|BreakHitResult _outhit)) (Game|GetPlayerCharacter 0)) (.bBlockingHit (Collision|BreakHitResult _outhit)))
    (Game|Damage|ApplyRadialDamage 5.0 _returnvalue 0.0 0 0 0 0 false "ECC_Visibility")))

(event Collision|EventActorBeginOverlap
  (params (OtherActor :type Actor%20Object%20Reference))
  (|CallParentFunction OtherActor) ; This node is disabled and will not be called.\nDrag off pins to build functionality.
)

(event EventTick
  (params (DeltaSeconds :type Float%20%28single-precision%29))
  (|CallParentFunction DeltaSeconds) ; This node is disabled and will not be called.\nDrag off pins to build functionality.
)

(fn ConstructionScript
  (|CallParentFunction))
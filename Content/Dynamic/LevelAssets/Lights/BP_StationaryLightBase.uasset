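; BP_StationaryLightBase is a base light Blueprint that exposes the color, intensity and attenuation radius of a point light as variables.
; The construction script applies these values to the PointLight component.
; BeginPlay repeats the same three setter calls, reapplying the values when play starts.
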(event EventBeginPlay
  (bind _pointlight (Variables|Default|GetPointLight))
  (Rendering|Components|Light|SetLightColor _pointlight (Variables|Settings|GetNewLightColor) true)
  (Rendering|Components|Light|SetIntensity _pointlight (Variables|Settings|GetLightIntensity))
  (Rendering|Lighting|SetAttenuationRadius _pointlight (Variables|Settings|GetAttenuationRadius)))

(fn ConstructionScript
  (bind _pointlight (Variables|Default|GetPointLight))
  (Rendering|Components|Light|SetLightColor _pointlight (Variables|Settings|GetNewLightColor) true)
  (Rendering|Components|Light|SetIntensity _pointlight (Variables|Settings|GetLightIntensity))
  (Rendering|Lighting|SetAttenuationRadius _pointlight (Variables|Settings|GetAttenuationRadius)))
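; AI controller for turrets that routes perception updates into blackboard keys.
; Each perception target update passes the sensed actor and stimulus to UpdateBlackboardKeys, and BeginPlay only calls the parent.
; An unconnected chain would copy the controlled BP_ShipTurret's health and shield from AsylumStats to the blackboard and zero its stamina key, but it never runs.
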(event OnTargetPerceptionUpdated(AIPerception)
  (params (Actor :type Actor%20Object%20Reference) (Stimulus :type AI%20Stimulus%20Structure))
  (CallFunction|UpdateBlackboardKeys Stimulus Actor))

(event EventBeginPlay
  (|CallParentFunction))

(fn ConstructionScript)
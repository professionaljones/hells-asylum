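; Humanoid AI controller that runs a behavior tree and keeps its blackboard updated for an AsylumCharacterAI pawn.
; On BeginPlay it binds a blackboard-update event, starts the tree and sets up the blackboard.
; UpdateAIData copies health, shield and equipped-weapon ammo to blackboard keys.
; Perception updates record stimulus location, plus attacker and receiver location for AsylumPlayerInterface actors, and clear those keys when sensing fails.
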(event OnTargetPerceptionUpdated(AIPerception)
  (params (Actor :type Actor%20Object%20Reference) (Stimulus :type AI%20Stimulus%20Structure))
  (CallFunction|UpdateBlackboardKeys Stimulus Actor))

(event EventBeginPlay
  (EventDispatchers|BindEventtoUpdateBlackboardData (EventDispatchers|CreateEvent :!event UpdateAIData))
  (AI|RunBehaviorTree (Variables|Default|GetCurrentBehaviorTree))
  (bind _blackboardcomponent (Class|AIController|UseBlackboard (Variables|Default|GetCurrentBlackboardData)))
  (Variables|Default|SetCurrentBlackboardComponent _blackboardcomponent)
  (Default|CallUpdateBlackboardData))

(fn ConstructionScript)

(fn UpdateAIData
  (bind _returnvalue (Pawn|GetControlledPawn))
  (bind _currentblackboardcomponent (Variables|Default|GetCurrentBlackboardComponent))
  (bind _asasylum_character_ai (Utilities|Casting|CastToAsylumCharacterAI _returnvalue))
  (bind _aistatscomponent (Variables|/Script/AsylumGame.AsylumCharacterAI|GetAIStatsComponent _asasylum_character_ai))
  (bind _ai_equippedweapon (Variables|/Script/AsylumGame.AsylumCharacterAI|GetAI_EquippedWeapon _asasylum_character_ai))
  (bind _characterstatsdatastruct (Variables|/Script/AsylumGame.CharacterStatsComponent|GetCharacterStatsDataStruct _aistatscomponent))
  (bind _weaponstatsdata (Variables|/Script/AsylumGame.BaseWeapon|GetWeaponStatsData _ai_equippedweapon))
  (bind (_fcurrenthealth _fcurrentshield) (Utilities|Struct|BreakCharacterStatsData _characterstatsdatastruct))
  (bind (_currentmagazineammo _maxmagazinecapacity) (Utilities|Struct|BreakWeaponStatsData _weaponstatsdata))
  (AI|Components|Blackboard|SetValueasFloat _currentblackboardcomponent (Variables|Default|GetCurrentHealthKey) _fcurrenthealth)
  (AI|Components|Blackboard|SetValueasFloat _currentblackboardcomponent (Variables|Default|GetCurrentShieldKey) _fcurrentshield)
  (Utilities|FlowControl|Sequence
    (:then_1
      (Utilities|IsValid _ai_equippedweapon
        (:Is%20Valid
          (AI|Components|Blackboard|SetValueasFloat _currentblackboardcomponent (Variables|Default|GetCurrentAmmoKey) _currentmagazineammo)
          (AI|Components|Blackboard|SetValueasFloat _currentblackboardcomponent (Variables|Default|GetMaxAmmoKey) _maxmagazinecapacity))))))

(fn UpdateBlackboardKeys
  (params (AIStimulus :type AI%20Stimulus%20Structure%20%28by%20ref%29) (TestObject :type Object%20Object%20Reference))
  (bind (_stimuluslocation _receiverlocation _bsuccessfullysensed) (Utilities|Struct|BreakAIStimulus AIStimulus))
  (bind _currentblackboardcomponent (Variables|Default|GetCurrentBlackboardComponent))
  (bind _currentblackboardcomponent_2 (Variables|Default|GetCurrentBlackboardComponent))
  (if _bsuccessfullysensed
    (Utilities|FlowControl|Sequence
      (:then_0
        (AI|Components|Blackboard|SetValueasVector (Variables|Default|GetCurrentBlackboardComponent) (Variables|Default|GetLastHeardKey) _stimuluslocation))
      (:then_1
        (if (Utilities|DoesObjectImplementInterface TestObject "/Script/AsylumGame.AsylumPlayerInterface")
          (AI|Components|Blackboard|SetValueasObject _currentblackboardcomponent_2 (Variables|Default|GetAttackerKey) TestObject)
          (AI|Components|Blackboard|SetValueasVector _currentblackboardcomponent_2 (Variables|Default|GetLastLocationKey) _receiverlocation))))
    (else
      (AI|Components|Blackboard|ClearValue _currentblackboardcomponent (Variables|Default|GetLastHeardKey))
      (AI|Components|Blackboard|ClearValue _currentblackboardcomponent (Variables|Default|GetLastLocationKey))
      (AI|Components|Blackboard|ClearValue _currentblackboardcomponent (Variables|Default|GetAttackerKey)))))